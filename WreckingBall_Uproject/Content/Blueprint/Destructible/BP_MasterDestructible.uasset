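; Master destructible wall actor that advances three static meshes through data-driven damage states when hit.
; Each hit actor registers only once until removed from the list, then plays a sound and advances the state, changing collision at the last one.
; Non-destructible instances instead receive an impulse along the impact normal.
; Valid hits also detach attached actors, waking and pushing physics-simulating BP_M_PhysicObject ones outward.
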(event `self.ReceiveBeginPlay`
  ;[0 0.1529 1 0.5] Begin Play
  (for _array_element (`self.GetAttachedActors` false)
    (`KismetSystemLibrary.PrintString` (`KismetSystemLibrary.GetDisplayName` _array_element))))

(event `Hit recieved`
  (params (HitActor :type "Actor Object Reference") (`Impact Normal` :type "Vector Structure"))
  ;[1 0 0.06535 0.5] Hit Recieve
  (`self.Hit Validator` HitActor
    (:`Can Hit`
      (`self.WallMeshHit` `Impact Normal`)
      (`self.ImpulseOnAttachedActors`))))

(event `Remove From List`
  (params (`Hit Actor` :type "Actor Object Reference"))
  ;[1 0 0.06535 0.5] Remove Hit Actor From List
  (`KismetArrayLibrary.Array_RemoveItem` (`self.HitActorList`) `Hit Actor`))

(fn `ImpulseOnAttachedActors`
  (for _array_element (`self.GetAttachedActors` false)
    (`/Engine/EditorBlueprintResources/StandardMacros.IsValid` _array_element
      (:`Is Valid`
        (`self.K2_DetachFromActor` _array_element "KeepRelative" "KeepRelative" "KeepRelative")
        (bind (_asbp_m_physic_object _bsuccess) (cast `/Game/Blueprint/PhysicalObject/BP_M_PhysicObject` _array_element :!pure true))
        (bind _sm_physicobject (`/Game/Blueprint/PhysicalObject/BP_M_PhysicObject.SM_PhysicObject` _asbp_m_physic_object))
        (if (and (`SceneComponent.IsSimulatingPhysics` _sm_physicobject "None") _bsuccess)
          (`PrimitiveComponent.WakeRigidBody` _sm_physicobject "None")
          (`PrimitiveComponent.AddImpulse` _sm_physicobject (* (`KismetMathLibrary.GetDirectionUnitVector` (`self.K2_GetActorLocation`) (`self.K2_GetActorLocation` _array_element)) 25.0) "None" true))))))

(fn `SingleMeshHit`
  (params (ImpactNormal :type "Vector Structure")))

(fn `UserConstructionScript`
  (bind (_wall01 _inbetween _wall02) (break `/Game/Blueprint/PhysicalObject/STR_Wall` (`|GetArrayItem` (`.DestructibleState_3_D65A5BFC4FAC6C6B845734A314E4CD8D` (break `/Game/Blueprint/PhysicalObject/STR_DestructibleWall` (`self.Destructible Wall State`))))))
  (`StaticMeshComponent.SetStaticMesh` (`self.SM_Wall_Side01`) _wall01)
  (`StaticMeshComponent.SetStaticMesh` (`self.SM_Wall_InBetween`) _inbetween)
  (`StaticMeshComponent.SetStaticMesh` (`self.SM_Wall_Side02`) _wall02))

(fn `WallMeshHit`
  (params (ImpactNormal :type "Vector Structure"))
  (bind _returnvalue (`self.GetComponentByClass` "/Script/Engine.StaticMeshComponent"))
  (bind _currentstate (`self.CurrentState`))
  (bind (_wall01 _inbetween _wall02) (break `/Game/Blueprint/PhysicalObject/STR_Wall` (`|GetArrayItem` (`.DestructibleState_3_D65A5BFC4FAC6C6B845734A314E4CD8D` (break `/Game/Blueprint/PhysicalObject/STR_DestructibleWall` (`self.Destructible Wall State`))) (`self.CurrentState`))))
  (`GameplayStatics.PlaySound2D` (`.HitSFX_19_EFF4C5B74A5BB19575709D8E92DDF7A1` (break `/Game/Blueprint/PhysicalObject/STR_DestructibleWall` (`self.Destructible Wall State`))) 1.0 1.0 0.0 null null)
  (if (`self.Can Be Destroyed`)
    (bind _result (`/Engine/EditorBlueprintResources/StandardMacros.IncrementInt` _currentstate)
      (:`  `
        (set `self.CurrentState` (`KismetMathLibrary.Clamp` _result 0 (`KismetArrayLibrary.Array_LastIndex` (`.DestructibleState_3_D65A5BFC4FAC6C6B845734A314E4CD8D` (break `/Game/Blueprint/PhysicalObject/STR_DestructibleWall` (`self.Destructible Wall State`))))))
        (`StaticMeshComponent.SetStaticMesh` (`self.SM_Wall_Side01`) _wall01)
        (`StaticMeshComponent.SetStaticMesh` (`self.SM_Wall_InBetween`) _inbetween)
        (`StaticMeshComponent.SetStaticMesh` (`self.SM_Wall_Side02`) _wall02)
        (if (== (`KismetArrayLibrary.Array_LastIndex` (`.DestructibleState_3_D65A5BFC4FAC6C6B845734A314E4CD8D` (break `/Game/Blueprint/PhysicalObject/STR_DestructibleWall` (`self.Destructible Wall State`)))) _currentstate)
          (`PrimitiveComponent.SetCollisionEnabled` (`self.SM_Wall_Side02`) (`self.LastIndexCollision`))
          (`PrimitiveComponent.SetCollisionEnabled` (`self.SM_Wall_InBetween`) (`self.LastIndexCollision`))
          (`PrimitiveComponent.SetCollisionEnabled` (`self.SM_Wall_Side01`) (`self.LastIndexCollision`)))))
    (else
      (`/Engine/EditorBlueprintResources/StandardMacros.IsValid` _returnvalue
        (:`Is Valid`
          (`PrimitiveComponent.AddImpulse` _returnvalue (* ImpactNormal (`self.ImpulseValue`)) "None" true))))))