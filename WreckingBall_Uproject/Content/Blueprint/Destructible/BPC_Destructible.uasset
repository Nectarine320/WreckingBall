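; Destructible component that makes its owning actor react to hits, with wall-specific handling for BP_M_PhysicObject owners.
; When destructible, each hit advances a damage state, swapping one mesh or three wall meshes and changing collision at the last state; an invalid single-mesh entry destroys the actor.
; Non-destructible owners get an impulse along the impact normal instead.
; Every hit also detaches the physics object's attached actors, pushing simulating ones away from it.
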(event `self.ReceiveBeginPlay`
  (bind (_asbp_m_physic_object _bsuccess) (cast `/Game/Blueprint/PhysicalObject/BP_M_PhysicObject` (`self.GetOwner`) :!pure true))
  (if _bsuccess
    (set `self.As BP Master Combustible Object` _asbp_m_physic_object)))

(event `Hit recieved`
  (params (`Impact Location` :type "Vector Structure") (`Impact Normal` :type "Vector Structure"))
  (bind _as_bp_master_combustible_object (`self.As BP Master Combustible Object`))
  (`/Engine/EditorBlueprintResources/StandardMacros.IsValid` _as_bp_master_combustible_object
    (:`Is Valid`
      (if (`/Game/Blueprint/PhysicalObject/BP_M_PhysicObject.IsWall` _as_bp_master_combustible_object)
        (`self.WallMeshHit` `Impact Normal`)
        (else
          (`self.SingleMeshHit` `Impact Normal` :!label _label))))
    (:`Is Not Valid`
      (goto _label)))
  (`self.ImpulseOnAttachedActors` (0.0 0.0 0.0) `Impact Normal`))

(fn `ImpulseOnAttachedActors`
  (params (`Hit Location` :type "Vector Structure") (`Hit Normal` :type "Vector Structure"))
  (bind _as_bp_master_combustible_object (`self.As BP Master Combustible Object`))
  (`/Engine/EditorBlueprintResources/StandardMacros.IsValid` _as_bp_master_combustible_object
    (:`Is Valid`
      (for _array_element (`/Game/Blueprint/PhysicalObject/BP_M_PhysicObject.AttachedActors` _as_bp_master_combustible_object)
        (`/Engine/EditorBlueprintResources/StandardMacros.IsValid` _array_element
          (:`Is Valid`
            (`Actor.K2_DetachFromActor` _array_element "KeepRelative" "KeepRelative" "KeepRelative")
            (bind (_asbp_m_physic_object _bsuccess) (cast `/Game/Blueprint/PhysicalObject/BP_M_PhysicObject` _array_element :!pure true))
            (bind _sm_physicobject (`/Game/Blueprint/PhysicalObject/BP_M_PhysicObject.SM_PhysicObject` _asbp_m_physic_object))
            (if (and (`SceneComponent.IsSimulatingPhysics` _sm_physicobject "None") _bsuccess)
              (`PrimitiveComponent.AddImpulse` _sm_physicobject (* (`KismetMathLibrary.GetDirectionUnitVector` (`Actor.K2_GetActorLocation` _as_bp_master_combustible_object) (`Actor.K2_GetActorLocation` _array_element)) 25.0) "None" true))))))))

(fn `SingleMeshHit`
  (params (ImpactNormal :type "Vector Structure"))
  (bind _staticmeshstate (`self.StaticMeshState`))
  (bind _current_state (`self.Current State`))
  (bind _returnvalue (`Actor.GetComponentByClass` (`self.GetOwner`) "/Script/Engine.StaticMeshComponent"))
  (bind _returnvalue_2 (`Actor.GetComponentByClass` (`self.GetOwner`) "/Script/Engine.StaticMeshComponent"))
  (bind _output (`|GetArrayItem` _staticmeshstate (`self.Current State`)))
  (`GameplayStatics.PlaySound2D` null 1.0 1.0 0.0 null null)
  (if (`self.CanBeDestroyed`)
    (bind _result (`/Engine/EditorBlueprintResources/StandardMacros.IncrementInt` _current_state)
      (:`  `
        (set `self.Current State` (`KismetMathLibrary.Clamp` _result 0 (`KismetArrayLibrary.Array_LastIndex` (`self.StaticMeshState`))))
        (`/Engine/EditorBlueprintResources/StandardMacros.IsValid` _returnvalue_2
          (:`Is Valid`
            (`/Engine/EditorBlueprintResources/StandardMacros.IsValid` _output
              (:`Is Valid`
                (`StaticMeshComponent.SetStaticMesh` _returnvalue_2 _output)
                (if (== (`KismetArrayLibrary.Array_LastIndex` _staticmeshstate) _current_state)
                  (`PrimitiveComponent.SetCollisionEnabled` _returnvalue_2 (`self.Last Index Collision`))))
              (:`Is Not Valid`
                (`|ExecutionSequence`
                  (:`then_1`
                    (`Actor.K2_DestroyActor` (`self.GetOwner`))))))))))
    (else
      (`/Engine/EditorBlueprintResources/StandardMacros.IsValid` _returnvalue
        (:`Is Valid`
          (`PrimitiveComponent.AddImpulse` _returnvalue (* ImpactNormal 500.0) "None" true))))))

(fn `WallMeshHit`
  (params (ImpactNormal :type "Vector Structure"))
  (bind _as_bp_master_combustible_object (`self.As BP Master Combustible Object`))
  (bind _current_state (`self.Current State`))
  (bind _returnvalue (`Actor.GetComponentByClass` (`self.GetOwner`) "/Script/Engine.StaticMeshComponent"))
  (bind (_wall01 _inbetween _wall02) (break `/Game/Blueprint/PhysicalObject/STR_Wall` (`|GetArrayItem` (`.DestructibleState_3_D65A5BFC4FAC6C6B845734A314E4CD8D` (break `/Game/Blueprint/PhysicalObject/STR_DestructibleWall` (`self.DestructibleWallState`))) (`self.Current State`))))
  (`GameplayStatics.PlaySound2D` (`.HitSFX_19_EFF4C5B74A5BB19575709D8E92DDF7A1` (break `/Game/Blueprint/PhysicalObject/STR_DestructibleWall` (`self.DestructibleWallState`))) 1.0 1.0 0.0 null null)
  (if (`self.CanBeDestroyed`)
    (bind _result (`/Engine/EditorBlueprintResources/StandardMacros.IncrementInt` _current_state)
      (:`  `
        (set `self.Current State` (`KismetMathLibrary.Clamp` _result 0 (`KismetArrayLibrary.Array_LastIndex` (`.DestructibleState_3_D65A5BFC4FAC6C6B845734A314E4CD8D` (break `/Game/Blueprint/PhysicalObject/STR_DestructibleWall` (`self.DestructibleWallState`))))))
        (`StaticMeshComponent.SetStaticMesh` (`/Game/Blueprint/PhysicalObject/BP_M_PhysicObject.SM_Wall_01` (`self.As BP Master Combustible Object`)) _wall01)
        (`StaticMeshComponent.SetStaticMesh` (`/Game/Blueprint/PhysicalObject/BP_M_PhysicObject.SM_PhysicObject` _as_bp_master_combustible_object) _inbetween)
        (`StaticMeshComponent.SetStaticMesh` (`/Game/Blueprint/PhysicalObject/BP_M_PhysicObject.SM_Wall_02` _as_bp_master_combustible_object) _wall02)
        (if (== (`KismetArrayLibrary.Array_LastIndex` (`.DestructibleState_3_D65A5BFC4FAC6C6B845734A314E4CD8D` (break `/Game/Blueprint/PhysicalObject/STR_DestructibleWall` (`self.DestructibleWallState`)))) _current_state)
          (`PrimitiveComponent.SetCollisionEnabled` (`/Game/Blueprint/PhysicalObject/BP_M_PhysicObject.SM_Wall_01` (`self.As BP Master Combustible Object`)) (`self.Last Index Collision`))
          (`PrimitiveComponent.SetCollisionEnabled` (`/Game/Blueprint/PhysicalObject/BP_M_PhysicObject.SM_PhysicObject` (`self.As BP Master Combustible Object`)) (`self.Last Index Collision`))
          (`PrimitiveComponent.SetCollisionEnabled` (`/Game/Blueprint/PhysicalObject/BP_M_PhysicObject.SM_Wall_02` (`self.As BP Master Combustible Object`)) (`self.Last Index Collision`)))))
    (else
      (`/Engine/EditorBlueprintResources/StandardMacros.IsValid` _returnvalue
        (:`Is Valid`
          (`PrimitiveComponent.AddImpulse` _returnvalue (* ImpactNormal 500.0) "None" true))))))