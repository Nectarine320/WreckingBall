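; Game Instance that manages local multiplayer join slots, including controllers, parity-based teams and per-slot ball choices.
; Input device events create or assign players to free slots during join sessions, with slot 0 held by the primary player.
; Gameplay tags track slot state, a timer grants disconnected joined players a grace period, and changes notify listeners.
; Non-shipping fake players aid testing, and random ball picks are weighted by player selections.
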(event `self.ReceiveInit`
  ;[0 0.1529 1 0.5] Begin Play / Initializer
  (`KismetSystemLibrary.ExecuteConsoleCommand` "CommonUI.ShouldVirtualAcceptSimulateMouseButton 0" null)
  (`self.ResetSlots`)
  (add `self.OnInputDeviceConnectionChange` (delegate `HandleInputDeviceConnectionChange`)))

(event `OnInputDeviceConnectionChange_Event`
  (params (NewConnectionState :type "EInputDeviceConnectionState Enum" :default "Invalid") (PlatformUserId :type "PlatformUserId Structure") (InputDeviceId :type "InputDeviceId Structure")))

(event `OnInputDeviceConnectionChange_Event_0`
  (params (NewConnectionState :type "EInputDeviceConnectionState Enum" :default "Invalid") (PlatformUserId :type "PlatformUserId Structure") (InputDeviceId :type "InputDeviceId Structure")))

(event `OnInputDeviceConnectionChange_Event_1`
  (params (NewConnectionState :type "EInputDeviceConnectionState Enum" :default "Invalid") (PlatformUserId :type "PlatformUserId Structure") (InputDeviceId :type "InputDeviceId Structure")))

(event `HandleInputDeviceConnectionChange` :!signature `self.OnInputDeviceConnectionChange`
  (params (NewConnectionState :type "EInputDeviceConnectionState Enum" :default "Invalid") (PlatformUserId :type "PlatformUserId Structure") (InputDeviceId :type "InputDeviceId Structure"))
  ;[1 0 0.06535 0.5] On Controller Update Detected
  (switch `EInputDeviceConnectionState` NewConnectionState
    (:`Disconnected`
      (`self.HandleControllerDisconnected` PlatformUserId))
    (:`Connected`
      (`self.RegisterControllerForUser` PlatformUserId)
      (`self.OnPlayerSlotsChanged`))))

(fn `AssignControllerToFreeSlot`
  (params (Controller :type "PlayerController Object Reference"))
  (bind _returnvalue (`KismetArrayLibrary.Array_Find` (`self.SlotControllers`) Controller))
  (if (>= _returnvalue 0)
    (if (`BlueprintGameplayTagLibrary.MatchesTag` (`|GetArrayItem` (`self.SlotStates`) _returnvalue) (struct :`TagName` "Player.Slot.Disconnected") true)
      (`self.SetSlotState` _returnvalue (struct :`TagName` "Player.Slot.Joined")))
    (else
      (bind _freeslotindex (`self.FindFreeSlot`))
      (if (> _freeslotindex 0)
        (`self.SetSlot` _freeslotindex Controller (struct :`TagName` "Player.Slot.Connected"))))))

(fn `CanStartMatch`
  (returns (CanStart :type Boolean))
  (bind _joinedcount (`self.GetJoinedCount`))
  (return (>= _joinedcount (`self.MinPlayersToStart`))))

(fn `ClearDisconnectedSlots`
  (for _index (range 1 (`self.MaxPlayers`))
    (if (`BlueprintGameplayTagLibrary.MatchesTag` (`|GetArrayItem` (`self.SlotStates`) _index) (struct :`TagName` "Player.Slot.Disconnected") true)
      (`self.ReleaseSlot` _index)))
  (`self.OnPlayerSlotsChanged`))

(fn `ClearSlotBallType`
  (params (SlotIndex :type Integer))
  (if (`KismetArrayLibrary.Array_IsValidIndex` (`self.SlotBallTypes`) SlotIndex)
    (`KismetArrayLibrary.Array_Set` (`self.SlotBallTypes`) (`local.SlotIndex`))))

(fn `CloseJoinSession`
  (params (KeepJoinedPlayers :type Boolean))
  (set `self.JoinSessionOpen` false)
  (`KismetSystemLibrary.K2_ClearAndInvalidateTimerHandle` (`self.DisconnectTimer`))
  (for _index (range 1 (`self.MaxPlayers`))
    (if (not (and KeepJoinedPlayers (`BlueprintGameplayTagLibrary.MatchesTag` (`|GetArrayItem` (`self.SlotStates`) _index) (struct :`TagName` "Player.Slot.Joined") true)))
      (`self.ReleaseSlot` _index)))
  (`self.OnPlayerSlotsChanged`))

(fn `DebugToggleFakePlayer`
  (params (SlotIndex :type Integer))
  (if (or (`KismetSystemLibrary.IsPackagedForDistribution`) (not (`self.JoinSessionOpen`)))
    _
    (elif (not (or (<= SlotIndex 0) (>= SlotIndex (`self.MaxPlayers`))))
      (if (`BlueprintGameplayTagLibrary.MatchesTag` (`|GetArrayItem` (`self.SlotStates`) SlotIndex) (struct :`TagName` "Player.Slot.Empty") true)
        (bind _returnvalue (`GameplayStatics.CreatePlayer` (+ SlotIndex 4)))
        (`self.SetSlot` SlotIndex _returnvalue (struct :`TagName` "Player.Slot.Joined"))
        (`KismetArrayLibrary.Array_Set` (`self.SlotIsDebug`) SlotIndex true)
        (elif (`|GetArrayItem` (`self.SlotIsDebug`) SlotIndex)
          (`self.ReleaseSlot` SlotIndex)))
      (`self.OnPlayerSlotsChanged`))))

(fn `FindFreeSlot`
  (returns (FreeSlotIndex :type Integer))
  (for _index (range 1 (`self.MaxPlayers`))
    (if (`BlueprintGameplayTagLibrary.MatchesTag` (`|GetArrayItem` (`self.SlotStates`) _index) (struct :`TagName` "Player.Slot.Empty") true)
      (return _index)))
  (return -1))

(fn `FindLastDebugSlot`
  (returns (DebugSlotIndex :type Integer))
  (locals (LastDebug :type Integer))
  (set `local.LastDebug` -1)
  (for _index (range 1 (`self.MaxPlayers`))
    (if (`|GetArrayItem` (`self.SlotIsDebug`) _index)
      (set `local.LastDebug` _index)))
  (return (`local.LastDebug`)))

(fn `FindSlotByControllerId`
  (params (ControllerId :type Integer))
  (returns (SlotIndex :type Integer))
  (return (`KismetArrayLibrary.Array_Find` (`self.SlotControllerIds`) ControllerId)))

(fn `FindSlotOfController`
  (params (Controller :type "PlayerController Object Reference"))
  (returns (SlotIndex :type Integer))
  (return (`KismetArrayLibrary.Array_Find` (`self.SlotControllers`) Controller)))

(fn `GetBallTypeOfSlot`
  (params (SlotIndex :type Integer))
  (returns (BallType :type "/Game/Blueprint/Ball/Data/PDA_BallType Object Reference"))
  (if (`KismetArrayLibrary.Array_IsValidIndex` (`self.SlotBallTypes`) SlotIndex)
    (return (`|GetArrayItem` (`self.SlotBallTypes`) (`local.SlotIndex`)))
    (else
      (return null))))

(fn `GetJoinedCount`
  (returns (JoinedCount :type Integer))
  (locals (Tally :type Integer))
  (set `local.Tally` 0)
  (for _array_element (`self.SlotStates`)
    (if (`BlueprintGameplayTagLibrary.MatchesTag` _array_element (struct :`TagName` "Player.Slot.Joined") true)
      (set `local.Tally` (+ (`local.Tally`) 1))))
  (return (`local.Tally`)))

(fn `GetSlotState`
  (params (SlotIndex :type Integer))
  (returns (State :type "GameplayTag Structure"))
  (return (`|GetArrayItem` (`self.SlotStates`) SlotIndex)))

(fn `GetSlotTeam`
  (params (SlotIndex :type Integer))
  (returns (TeamIndex :type Integer))
  (return (mod SlotIndex 2)))

(fn `HandleControllerDisconnected`
  (params (UserId :type "PlatformUserId Structure"))
  (if (not (not (`self.JoinSessionOpen`)))
    (bind _returnvalue (`InputDeviceLibrary.GetPlayerControllerFromPlatformUser` UserId))
    (bind _returnvalue_2 (`KismetArrayLibrary.Array_Find` (`self.SlotControllers`) _returnvalue))
    (if (> _returnvalue_2 0)
      (if (`BlueprintGameplayTagLibrary.MatchesTag` (`|GetArrayItem` (`self.SlotStates`) _returnvalue_2) (struct :`TagName` "Player.Slot.Joined") true)
        (`self.SetSlotState` _returnvalue_2 (struct :`TagName` "Player.Slot.Disconnected"))
        (bind _returnvalue_3 (`KismetSystemLibrary.K2_SetTimer` self "ClearDisconnectedSlots" (`self.DisconnectGraceSeconds`)))
        (set `self.DisconnectTimer` _returnvalue_3)
        (else
          (`self.ReleaseSlot` _returnvalue_2)))
      (`self.OnPlayerSlotsChanged`))))

(fn `JoinSlot`
  (params (Controller :type "PlayerController Object Reference"))
  (returns (Joined :type Boolean))
  (bind _returnvalue (`KismetArrayLibrary.Array_Find` (`self.SlotControllers`) Controller))
  (if (> _returnvalue 0)
    (if (`BlueprintGameplayTagLibrary.MatchesTag` (`|GetArrayItem` (`self.SlotStates`) _returnvalue) (struct :`TagName` "Player.Slot.Connected") true)
      (`self.SetSlotState` _returnvalue (struct :`TagName` "Player.Slot.Joined"))
      (`self.OnPlayerSlotsChanged`)
      (return true)
      (else
        _)))
  (return false))

(fn `LeaveSlot`
  (params (Controller :type "PlayerController Object Reference"))
  (returns (Left :type Boolean))
  (bind _returnvalue (`KismetArrayLibrary.Array_Find` (`self.SlotControllers`) Controller))
  (if (> _returnvalue 0)
    (if (`BlueprintGameplayTagLibrary.MatchesTag` (`|GetArrayItem` (`self.SlotStates`) _returnvalue) (struct :`TagName` "Player.Slot.Joined") true)
      (if (`|GetArrayItem` (`self.SlotIsDebug`) _returnvalue)
        (`self.ReleaseSlot` _returnvalue)
        (else
          (`self.SetSlotState` _returnvalue (struct :`TagName` "Player.Slot.Connected"))
          (`self.ClearSlotBallType` _returnvalue)))
      (`self.OnPlayerSlotsChanged`)
      (return true)
      (else
        _)))
  (return false))

(fn `OpenJoinSession`
  (params (PrimaryController :type "PlayerController Object Reference"))
  (set `self.JoinSessionOpen` true)
  (`self.ResetSlots`)
  (`self.SetSlot` 0 PrimaryController (struct :`TagName` "Player.Slot.Joined"))
  (`self.RegisterConnectedControllers`)
  (`self.OnPlayerSlotsChanged`))

(fn `PickWeightedBallType`
  (returns (BallType :type "/Game/Blueprint/Ball/Data/PDA_BallType Object Reference"))
  (locals (ValidBallTypes :type "Array of /Game/Blueprint/Ball/Data/PDA_BallType Object Reference"))
  (`KismetArrayLibrary.Array_Clear` (`local.ValidBallTypes`))
  (for _array_element (`self.SlotBallTypes`)
    (`/Engine/EditorBlueprintResources/StandardMacros.IsValid` _array_element
      (:`Is Valid`
        (`KismetArrayLibrary.Array_Add` (`local.ValidBallTypes`) _array_element))))
  (if (`KismetArrayLibrary.Array_IsEmpty` (`local.ValidBallTypes`))
    (return null)
    (else
      (return (`KismetArrayLibrary.Array_Random` (`local.ValidBallTypes`))))))

(fn `RegisterConnectedControllers`
  (bind _outinputdevices (`InputDeviceLibrary.GetAllConnectedInputDevices`))
  (for _array_element _outinputdevices
    (bind _returnvalue (`InputDeviceLibrary.GetUserForInputDevice` _array_element))
    (`self.RegisterControllerForUser` _returnvalue)))

(fn `RegisterControllerForUser`
  (params (UserId :type "PlatformUserId Structure"))
  (if (not (not (`self.JoinSessionOpen`)))
    (bind _returnvalue (`InputDeviceLibrary.GetPlayerControllerFromPlatformUser` UserId))
    (`/Engine/EditorBlueprintResources/StandardMacros.IsValid` _returnvalue
      (:`Is Valid`
        (`self.AssignControllerToFreeSlot` _returnvalue))
      (:`Is Not Valid`
        (bind _freeslotindex (`self.FindFreeSlot`))
        (if (> _freeslotindex 0)
          (bind _returnvalue_2 (`GameplayStatics.CreatePlayerFromPlatformUser` UserId))
          (`self.SetSlot` _freeslotindex _returnvalue_2 (struct :`TagName` "Player.Slot.Connected")))))))

(fn `ReleaseSlot`
  (params (SlotIndex :type Integer))
  (locals (ReleasedController :type "PlayerController Object Reference"))
  (if (not (<= SlotIndex 0))
    (set `local.ReleasedController` (`|GetArrayItem` (`self.SlotControllers`) SlotIndex))
    (`self.SetSlot` SlotIndex null (struct :`TagName` "Player.Slot.Empty"))
    (`KismetArrayLibrary.Array_Set` (`self.SlotIsDebug`) SlotIndex)
    (`self.ClearSlotBallType` (`local.SlotIndex`))
    (`/Engine/EditorBlueprintResources/StandardMacros.IsValid` (`local.ReleasedController`)
      (:`Is Valid`
        (`GameplayStatics.RemovePlayer` (`local.ReleasedController`) true)))))

(fn `ResetSlots`
  (`KismetArrayLibrary.Array_Resize` (`self.SlotControllers`) (`self.MaxPlayers`))
  (`KismetArrayLibrary.Array_Resize` (`self.SlotStates`) (`self.MaxPlayers`))
  (`KismetArrayLibrary.Array_Resize` (`self.SlotIsDebug`) (`self.MaxPlayers`))
  (for _index (range (`self.MaxPlayers`))
    (`self.SetSlot` _index null (struct :`TagName` "Player.Slot.Empty"))
    (`KismetArrayLibrary.Array_Set` (`self.SlotIsDebug`) _index))
  (`KismetArrayLibrary.Array_Clear` (`self.SlotBallTypes`)))

(fn `ResumeJoinSession`
  (set `self.JoinSessionOpen` true)
  (`self.OnPlayerSlotsChanged`))

(fn `SetSlot`
  (params (SlotIndex :type Integer) (Controller :type "PlayerController Object Reference") (State :type "GameplayTag Structure"))
  (`KismetArrayLibrary.Array_Set` (`self.SlotControllers`) SlotIndex Controller)
  (`KismetArrayLibrary.Array_Set` (`self.SlotStates`) SlotIndex State)
  (`/Engine/EditorBlueprintResources/StandardMacros.IsValid` Controller
    (:`Is Valid`
      (`KismetArrayLibrary.Array_Set` (`self.SlotControllerIds`) SlotIndex (`GameplayStatics.GetPlayerControllerID` Controller) true))
    (:`Is Not Valid`
      (`KismetArrayLibrary.Array_Set` (`self.SlotControllerIds`) SlotIndex -1 true))))

(fn `SetSlotState`
  (params (SlotIndex :type Integer) (State :type "GameplayTag Structure"))
  (`KismetArrayLibrary.Array_Set` (`self.SlotStates`) SlotIndex State))

(fn `StoreSlotBallType`
  (params (SlotIndex :type Integer) (BallType :type "/Game/Blueprint/Ball/Data/PDA_BallType Object Reference"))
  (`KismetArrayLibrary.Array_Set` (`self.SlotBallTypes`) SlotIndex BallType true))