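; Master ranged equipment Blueprint for an extinguisher-style tool that fires dowsing volumes from a bone on its mesh.
; While in shooting position, triggered input spawns an extinguisher volume aimed by a trace toward a randomly jittered screen-center point.
; Start/stop input toggles the character's shooting flag and audio; both enable collision on the hidden foam cone attached at the nozzle.
; An unjittered two-trace legacy aiming function remains, uncalled here.
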(event `self.ReceiveBeginPlay`
  (`parent.ReceiveBeginPlay`)
  (bind _asbp_dowsing_volume_static_cone (cast `/Game/Blueprint/DowsingVolumes/BP_DowsingVolume_StaticCone` (`ChildActorComponent.ChildActor` (`self.ChildActor`))))
  (bind _output_get (set `self.As BP Dowsing Volume Static Cone` _asbp_dowsing_volume_static_cone))
  (bind _sm_foam (`/Game/Blueprint/DowsingVolumes/BP_Master_DowsingVolume.SM_Foam` _output_get))
  (`SceneComponent.K2_AttachToComponent` _sm_foam (`self.SK_Equipment`) "Nuzzle" "SnapToTarget" "SnapToTarget" "KeepWorld" true)
  (`PrimitiveComponent.SetCollisionEnabled` _sm_foam "NoCollision")
  (`SceneComponent.SetHiddenInGame` _sm_foam true false))

(event `Shooting Triggered`
  (bind _as_bp_generic_character (`self.As BP Generic Character`))
  ;[1 0 0.06535 0.5] Input Shooting
  (if (`/Game/Blueprint/Character/Master/BP_GenericCharacter.InShootingPosition` (`self.As BP Generic Character`))
    (bind (_traceorigine _traceend) (`self.ShootingRaytrace`))
    (`|SpawnActorFromClass` "/Game/Blueprint/DowsingVolumes/BP_DowsingVolume_Extinguisher.BP_DowsingVolume_Extinguisher_C" (`KismetMathLibrary.MakeTransform` _traceorigine (`KismetMathLibrary.FindLookAtRotation` _traceorigine _traceend)) "Undefined" "MultiplyWithRoot" _as_bp_generic_character _as_bp_generic_character)))

(event `Shooting Started`
  ;[1 0 0.06535 0.5] Input Shooting
  (set `/Game/Blueprint/Character/Master/BP_GenericCharacter.IsShooting` true (`self.As BP Generic Character`))
  (`PrimitiveComponent.SetCollisionEnabled` (`/Game/Blueprint/DowsingVolumes/BP_Master_DowsingVolume.SM_Foam` (`self.As BP Dowsing Volume Static Cone`)) "QueryAndPhysics")
  (bind _returnvalue (`AddComponent|NODE_AddAudioComponent-0`))
  (set `self.SFX Component` _returnvalue))

(event `Shooting Completed`
  ;[1 0 0.06535 0.5] Input Shooting
  (set `/Game/Blueprint/Character/Master/BP_GenericCharacter.IsShooting` false (`self.As BP Generic Character`))
  (`PrimitiveComponent.SetCollisionEnabled` (`/Game/Blueprint/DowsingVolumes/BP_Master_DowsingVolume.SM_Foam` (`self.As BP Dowsing Volume Static Cone`)) "QueryAndPhysics")
  (`AudioComponent.Stop` (`self.SFX Component`)))

(fn `ShootingRaytrace`
  (returns (TraceOrigine :type "Vector Structure") (TraceEnd :type "Vector Structure") (OutHit :type "HitResult Structure") (`Return Value` :type Boolean))
  (bind _returnvalue (`GameplayStatics.GetPlayerController` 0))
  (bind _random_treshold (`self.Random Treshold`))
  (bind (_sizex _sizey) (`PlayerController.GetViewportSize` _returnvalue))
  (bind _returnvalue_location (`KismetMathLibrary.BreakTransform` (`SkinnedMeshComponent.GetBoneTransform` (`self.SK_Equipment`) (`self.SourceOfBoneProjectile`) "RTS_World")))
  (bind _returnvalue_2 (`KismetMathLibrary.Conv_IntToDouble` (/ _sizey 2)))
  (bind _returnvalue_3 (`KismetMathLibrary.Conv_IntToDouble` (/ _sizex 2)))
  (bind (_worldposition _worlddirection) (`GameplayStatics.DeprojectScreenToWorld` _returnvalue (`KismetMathLibrary.MakeVector2D` (`KismetMathLibrary.RandomFloatInRange` (- _returnvalue_3 _random_treshold) (+ _returnvalue_3 _random_treshold)) (`KismetMathLibrary.RandomFloatInRange` (- _returnvalue_2 _random_treshold) (+ _returnvalue_2 _random_treshold)))))
  (bind _returnvalue_4 (+ _worldposition (* (`self.Shooting Range`) _worlddirection)))
  (bind (_outhit _returnvalue_5) (`KismetSystemLibrary.LineTraceSingle` _returnvalue_location _returnvalue_4 "TraceTypeQuery1" false (`|MakeArray` (`GameplayStatics.GetPlayerPawn` 0) (`GameplayStatics.GetPlayerPawn` 1) :!type "Actor Object Reference") "None" true (struct :`R` 1.0 :`B` 0.836866 :`A` 1.0)))
  (bind (_bblockinghit _binitialoverlap _time _distance _location _impactpoint) (`GameplayStatics.BreakHitResult` _outhit))
  (return _returnvalue_location (select `bool` _bblockinghit :`false` _returnvalue_4 :`true` _impactpoint) _outhit _returnvalue_5))

(fn `ShootingRaytrace_Legacy`
  (returns (TraceOrigine :type "Vector Structure") (TraceEnd :type "Vector Structure") (OutHit :type "HitResult Structure") (`Return Value` :type Boolean))
  (bind _returnvalue (`GameplayStatics.GetPlayerController` 0))
  (bind (_sizex _sizey) (`PlayerController.GetViewportSize` _returnvalue))
  (bind _returnvalue_location (`KismetMathLibrary.BreakTransform` (`SkinnedMeshComponent.GetBoneTransform` (`self.SK_Equipment`) (`self.SourceOfBoneProjectile`) "RTS_World")))
  (bind (_worldposition _worlddirection) (`GameplayStatics.DeprojectScreenToWorld` _returnvalue (`KismetMathLibrary.MakeVector2D` (`KismetMathLibrary.Conv_IntToDouble` (/ _sizex 2)) (`KismetMathLibrary.Conv_IntToDouble` (/ _sizey 2)))))
  (bind _returnvalue_2 (+ _worldposition (* (`self.Shooting Range`) _worlddirection)))
  (bind (_outhit _returnvalue_3) (`KismetSystemLibrary.LineTraceSingle` _worldposition _returnvalue_2 "TraceTypeQuery1" true (`|MakeArray` (`GameplayStatics.GetPlayerPawn` 0) :!type "Actor Object Reference") "ForOneFrame"))
  (bind _returnvalue_4 (select `bool` _returnvalue_3 :`false` _returnvalue_2 :`true` (`.ImpactPoint` (`GameplayStatics.BreakHitResult` _outhit))))
  (bind (_outhit_2 _returnvalue_5) (`KismetSystemLibrary.LineTraceSingle` _returnvalue_location _returnvalue_4 "TraceTypeQuery1" false (`|MakeArray` (`GameplayStatics.GetPlayerPawn` 0) :!type "Actor Object Reference") "None" true (struct :`R` 1.0 :`B` 0.836866 :`A` 1.0)))
  (return _returnvalue_location _returnvalue_4 _outhit_2 _returnvalue_5))

(fn `UserConstructionScript`
  (`parent.UserConstructionScript`))