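; Base Blueprint for dowsing volumes, moving sphere-collision actors with foam behavior that depends on rotation.
; A hit-scan function multi-sphere traces at twice the collision radius from the previous location to a velocity-derived point near the current one, ignoring owner and player.
; It stores the location for the next trace and returns the hits.
; The FoamAngleBehavior macro sorts rotation roll into flat-floor, wall-drip or ceiling-drop outputs.
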(fn `MultiHitScanVelocityTrace`
  (returns (OutHits :type "Array of HitResult Structure") (ReturnValue :type Boolean))
  (bind _returnvalue (`self.K2_GetActorLocation`))
  (bind (_outhits _returnvalue_2) (`KismetSystemLibrary.SphereTraceMulti` (`self.Previous Location`) (+ _returnvalue (* (`KismetMathLibrary.GetDirectionUnitVector` _returnvalue (* (`GameplayStatics.GetWorldDeltaSeconds`) (`self.GetVelocity`))) 15.0)) (* (`SphereComponent.SphereRadius` (`self.SphereCollision`)) 2.0) "TraceTypeQuery1" true (`|MakeArray` (`self.GetOwner`) (`GameplayStatics.GetPlayerCharacter` 0) :!type "Actor Object Reference")))
  (set `self.Previous Location` (`self.K2_GetActorLocation`))
  (return _outhits _returnvalue_2))

(fn `UserConstructionScript`)