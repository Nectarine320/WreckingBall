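; Extinguisher foam projectile, a dowsing volume that launches with randomized speed and size and wobbles in flight through a looping scale timeline.
; Tick runs a velocity-based multi-trace until a blocking hit stops movement and snaps the foam to the surface normal.
; After a randomized lifetime, a timeline shrinks it from a flattened scale while sinking it, then destroys it.
; A FoamAngleBehavior macro sorts roll into floor, wall or ceiling, but is unused here.
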(event `self.ReceiveBeginPlay`
  (bind _projectilemovement (`self.ProjectileMovement`))
  ;[0 0.1529 1 0.5] Begin Play
  (set `self.Previous Location` (`self.K2_GetActorLocation`))
  (set `ProjectileMovementComponent.InitialSpeed` (* (`ProjectileMovementComponent.InitialSpeed` _projectilemovement) (`KismetMathLibrary.RandomFloatInRange` 1.0 1.25)) _projectilemovement)
  (bind _output_get (set `self.InitialScale` (`KismetMathLibrary.Conv_DoubleToVector` (`KismetMathLibrary.RandomFloatInRange` 0.25 0.6))))
  (`SceneComponent.SetRelativeScale3D` (`self.SM_Foam_0`) _output_get)
  (`self.AnimAirBlob`)
  (`self.SetActorTickEnabled` true))

(event `AnimAirBlob`
  (bind (_initialscale_x _initialscale_y _initialscale_z) (`KismetMathLibrary.BreakVector` (`self.InitialScale`)))
  (bind _returnvalue (`KismetMathLibrary.RandomFloatInRange` (`self.MinMultiplier`) (`self.MaxMultiplier`)))
  ;[2 1.759 0.1667 0.5] In Air Animation
  (bind (_direction _blobbyinairanimation) (`Timeline|In Air Blob` :!label _label)
    (:`Update`
      (set `self.Blobby in Air Animation` _blobbyinairanimation)
      (bind _output_get (set `self.CurrentScale` (`KismetMathLibrary.VLerp` (`self.InitialScale`) (`self.BlobRandomScale`) _blobbyinairanimation)))
      (`SceneComponent.SetRelativeScale3D` (`self.SM_Foam_0`) _output_get))
    (:`BeginingLoop`
      (set `self.BlobRandomScale` (`KismetMathLibrary.MakeVector` (* _initialscale_x _returnvalue) (* _initialscale_y _returnvalue) (* _initialscale_z _returnvalue))))))

(event `StopAnimAirBlob`
  ;[2 1.759 0.1667 0.5] In Air Animation
  (goto _label :!via `Stop`))

(event `AnimFlatBlob`
  ;[2 1.759 0.1667 0.5] Landing Flat Animation
  (`KismetSystemLibrary.Delay` (* (`self.FoamLife`) (`KismetMathLibrary.RandomFloatInRange` 0.9 1.2)))
  (`self.Anim Death`))

(event `Anim Death`
  (bind (_currentscale_x _currentscale_y _currentscale_z) (`KismetMathLibrary.BreakVector` (`self.CurrentScale`)))
  (bind _flatmodifierxy (`self.FlatModifierXY`))
  (bind _returnvalue (`KismetMathLibrary.MakeVector` (* _currentscale_x _flatmodifierxy) (* _currentscale_y _flatmodifierxy) (* _currentscale_z 1.0)))
  ;[2 1.759 0.1667 0.5] Drying Out Animation
  (`TimelineComponent.SetPlayRate` (`self.DeathAnimTimeline`) (`KismetMathLibrary.RandomFloatInRange` 0.9 1.2))
  (bind (_direction _xy _z) (`Timeline|DeathAnimTimeline`)
    (:`Update`
      (bind (_returnvalue_x _returnvalue_y) (`KismetMathLibrary.BreakVector` (`KismetMathLibrary.VLerp` _returnvalue (0.01 0.01 0.01) _z)))
      (bind (_returnvalue_x_2 _returnvalue_y_2 _returnvalue_z) (`KismetMathLibrary.BreakVector` (`KismetMathLibrary.VLerp` _returnvalue (0.01 0.01 0.01) _xy)))
      (`SceneComponent.SetRelativeScale3D` (`self.SM_Foam_0`) (`KismetMathLibrary.MakeVector` _returnvalue_x _returnvalue_y _returnvalue_z))
      (`self.K2_SetActorLocation` (- (`self.K2_GetActorLocation`) (0.0 0.0 0.35))))
    (:`Finished`
      (`self.K2_DestroyActor`))))

(event `Trigger Projectile Tick`)

(event `self.ReceiveTick`
  (params (DeltaSeconds :type "Float (single-precision)"))
  (bind _projectilemovement (`self.ProjectileMovement`))
  (bind (_bblockinghit _binitialoverlap _time _distance _location _impactpoint _normal) (`GameplayStatics.BreakHitResult` (`self.Out Hit`)))
  (if (`self.HasImpacted`)
    (`self.SetActorTickEnabled` false)
    (else
      (bind (_outhits _returnvalue) (`self.MultiHitScanVelocityTrace`))
      (if _returnvalue
        (for _array_element _outhits :!label _label_2
          (bind _output_get (set `self.Out Hit` _array_element))
          (bind _output_get_2 (set `self.Hit Actor` (`.HitActor` (`GameplayStatics.BreakHitResult` _output_get))))
          (if (and (or (not (== (`self.GetOwner`) _output_get_2)) (not (== _output_get_2 (cast `/Game/Blueprint/DowsingVolumes/BP_Master_DowsingVolume` _output_get_2 :!pure true)))) _bblockinghit)
            (`MovementComponent.StopMovementImmediately` _projectilemovement)
            (`ProjectileMovementComponent.StopSimulating` _projectilemovement (`self.Out Hit`))
            (`self.StopAnimAirBlob`)
            (`self.AnimFlatBlob`)
            (bind _output_get_3 (set `self.ImpactAngle` (`KismetMathLibrary.MakeRotFromZ` _normal)))
            (`self.K2_SetActorLocationAndRotation` _impactpoint _output_get_3 false true)
            (set `self.HasImpacted` true)
            (`self.stop loop`)))))))

(event `stop loop`
  (goto _label_2 :!via `Break`))

(fn `UserConstructionScript`)