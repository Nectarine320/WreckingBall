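; Front-end player controller for local multiplayer menus, handling slot join/leave and ball selection input.
; Swaps Enhanced Input mapping contexts, giving player one CommonUI-based contexts and other players their own, retrying setup next tick until the subsystem exists.
; Routes join, leave and debug fake-player toggles to GI_Core, and relays selection input by slot to WBP_BallSelection.
; Player one's gamepad presses restore lost focus on the top menu screen.
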(event `self.ReceiveBeginPlay`
  ;[0 0.1529 1 0.5] Begin Play / Initializer
  (`self.InitializeFrontEndInput`))

(event `EnhancedInput|/Game/Blueprint/PlayerController/Input/UI/Actions/IA_Join`
  (params (ActionValue :type Boolean) (ElapsedSeconds :type "Float (double-precision)") (TriggeredSeconds :type "Float (double-precision)") (InputAction :type "InputAction Object Reference" :default "/Game/Blueprint/PlayerController/Input/UI/Actions/IA_Join.IA_Join"))
  ;[1 0 0.06535 0.5] On Joinned / Left Input
  (:`Started`
    (bind _asgi_core (cast `/Game/Blueprint/Core/GI_Core` (`GameplayStatics.GetGameInstance`)))
    (`/Game/Blueprint/Core/GI_Core.JoinSlot` _asgi_core self)))

(event `Key|F2`
  (params (Key :type "Key Structure"))
  ; DEBUG BUTTONS
  (:`Pressed`
    (`self.DebugTogglePlayerSlot` 1)))

(event `Key|F3`
  (params (Key :type "Key Structure"))
  ; DEBUG BUTTONS
  (:`Pressed`
    (`self.DebugTogglePlayerSlot` 2)))

(event `EnhancedInput|/Game/Blueprint/PlayerController/Input/UI/Actions/IA_Leave`
  (params (ActionValue :type Boolean) (ElapsedSeconds :type "Float (double-precision)") (TriggeredSeconds :type "Float (double-precision)") (InputAction :type "InputAction Object Reference" :default "/Game/Blueprint/PlayerController/Input/UI/Actions/IA_Leave.IA_Leave"))
  ;[1 0 0.06535 0.5] On Joinned / Left Input
  (:`Started`
    (bind _asgi_core (cast `/Game/Blueprint/Core/GI_Core` (`GameplayStatics.GetGameInstance`)))
    (`/Game/Blueprint/Core/GI_Core.LeaveSlot` _asgi_core self)))

(event `Key|F4`
  (params (Key :type "Key Structure"))
  ; DEBUG BUTTONS
  (:`Pressed`
    (`self.DebugTogglePlayerSlot` 3)))

(event `EnhancedInput|/Game/Blueprint/PlayerController/Input/UI/Actions/IA_Select_Left`
  (params (ActionValue :type Boolean) (ElapsedSeconds :type "Float (double-precision)") (TriggeredSeconds :type "Float (double-precision)") (InputAction :type "InputAction Object Reference" :default "/Game/Blueprint/PlayerController/Input/UI/Actions/IA_Select_Left.IA_Select_Left"))
  ;[1 0 0.06535 0.5] Menu Selection
  (:`Started`
    (`self.RelayBallNavigate` -1)))

(event `EnhancedInput|/Game/Blueprint/PlayerController/Input/UI/Actions/IA_Select_Right`
  (params (ActionValue :type Boolean) (ElapsedSeconds :type "Float (double-precision)") (TriggeredSeconds :type "Float (double-precision)") (InputAction :type "InputAction Object Reference" :default "/Game/Blueprint/PlayerController/Input/UI/Actions/IA_Select_Right.IA_Select_Right"))
  ;[1 0 0.06535 0.5] Menu Selection
  (:`Started`
    (`self.RelayBallNavigate` 1)))

(event `EnhancedInput|/Game/Blueprint/PlayerController/Input/UI/Actions/IA_Select_Accept`
  (params (ActionValue :type Boolean) (ElapsedSeconds :type "Float (double-precision)") (TriggeredSeconds :type "Float (double-precision)") (InputAction :type "InputAction Object Reference" :default "/Game/Blueprint/PlayerController/Input/UI/Actions/IA_Select_Accept.IA_Select_Accept"))
  ;[1 0 0.06535 0.5] Menu Selection
  (:`Started`
    (`self.RelayBallAccept`)))

(event `EnhancedInput|/Game/Blueprint/PlayerController/Input/UI/Actions/IA_Select_Back`
  (params (ActionValue :type Boolean) (ElapsedSeconds :type "Float (double-precision)") (TriggeredSeconds :type "Float (double-precision)") (InputAction :type "InputAction Object Reference" :default "/Game/Blueprint/PlayerController/Input/UI/Actions/IA_Select_Back.IA_Select_Back"))
  ;[1 0 0.06535 0.5] Menu Selection
  (:`Started`
    (`self.RelayBallBack`)))

(event `Key|AnyKey` :consume false
  (params (Key :type "Key Structure"))
  ;[1 0 0.06535 0.5] Widget Focus
  (:`Pressed`
    (`self.RestoreMenuFocus` Key)))

(fn `DebugTogglePlayerSlot`
  (params (SlotIndex :type Integer))
  (bind _asgi_core (cast `/Game/Blueprint/Core/GI_Core` (`GameplayStatics.GetGameInstance`)))
  (`/Game/Blueprint/Core/GI_Core.DebugToggleFakePlayer` _asgi_core SlotIndex))

(fn `FindBallSelectionScreen`
  (returns (Screen :type "/Game/Blueprint/UI/Menu/WBP_BallSelection Object Reference"))
  (bind _foundwidgets (`WidgetBlueprintLibrary.GetAllWidgetsOfClass` "/Game/Blueprint/UI/Menu/WBP_BallSelection.WBP_BallSelection_C" false))
  (if (> (`KismetArrayLibrary.Array_Length` _foundwidgets) 0)
    (return (`|GetArrayItem` _foundwidgets))
    (else
      (return null))))

(fn `FindOwnSlotIndex`
  (returns (SlotIndex :type Integer))
  (if (== self (`GameplayStatics.GetPlayerController` 0))
    (return 0)
    (else
      (bind _asgi_core (cast `/Game/Blueprint/Core/GI_Core` (`GameplayStatics.GetGameInstance`))
        (:`then`
          (bind _slotindex (`/Game/Blueprint/Core/GI_Core.FindSlotOfController` _asgi_core self))
          (return _slotindex))
        (:`CastFailed`
          (return -1))))))

(fn `InitializeFrontEndInput`
  (`/Engine/EditorBlueprintResources/StandardMacros.IsValid` (pcsubsystem `EnhancedInputLocalPlayerSubsystem` self)
    (:`Is Valid`
      (`EnhancedInputSubsystemInterface.AddMappingContext` (pcsubsystem `EnhancedInputLocalPlayerSubsystem` self) (select `bool` (== self (`GameplayStatics.GetPlayerController` 0)) :`false` "/Game/Blueprint/PlayerController/Input/UI/IMC_FrontEnd.IMC_FrontEnd" :`true` "/Game/Blueprint/PlayerController/Input/UI/IMC_CommonUI.IMC_CommonUI" :!type "InputMappingContext Object Reference") 0 (struct)))
    (:`Is Not Valid`
      (`KismetSystemLibrary.K2_SetTimerForNextTick` self "InitializeFrontEndInput"))))

(fn `RelayBallAccept`
  (bind _screen (`self.FindBallSelectionScreen`))
  (bind _slotindex (`self.FindOwnSlotIndex`))
  (`/Engine/EditorBlueprintResources/StandardMacros.IsValid` _screen
    (:`Is Valid`
      (`/Game/Blueprint/UI/Menu/WBP_BallSelection.HandlePlayerAccept` _screen _slotindex))))

(fn `RelayBallBack`
  (bind _screen (`self.FindBallSelectionScreen`))
  (bind _slotindex (`self.FindOwnSlotIndex`))
  (`/Engine/EditorBlueprintResources/StandardMacros.IsValid` _screen
    (:`Is Valid`
      (`/Game/Blueprint/UI/Menu/WBP_BallSelection.HandlePlayerBack` _screen _slotindex))))

(fn `RelayBallNavigate`
  (params (Direction :type Integer))
  (bind _screen (`self.FindBallSelectionScreen`))
  (bind _slotindex (`self.FindOwnSlotIndex`))
  (`/Engine/EditorBlueprintResources/StandardMacros.IsValid` _screen
    (:`Is Valid`
      (`/Game/Blueprint/UI/Menu/WBP_BallSelection.HandlePlayerNavigate` _screen _slotindex (`local.Direction`)))))

(fn `RestoreMenuFocus`
  (params (Key :type "Key Structure" :default "None"))
  (if (and (`KismetInputLibrary.Key_IsGamepadKey` (`local.Key`)) (== self (`GameplayStatics.GetPlayerController` 0)))
    (bind _widget (`/Game/Blueprint/UI/BPFL_UI.PeekContentOnLayer` self (struct :`TagName` "UI.Layer.Menu")))
    (bind _aswbp_menu_screen_base (cast `/Game/Blueprint/UI/Common/WBP_MenuScreenBase` _widget))
    (if (not (`Widget.HasUserFocusedDescendants` _aswbp_menu_screen_base self))
      (bind _focustargetwidget (`/Game/Blueprint/UI/Common/WBP_MenuScreenBase.FocusTargetWidget` _aswbp_menu_screen_base))
      (`/Engine/EditorBlueprintResources/StandardMacros.IsValid` _focustargetwidget
        (:`Is Valid`
          (`/Game/Blueprint/UI/Common/WBP_MenuScreenBase.FocusMenuScreen` _aswbp_menu_screen_base _focustargetwidget))))))

(fn `SetBallSelectInputActive`
  (params (Active :type Boolean))
  (`/Engine/EditorBlueprintResources/StandardMacros.IsValid` (pcsubsystem `EnhancedInputLocalPlayerSubsystem` self)
    (:`Is Valid`
      (if (== self (`GameplayStatics.GetPlayerController` 0))
        (if (`local.Active`)
          (`EnhancedInputSubsystemInterface.AddMappingContext` (pcsubsystem `EnhancedInputLocalPlayerSubsystem` self) "/Game/Blueprint/PlayerController/Input/UI/IMC_BallSelectP1.IMC_BallSelectP1" 1 (struct))
          (else
            (`EnhancedInputSubsystemInterface.RemoveMappingContext` (pcsubsystem `EnhancedInputLocalPlayerSubsystem` self) "/Game/Blueprint/PlayerController/Input/UI/IMC_BallSelectP1.IMC_BallSelectP1" (struct))))
        (elif (`local.Active`)
          (`EnhancedInputSubsystemInterface.RemoveMappingContext` (pcsubsystem `EnhancedInputLocalPlayerSubsystem` self) "/Game/Blueprint/PlayerController/Input/UI/IMC_FrontEnd.IMC_FrontEnd" (struct))
          (`EnhancedInputSubsystemInterface.AddMappingContext` (pcsubsystem `EnhancedInputLocalPlayerSubsystem` self) "/Game/Blueprint/PlayerController/Input/UI/IMC_BallSelect.IMC_BallSelect" 0 (struct))
          (else
            (`EnhancedInputSubsystemInterface.RemoveMappingContext` (pcsubsystem `EnhancedInputLocalPlayerSubsystem` self) "/Game/Blueprint/PlayerController/Input/UI/IMC_BallSelect.IMC_BallSelect" (struct))
            (`EnhancedInputSubsystemInterface.AddMappingContext` (pcsubsystem `EnhancedInputLocalPlayerSubsystem` self) "/Game/Blueprint/PlayerController/Input/UI/IMC_FrontEnd.IMC_FrontEnd" 0 (struct))))))))

(fn `UserConstructionScript`)