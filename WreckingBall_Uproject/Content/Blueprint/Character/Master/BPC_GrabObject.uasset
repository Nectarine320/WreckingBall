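; Character component that handles picking up, carrying, dropping and throwing NPCs, equipment and physics objects.
; Pickup triggers any current interactable, then, if empty-handed, searches sphere overlaps in priority order: pawn, equipment, physics body.
; Drop, shoot and attack inputs act on the held type, throwing it or driving melee and ranged equipment.
; A looping timer moves physics-handle objects using mass-dependent sway, velocity lag, spring-smoothed camera lag and tilt.
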(event `Initialize Update Grab Item Position`
  ;[0 0.1529 1 0.5] Initialize Grab Item Position
  (bind _returnvalue (`KismetSystemLibrary.K2_SetTimerDelegate` (delegate `Update Grab Item Position`) 0.001 true true))
  (set `self.Timer Update Grab Item Position` _returnvalue))

(event `self.ReceiveBeginPlay`
  ;[0 0.1529 1 0.5] Begin Play
  (bind _asbp_generic_character (cast `/Game/Blueprint/Character/Master/BP_GenericCharacter` (`self.GetOwner`)))
  (set `self.As BP Generic Character` _asbp_generic_character)
  (`self.Initialize Update Grab Item Position`)
  (bind _asplayer_controller (cast `PlayerController` (`Pawn.GetController` (`self.As BP Generic Character`))))
  (bind _returnvalue (pcsubsystem `EnhancedInputLocalPlayerSubsystem` _asplayer_controller))
  (`/Engine/EditorBlueprintResources/StandardMacros.IsValid` _returnvalue
    (:`Is Valid`
      (`EnhancedInputSubsystemInterface.AddMappingContext` _returnvalue "/Game/Input/IMC_PickupPhysicObject.IMC_PickupPhysicObject" 1 (struct)))))

(event `EnhancedInput|/Game/Input/Actions/IA_Pickup`
  (params (ActionValue :type Boolean) (ElapsedSeconds :type "Float (double-precision)") (TriggeredSeconds :type "Float (double-precision)") (InputAction :type "InputAction Object Reference" :default "/Game/Input/Actions/IA_Pickup.IA_Pickup"))
  (bind _as_bp_generic_character (`self.As BP Generic Character`))
  ;[1 0 0.06535 0.5] PickUp Input
  (:`Started`
    (`/Engine/EditorBlueprintResources/StandardMacros.IsValid` _as_bp_generic_character
      (:`Is Valid`
        (`self.Interactable` _as_bp_generic_character)
        (if (not (`self.Grabbing`))
          (`self.PickUpHierarchy`))))))

(event `Update Grab Item Position`
  ;[0 1 0.07739 0.5] Update Grab Item Position
  (`self.UpdatePhysicActorPosition`))

(event `EnhancedInput|/Game/Input/Actions/IA_DropItem`
  (params (ActionValue :type Boolean) (ElapsedSeconds :type "Float (double-precision)") (TriggeredSeconds :type "Float (double-precision)") (InputAction :type "InputAction Object Reference" :default "/Game/Input/Actions/IA_DropItem.IA_DropItem"))
  (bind _handequipement (`/Game/Blueprint/Character/Master/BP_GenericCharacter.HandEquipement` (`self.As BP Generic Character`)))
  ;[1 0 0.06535 0.5] PickUp Input
  (:`Started`
    (if (`self.Grabbing`)
      (switch `/Game/Blueprint/Character/Master/E_PickUpType` (`self.PickUpType`)
        (:`NewEnumerator0`
          (`/Game/Blueprint/Character/Player/BP_PlayerFireMan.DropRescue` (`self.As BP Player Fire Man`) false)
          (set `self.Grabbing` false))
        (:`NewEnumerator1`
          (`/Engine/EditorBlueprintResources/StandardMacros.IsValid` _handequipement
            (:`Is Valid`
              (`/Game/Blueprint/Equipement/Master/BP_Master_Equipement.Drop Item` _handequipement)
              (set `self.Grabbing` false))))
        (:`NewEnumerator2`
          (`PhysicsHandleComponent.ReleaseComponent` (`/Game/Blueprint/Character/Master/BP_GenericCharacter.PhysicsHandle` (`self.As BP Generic Character`)))
          (`self.ClearPhysicActorData`))))))

(event `EnhancedInput|/Game/Input/Actions/IA_Attack`
  (params (ActionValue :type Boolean) (ElapsedSeconds :type "Float (double-precision)") (TriggeredSeconds :type "Float (double-precision)") (InputAction :type "InputAction Object Reference" :default "/Game/Input/Actions/IA_Attack.IA_Attack"))
  (:`Started`
    (bind _asbp_equipment_melee (cast `/Game/Blueprint/Equipement/Master/BP_Equipment_Melee` (`/Game/Blueprint/Character/Master/BP_GenericCharacter.HandEquipement` (`self.As BP Generic Character`))))
    (`/Game/Blueprint/Equipement/Master/BP_Equipment_Melee.HittingStart` _asbp_equipment_melee))
  (:`Canceled`
    (bind _asbp_equipment_melee_2 (cast `/Game/Blueprint/Equipement/Master/BP_Equipment_Melee` (`/Game/Blueprint/Character/Master/BP_GenericCharacter.HandEquipement` (`self.As BP Generic Character`)) :!label _label))
    (`/Game/Blueprint/Equipement/Master/BP_Equipment_Melee.HittingComplete` _asbp_equipment_melee_2))
  (:`Completed`
    (goto _label)))

(event `EnhancedInput|/Game/Input/Actions/IA_Shoot`
  (params (ActionValue :type Boolean) (ElapsedSeconds :type "Float (double-precision)") (TriggeredSeconds :type "Float (double-precision)") (InputAction :type "InputAction Object Reference" :default "/Game/Input/Actions/IA_Shoot.IA_Shoot"))
  (:`Triggered`
    (switch `/Game/Blueprint/Character/Master/E_PickUpType` (`self.PickUpType`)
      (:`NewEnumerator1`
        (bind _asbp_equipement_range (cast `/Game/Blueprint/Equipement/Master/BP_Equipement_Range` (`/Game/Blueprint/Character/Master/BP_GenericCharacter.HandEquipement` (`self.As BP Generic Character`))))
        (`/Game/Blueprint/Equipement/Master/BP_Equipement_Range.Shooting Triggered` _asbp_equipement_range))))
  (:`Started`
    (if (`self.Grabbing`)
      (switch `/Game/Blueprint/Character/Master/E_PickUpType` (`self.PickUpType`)
        (:`NewEnumerator0`
          (`/Game/Blueprint/Character/Player/BP_PlayerFireMan.DropRescue` (`self.As BP Player Fire Man`) true)
          (set `self.Grabbing` false))
        (:`NewEnumerator1`
          (switch `/Game/Blueprint/Character/Master/E_PickUpType` (`self.PickUpType`)
            (:`NewEnumerator1`
              (bind _asbp_equipement_range_2 (cast `/Game/Blueprint/Equipement/Master/BP_Equipement_Range` (`/Game/Blueprint/Character/Master/BP_GenericCharacter.HandEquipement` (`self.As BP Generic Character`))))
              (`/Game/Blueprint/Equipement/Master/BP_Equipement_Range.Shooting Started` _asbp_equipement_range_2))))
        (:`NewEnumerator2`
          (`self.ThrowPhysicActor`)
          (`self.ClearPhysicActorData`)))))
  (:`Completed`
    (switch `/Game/Blueprint/Character/Master/E_PickUpType` (`self.PickUpType`)
      (:`NewEnumerator1`
        (bind _asbp_equipement_range_3 (cast `/Game/Blueprint/Equipement/Master/BP_Equipement_Range` (`/Game/Blueprint/Character/Master/BP_GenericCharacter.HandEquipement` (`self.As BP Generic Character`))))
        (`/Game/Blueprint/Equipement/Master/BP_Equipement_Range.Shooting Completed` _asbp_equipement_range_3)))))

(event `Key|E`
  (params (Key :type "Key Structure"))
  (:`Pressed`
    (bind _returnvalue (`KismetSystemLibrary.K2_SetTimerDelegate` (delegate `Test bullet Shooting`) 0.033333 true true))
    (set `self.NewVar` _returnvalue)))

(event `Test bullet Shooting`
  (switch `/Game/Blueprint/Character/Master/E_PickUpType` (`self.PickUpType`)
    (:`NewEnumerator1`
      (bind _asbp_equipement_range (cast `/Game/Blueprint/Equipement/Master/BP_Equipement_Range` (`/Game/Blueprint/Character/Master/BP_GenericCharacter.HandEquipement` (`self.As BP Generic Character`))))
      (`/Game/Blueprint/Equipement/Master/BP_Equipement_Range.Shooting Triggered` _asbp_equipement_range)
      (if (`self.Grabbing`)
        (switch `/Game/Blueprint/Character/Master/E_PickUpType` (`self.PickUpType`)
          (:`NewEnumerator0`
            (`/Game/Blueprint/Character/Player/BP_PlayerFireMan.DropRescue` (`self.As BP Player Fire Man`) true)
            (set `self.Grabbing` false))
          (:`NewEnumerator1`
            (switch `/Game/Blueprint/Character/Master/E_PickUpType` (`self.PickUpType`)
              (:`NewEnumerator1`
                (bind _asbp_equipement_range_2 (cast `/Game/Blueprint/Equipement/Master/BP_Equipement_Range` (`/Game/Blueprint/Character/Master/BP_GenericCharacter.HandEquipement` (`self.As BP Generic Character`))))
                (`/Game/Blueprint/Equipement/Master/BP_Equipement_Range.Shooting Started` _asbp_equipement_range_2)))))))))

(fn `CalculateAngularLagVariation`
  (bind _returnvalue (`PrimitiveComponent.GetMass` (`self.Pick Up Actor Component`)))
  (bind (_asbp_player_fire_man _bsuccess) (cast `/Game/Blueprint/Character/Player/BP_PlayerFireMan` (`self.As BP Generic Character`) :!pure true))
  (if _bsuccess
    (bind _output_get (set `self.AngularLagVar` (+ (+ (* (`/Game/Blueprint/Character/Player/BP_PlayerFireMan.Delta X` _asbp_player_fire_man) _returnvalue (`self.AngularLagVariationMultiplier`) (`SceneComponent.GetRightVector` (`/Game/Blueprint/Character/Player/BP_PlayerFireMan.FollowCamera` _asbp_player_fire_man))) (* (`/Game/Blueprint/Character/Player/BP_PlayerFireMan.Delta Y` _asbp_player_fire_man) _returnvalue (`self.AngularLagVariationMultiplier`) (`SceneComponent.GetUpVector` (`/Game/Blueprint/Character/Player/BP_PlayerFireMan.FollowCamera` _asbp_player_fire_man)))) (`self.AngularLagVar`))))
    (bind _returnvalue_2 (`KismetMathLibrary.VectorSpringInterp` _output_get (0.0 0.0 0.0) (`self.Spring State`) 10.0 0.3 (`GameplayStatics.GetWorldDeltaSeconds`) 10.0))
    (set `self.AngularLagVar` _returnvalue_2)))

(fn `CalculateAngularTiltVariation`
  (bind (_y _z) (`self.CalculateAngularTiltVariationBasedOnCharacterVelocity`))
  (bind (_return_value_x__roll_ _return_value_y__pitch_ _return_value_z__yaw_) (`self.CalculateAngularTiltVariationBasedOnCameraRotation`))
  (if (`.bSuccess` (cast `/Game/Blueprint/Character/Player/BP_PlayerFireMan` (`self.As BP Generic Character`) :!pure true))
    (bind _output_get (set `self.AngularTiltVar` (`KismetMathLibrary.MakeRotator` _return_value_x__roll_ _return_value_y__pitch_ _return_value_z__yaw_)))
    (set `self.AngularTiltVar` (`KismetMathLibrary.RInterpTo` _output_get (`KismetMathLibrary.MakeRotator` _y _z) (`GameplayStatics.GetWorldDeltaSeconds`) 2.0))))

(fn `CalculateAngularTiltVariationBasedOnCameraRotation`
  (returns (`Return Value X (Roll)` :type "Float (double-precision)") (`Return Value Y (Pitch)` :type "Float (double-precision)") (`Return Value Z (Yaw)` :type "Float (double-precision)"))
  (bind _returnvalue (`self.InvertMassMultiplier`))
  (bind _cameraangulartiltmodifier (`self.CameraAngularTiltModifier`))
  (bind (_asbp_player_fire_man _bsuccess) (cast `/Game/Blueprint/Character/Player/BP_PlayerFireMan` (`self.As BP Generic Character`) :!pure true))
  (bind (_returnvalue_roll _returnvalue_pitch _returnvalue_yaw) (`KismetMathLibrary.BreakRotator` (`KismetMathLibrary.ComposeRotators` (`KismetMathLibrary.MakeRotator` (* (`/Game/Blueprint/Character/Player/BP_PlayerFireMan.Delta X` _asbp_player_fire_man) _cameraangulartiltmodifier _returnvalue) (* (`/Game/Blueprint/Character/Player/BP_PlayerFireMan.Delta Y` _asbp_player_fire_man) _cameraangulartiltmodifier _returnvalue)) (`self.AngularTiltVar`))))
  (if _bsuccess
    (return _returnvalue_roll _returnvalue_pitch _returnvalue_yaw)))

(fn `CalculateAngularTiltVariationBasedOnCharacterVelocity`
  (returns (Y :type "Float (double-precision)") (Z :type "Float (double-precision)"))
  (bind _as_bp_generic_character (`self.As BP Generic Character`))
  (bind _tiltrotationoffset (`self.TiltRotationOffset`))
  (bind (_returnvalue_roll _returnvalue_pitch _returnvalue_yaw) (`KismetMathLibrary.BreakRotator` (`Pawn.GetControlRotation` _as_bp_generic_character)))
  (bind _returnvalue (* _tiltrotationoffset -1.0))
  (bind _charactermovement (`Character.CharacterMovement` _as_bp_generic_character))
  (bind _maxwalkspeed (`CharacterMovementComponent.MaxWalkSpeed` _charactermovement))
  (bind (_returnvalue_x _returnvalue_y _returnvalue_z) (`KismetMathLibrary.BreakVector` (`KismetMathLibrary.LessLess_VectorRotator` (`MovementComponent.Velocity` _charactermovement) (`KismetMathLibrary.MakeRotator` 0.0 0.0 _returnvalue_yaw))))
  (bind _returnvalue_2 (* _maxwalkspeed -1.0))
  (return (`KismetMathLibrary.MapRangeClamped` _returnvalue_y _returnvalue_2 _maxwalkspeed _returnvalue _tiltrotationoffset) (`KismetMathLibrary.MapRangeClamped` _returnvalue_z _returnvalue_2 _maxwalkspeed _returnvalue _tiltrotationoffset)))

(fn `CalculateDesiredLocationForHeldPhysicActor`
  (bind _as_bp_generic_character (`self.As BP Generic Character`))
  (bind _desireddistancefromplayer (`self.DesiredDistanceFromPlayer`))
  (bind (_asbp_player_fire_man _bsuccess) (cast `/Game/Blueprint/Character/Player/BP_PlayerFireMan` _as_bp_generic_character :!pure true))
  (bind _capsulecomponent (`Character.CapsuleComponent` _as_bp_generic_character))
  (bind (_returnvalue_x _returnvalue_y _returnvalue_z) (`KismetMathLibrary.BreakVector` (`SceneComponent.GetForwardVector` _capsulecomponent)))
  (bind (_returnvalue_x_2 _returnvalue_y_2 _returnvalue_z_2) (`KismetMathLibrary.BreakVector` (`SceneComponent.GetForwardVector` (`/Game/Blueprint/Character/Player/BP_PlayerFireMan.FollowCamera` _asbp_player_fire_man))))
  (set `self.DesiredLocationForHeldObject` (+ (`SceneComponent.K2_GetComponentLocation` _capsulecomponent) (select `bool` _bsuccess :`false` (* (`KismetMathLibrary.MakeVector` _returnvalue_x _returnvalue_y _returnvalue_z) _desireddistancefromplayer) :`true` (* (`KismetMathLibrary.MakeVector` _returnvalue_x _returnvalue_y _returnvalue_z_2) _desireddistancefromplayer)))))

(fn `CalculatePositionalSway`
  (bind _currentpositionswaymodifier (`self.CurrentPositionSwayModifier`))
  (bind _charactermovement (`Character.CharacterMovement` (`self.As BP Generic Character`)))
  (set `self.CurrentPositionSwayModifier` (+ (`self.CurrentPositionSwayModifier`) (* (`KismetMathLibrary.MapRangeClamped` (`KismetMathLibrary.VSize` (`MovementComponent.Velocity` _charactermovement)) 0.0 (`CharacterMovementComponent.MaxWalkSpeed` _charactermovement) 0.8 1.5) (`GameplayStatics.GetWorldDeltaSeconds`) (`self.InvertMassMultiplier`))))
  (set `self.PositionSway` (`KismetMathLibrary.MakeVector` 0.0 (* (`KismetMathLibrary.DegCos` _currentpositionswaymodifier) 1.1) (* (`KismetMathLibrary.DegSin` _currentpositionswaymodifier) 1.1))))

(fn `CalculateRotationalSway`
  (bind _charactermovement (`Character.CharacterMovement` (`self.As BP Generic Character`)))
  (set `self.CurrentRotationSwayMultiplier` (+ (`self.CurrentRotationSwayMultiplier`) (* (`KismetMathLibrary.MapRangeClamped` (`KismetMathLibrary.VSize` (`MovementComponent.Velocity` _charactermovement)) 0.0 (`CharacterMovementComponent.MaxWalkSpeed` _charactermovement) 0.25 0.75) (`GameplayStatics.GetWorldDeltaSeconds`) (`self.InvertMassMultiplier`))))
  (set `self.RotationalSway` (`KismetMathLibrary.MakeRotator` (* (`KismetMathLibrary.DegSin` (`self.CurrentRotationSwayMultiplier`)) 7.0) (* (`KismetMathLibrary.DegSin` (`self.CurrentRotationSwayMultiplier`)) 9.0) (* (`KismetMathLibrary.DegCos` (`self.CurrentRotationSwayMultiplier`)) 5.0))))

(fn `CalculateVelocityLag`
  (bind _returnvalue (`Controller.GetControlRotation` (`GameplayStatics.GetPlayerController` 0)))
  (bind (_returnvalue_x _returnvalue_y _returnvalue_z) (`KismetMathLibrary.BreakVector` (`KismetMathLibrary.LessLess_VectorRotator` (`MovementComponent.Velocity` (`Character.CharacterMovement` (`self.As BP Generic Character`))) _returnvalue)))
  (set `self.VelocityLag` (* (`KismetMathLibrary.GreaterGreater_VectorRotator` (`KismetMathLibrary.MakeVector` 0.0 _returnvalue_y _returnvalue_z) _returnvalue) (`self.VelocityLagMultiplier`) (`self.InvertMassMultiplier`))))

(fn `ClearPhysicActorData`
  (set `self.Pick Up Actor` null)
  (set `self.Pick Up Actor Component` null)
  (set `/Game/Blueprint/Character/Master/BP_GenericCharacter.CarryingInFrontOfHim` false (`self.As BP Generic Character`))
  (set `self.Grabbing` false))

(fn `Interactable`
  (params (`Generic Character` :type "/Game/Blueprint/Character/Master/BP_GenericCharacter Object Reference"))
  (bind _interactable (`/Game/Blueprint/Character/Master/BP_GenericCharacter.Interactable` `Generic Character`))
  (`/Engine/EditorBlueprintResources/StandardMacros.IsValid` _interactable
    (:`Is Valid`
      (`/Game/Blueprint/Interactable/BP_Master_Interactable.Interact Behavior` _interactable `Generic Character`))))

(fn `PickUpEquipement`
  (params (Array :type "Array of Actor Object Reference") (Owner :type "Actor Object Reference"))
  (locals (L_Owner :type "Actor Object Reference") (L_ArrayActor :type "Actor Object Reference") (L_ArrayComponent :type "StaticMeshComponent Object Reference"))
  (bind _pickupequipementactor (`self.PickUpEquipementActor`))
  (set `local.L_Owner` Owner)
  (set `self.Closest Distance` (+ (`self.CasterSphereRadius`) 100.0))
  (for _array_element Array
    (bind _output_get (set `local.L_ArrayActor` _array_element))
    (bind _asbp_master_pick_up_items (cast `/Game/Blueprint/Equipement/Master/BP_Master_PickUpItems` _output_get))
    (bind _returnvalue (`Actor.GetDistanceTo` _asbp_master_pick_up_items (`local.L_Owner`)))
    (if (<= _returnvalue (`self.Closest Distance`))
      (set `self.Closest Distance` _returnvalue)
      (set `self.PickUpEquipementActor` _asbp_master_pick_up_items)))
  (`/Engine/EditorBlueprintResources/StandardMacros.IsValid` _pickupequipementactor
    (:`Is Valid`
      (`/Game/Blueprint/Equipement/Master/BP_Master_PickUpItems.PickupBehavior` _pickupequipementactor (`self.As BP Generic Character`))
      (set `self.Grabbing` true)
      (set `self.PickUpType` "NewEnumerator1"))))

(fn `PickUpHierarchy`
  (bind _pickupitemsequipementcandidate (`self.PickUpItemsEquipementCandidate`))
  ; Pawn PickUp
  (bind (_outactors _returnvalue) (`KismetSystemLibrary.SphereOverlapActors` (`self.CasterSpherePosition` 50.0) 200.0 (`|MakeArray` "ObjectTypeQuery3" :!type "EObjectTypeQuery Enum") null (`|MakeArray` (`self.GetOwner`))))
  (if _returnvalue
    (`self.PickUpPawn` _outactors (`self.GetOwner`))
    (else
      (`KismetArrayLibrary.Array_Clear` (`self.PickUpItemsEquipementCandidate`))
      ; Equipement PickUp
      (bind (_outactors_2 _returnvalue_2) (`KismetSystemLibrary.SphereOverlapActors` (`self.CasterSpherePosition` 50.0) (`self.CasterSphereRadius`) (`|MakeArray` "ObjectTypeQuery1" "ObjectTypeQuery2" :!type "EObjectTypeQuery Enum") null (`|MakeArray` (`self.GetOwner`))))
      (if _returnvalue_2
        (for _array_element _outactors_2
          (bind _asbp_master_pick_up_items (cast `/Game/Blueprint/Equipement/Master/BP_Master_PickUpItems` _array_element))
          (`KismetArrayLibrary.Array_Add` _pickupitemsequipementcandidate _asbp_master_pick_up_items))
        (`/Engine/EditorBlueprintResources/StandardMacros.IsValid` (`|GetArrayItem` _pickupitemsequipementcandidate)
          (:`Is Valid`
            (`self.PickUpEquipement` _pickupitemsequipementcandidate (`self.GetOwner`)))
          (:`Is Not Valid`
            ; Physic PickUp
            (bind (_outactors_3 _returnvalue_3) (`KismetSystemLibrary.SphereOverlapActors` (`self.CasterSpherePosition` 50.0) (`self.CasterSphereRadius`) (`|MakeArray` "ObjectTypeQuery4" "ObjectTypeQuery2" :!type "EObjectTypeQuery Enum") null (`|MakeArray` (`self.GetOwner`)) :!label _label))
            (if _returnvalue_3
              (`self.PickUpPhysicObject` _outactors_3 (`self.GetOwner`)))))
        (else
          (goto _label))))))

(fn `PickUpPawn`
  (params (Array :type "Array of Actor Object Reference") (Owner :type "Actor Object Reference"))
  (locals (L_Owner :type "Actor Object Reference") (L_ArrayActor :type "Actor Object Reference") (L_ArrayComponent :type "StaticMeshComponent Object Reference"))
  (bind _pickuppawnactor (`self.PickUpPawnActor`))
  (set `local.L_Owner` Owner)
  (set `self.Closest Distance` (+ (`self.CasterSphereRadius`) 100.0))
  (for _array_element Array
    (bind _output_get (set `local.L_ArrayActor` _array_element))
    (bind _asbp_npc (cast `/Game/Blueprint/Character/NPCs/BP_NPC` _output_get))
    (bind _returnvalue (`Actor.GetDistanceTo` _asbp_npc (`local.L_Owner`)))
    (if (<= _returnvalue (`self.Closest Distance`))
      (set `self.Closest Distance` _returnvalue)
      (set `self.PickUpPawnActor` _asbp_npc)))
  (`/Engine/EditorBlueprintResources/StandardMacros.IsValid` _pickuppawnactor
    (:`Is Valid`
      (bind _asbp_player_fire_man (cast `/Game/Blueprint/Character/Player/BP_PlayerFireMan` (`self.As BP Generic Character`)))
      (bind _output_get_2 (set `self.As BP Player Fire Man` _asbp_player_fire_man))
      (`/Game/Blueprint/Character/Player/BP_PlayerFireMan.Rescueing` _output_get_2 _pickuppawnactor)
      (set `self.Grabbing` true)
      (set `self.PickUpType` "NewEnumerator0")
      (set `/Game/Blueprint/Character/Master/BP_GenericCharacter.CarryingOverHead` true _pickuppawnactor))))

(fn `PickUpPhysicObject`
  (params (Array :type "Array of Actor Object Reference") (Owner :type "Actor Object Reference"))
  (locals (L_Owner :type "Actor Object Reference") (L_ArrayActor :type "Actor Object Reference") (L_ArrayComponent :type "StaticMeshComponent Object Reference"))
  (bind _l_arraycomponent (`local.L_ArrayComponent`))
  (bind _pick_up_actor (`self.Pick Up Actor`))
  (set `local.L_Owner` Owner)
  (set `self.Closest Distance` (+ (`self.CasterSphereRadius`) 100.0))
  (for _array_element Array
    (bind _output_get (set `local.L_ArrayActor` _array_element))
    (`/Engine/EditorBlueprintResources/StandardMacros.IsValid` _output_get
      (:`Is Valid`
        (for _array_element_2 (`Actor.K2_GetComponentsByClass` _output_get "/Script/Engine.StaticMeshComponent")
          (bind _output_get_2 (set `local.L_ArrayComponent` _array_element_2))
          (`KismetSystemLibrary.PrintString` (`KismetSystemLibrary.GetDisplayName` (`local.L_ArrayActor`)) false true (`KismetMathLibrary.Conv_VectorToLinearColor` (`KismetMathLibrary.RandomUnitVector`)))
          (bind _returnvalue (`KismetMathLibrary.Vector_Distance` (`SceneComponent.K2_GetComponentLocation` _output_get_2) (`Actor.K2_GetActorLocation` (`local.L_Owner`))))
          (if (<= _returnvalue (`self.Closest Distance`))
            (set `self.Closest Distance` _returnvalue)
            (set `self.Pick Up Actor` (`local.L_ArrayActor`)))))))
  (`/Engine/EditorBlueprintResources/StandardMacros.IsValid` _pick_up_actor
    (:`Is Valid`
      (for _array_element_3 (`Actor.K2_GetComponentsByClass` _pick_up_actor "/Script/Engine.StaticMeshComponent")
        (bind _output_get_3 (set `local.L_ArrayComponent` _array_element_3))
        (`/Engine/EditorBlueprintResources/StandardMacros.IsValid` _output_get_3
          (:`Is Valid`
            (if (`SceneComponent.IsSimulatingPhysics` _output_get_3 "None")
              (set `self.Pick Up Actor Component` _output_get_3)
              (`PrimitiveComponent.SetUseCCD` _output_get_3 true "None")
              (`PhysicsHandleComponent.GrabComponentAtLocationWithRotation` (`/Game/Blueprint/Character/Master/BP_GenericCharacter.PhysicsHandle` (`self.As BP Generic Character`)) (`local.L_ArrayComponent`) "None" (`SceneComponent.K2_GetComponentLocation` _l_arraycomponent) (`SceneComponent.K2_GetComponentRotation` _l_arraycomponent))
              (set `/Game/Blueprint/Character/Master/BP_GenericCharacter.CarryingInFrontOfHim` true (`self.As BP Generic Character`))
              (set `self.Grabbing` true)
              (set `self.PickUpType` "NewEnumerator2")
              (`KismetSystemLibrary.K2_UnPauseTimerHandle` (`self.Timer Update Grab Item Position`)))))))))

(fn `ThrowPhysicActor`
  (bind _physicactorthrowingstrength (`self.PhysicActorThrowingStrength`))
  (bind _as_bp_generic_character (`self.As BP Generic Character`))
  (bind (_asbp_player_fire_man _bsuccess) (cast `/Game/Blueprint/Character/Player/BP_PlayerFireMan` _as_bp_generic_character :!pure true))
  (bind _physicshandle (`/Game/Blueprint/Character/Master/BP_GenericCharacter.PhysicsHandle` (`self.As BP Generic Character`)))
  (bind _output_get (set `self.Physic component` (`PhysicsHandleComponent.GetGrabbedComponent` _physicshandle)))
  (`PhysicsHandleComponent.ReleaseComponent` _physicshandle)
  (`PrimitiveComponent.AddImpulse` _output_get (select `bool` _bsuccess :`false` (`Actor.K2_GetActorLocation` _as_bp_generic_character) :`true` (* (`SceneComponent.GetForwardVector` (`/Game/Blueprint/Character/Player/BP_PlayerFireMan.FollowCamera` _asbp_player_fire_man)) (`KismetMathLibrary.FClamp` (/ _physicactorthrowingstrength (/ (`PrimitiveComponent.GetMass` (`self.Pick Up Actor Component`)) 10.0)) 10.0 _physicactorthrowingstrength))) "None" true))

(fn `UpdatePhysicActorPosition`
  (bind (_returnvalue_roll _returnvalue_pitch _returnvalue_yaw) (`KismetMathLibrary.BreakRotator` (`SceneComponent.K2_GetComponentRotation` (`Character.CapsuleComponent` (`self.As BP Generic Character`)))))
  (if (`self.Grabbing`)
    ; Calculate Location
    (`self.CalculateDesiredLocationForHeldPhysicActor`)
    (`self.CalculatePositionalSway`)
    (`self.CalculateVelocityLag`)
    (`self.CalculateAngularLagVariation`)
    (`self.CalculateAngularTiltVariation`)
    (`self.CalculateRotationalSway`)
    (`PhysicsHandleComponent.SetTargetLocationAndRotation` (`/Game/Blueprint/Character/Master/BP_GenericCharacter.PhysicsHandle` (`self.As BP Generic Character`)) (+ (- (+ (`self.PositionSway`) (`self.DesiredLocationForHeldObject`)) (`self.VelocityLag`)) (`self.AngularLagVar`)) (`KismetMathLibrary.ComposeRotators` (`KismetMathLibrary.ComposeRotators` (`self.AngularTiltVar`) (`self.RotationalSway`)) (`KismetMathLibrary.MakeRotator` 0.0 0.0 _returnvalue_yaw)))
    (else
      (`KismetSystemLibrary.K2_PauseTimerHandle` (`self.Timer Update Grab Item Position`)))))