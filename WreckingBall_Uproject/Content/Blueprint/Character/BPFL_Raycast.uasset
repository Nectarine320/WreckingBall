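; Blueprint function library with a raycast helper that finds what a skeletal mesh bone points at under the screen center.
; It deprojects the first local player's viewport center and traces along it up to a scan distance, taking the impact point or the ray's far end as target.
; A second trace from the bone to that target returns origin, end and hit, so obstructions between bone and aim point register.
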(fn `PointingMiddleOfScreen`
  (params (`Scan Distance` :type "Float (double-precision)") (SkinnedMeshComponent :type "SkinnedMeshComponent Object Reference") (InBoneName :type Name) (TraceChannel :type "ETraceTypeQuery Enum" :default "TraceTypeQuery1") (ActorsToIgnore :type "Array of Actor Object Reference (by ref)") (DrawDebugType :type "EDrawDebugTrace Enum" :default "None"))
  (returns (TraceOrigine :type "Vector Structure") (TraceEnd :type "Vector Structure") (OutHit :type "HitResult Structure") (`Return Value` :type Boolean))
  (bind _returnvalue (`GameplayStatics.GetPlayerController` null))
  (bind _returnvalue_location (`KismetMathLibrary.BreakTransform` (`SkinnedMeshComponent.GetBoneTransform` SkinnedMeshComponent InBoneName "RTS_World")))
  (bind (_sizex _sizey) (`PlayerController.GetViewportSize` _returnvalue))
  (bind (_worldposition _worlddirection) (`GameplayStatics.DeprojectScreenToWorld` _returnvalue (`KismetMathLibrary.MakeVector2D` (`KismetMathLibrary.Conv_IntToDouble` (/ _sizex 2)) (`KismetMathLibrary.Conv_IntToDouble` (/ _sizey 2)))))
  (bind _returnvalue_2 (+ _worldposition (* `Scan Distance` _worlddirection)))
  (bind (_outhit _returnvalue_3) (`KismetSystemLibrary.LineTraceSingle` null _worldposition _returnvalue_2 TraceChannel false ActorsToIgnore DrawDebugType))
  (bind _returnvalue_4 (select `bool` _returnvalue_3 :`false` _returnvalue_2 :`true` (`.ImpactPoint` (`GameplayStatics.BreakHitResult` _outhit))))
  (bind (_outhit_2 _returnvalue_5) (`KismetSystemLibrary.LineTraceSingle` null _returnvalue_location _returnvalue_4 TraceChannel false ActorsToIgnore DrawDebugType true (struct :`R` 1.0 :`B` 0.836866 :`A` 1.0)))
  (return _returnvalue_location _returnvalue_4 _outhit_2 _returnvalue_5))