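; Character component for picking up, carrying, dropping and throwing physics objects, and for kicking, passing or losing a dribbled soccer ball.
; Sphere overlaps find the nearest target: objects attach to the PhysicsHandle using their profile's grab settings, while balls gain a Possessor and go to BallDribble.
; A looping timer charges shot strength from the player's kick profile and feeds the gauge.
; Release applies an impulse shaped by the object's physics profile, with speed cap and random loft.
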(event `self.ReceiveBeginPlay`
  ;[0 0.1529 1 0.5] Begin Play
  (`self.InitializeOwner`))

(event `GrabRequested`
  ;[1 0 0.06535 0.5] PickUp Input
  (`/Engine/EditorBlueprintResources/StandardMacros.IsValid` (`self.As BP Generic Character`)
    (:`Is Valid`
      (if (not (`WB_PlayerStateComponent.IsHoldingAnything` (`/Game/Blueprint/Character/BP_GenericCharacter.PlayerStateComponent` (`self.As BP Generic Character`))))
        (bind (_outactors _returnvalue) (`KismetSystemLibrary.SphereOverlapActors` (`self.CasterSpherePosition` 25.0) (`self.CasterSphereRadius`) (`|MakeArray` "ObjectTypeQuery4" "ObjectTypeQuery2" :!type "EObjectTypeQuery Enum") null (`|MakeArray` (`self.GetOwner`))))
        (if _returnvalue
          (`self.PickUpPhysicObject` _outactors (`self.GetOwner`)))))))

(event `ShootReleased`
  (if (and (`WB_PlayerStateComponent.IsHoldingAnything` (`/Game/Blueprint/Character/BP_GenericCharacter.PlayerStateComponent` (`self.As BP Generic Character`))) (`self.Shooting`))
    (`self.ThrowPhysicActor`)
    (`self.ClearPhysicActorData`)
    (set `self.Shooting` false)))

(event `ShootChargeStarted`
  (if (`WB_PlayerStateComponent.IsHoldingAnything` (`/Game/Blueprint/Character/BP_GenericCharacter.PlayerStateComponent` (`self.As BP Generic Character`)))
    (bind _returnvalue (`KismetSystemLibrary.K2_SetTimerDelegate` (delegate `Update Shooting Strength`) 0.033 true true))
    (set `self.Shooting Strength Timer` _returnvalue)
    (set `self.Shooting` true)))

(event `Update Shooting Strength`
  (bind _output_get (set `self.ShootingStrenghtLerpValue` (`KismetMathLibrary.FClamp` (+ (`self.ShootingStrenghtLerpValue`) (`WB_KickProfile.GetChargeStep` (`WB_PlayerProfileLibrary.GetPlayerKickProfile` (`self.As BP Generic Character`)) 0.033)))))
  (set `self.ShootingStrenghtModifier` (`WB_KickProfile.GetStrengthForCharge` (`WB_PlayerProfileLibrary.GetPlayerKickProfile` (`self.As BP Generic Character`)) _output_get))
  (`self.UpdateKickProgressBar` _output_get)
  (`WB_PlayerStateComponent.SetActionCharge` (`/Game/Blueprint/Character/BP_GenericCharacter.PlayerStateComponent` (`self.As BP Generic Character`)) (`self.ShootingStrenghtLerpValue`)))

(event `DropHeldItem`
  ;[1 0 0.06535 0.5] Input Drop Item
  (`self.ReleaseHeldComponent`)
  (`self.Update Master Ball`)
  (`self.ClearPhysicActorData`)
  (set `self.Shooting` false))

(event `CancelShootCharge`
  ;[1 0 0.06535 0.5] Event Cancel Shooting Charge
  (`KismetSystemLibrary.K2_PauseTimerHandle` (`self.Shooting Strength Timer`))
  (set `self.ShootingStrenghtLerpValue` 0.0)
  (set `self.ShootingStrenghtModifier` 1.0)
  (`self.PauseKickProgressBar`)
  (set `self.Shooting` false))

(fn `ApplyKickLoft`
  (params (Velocity :type "Vector Structure") (MaxAngle :type "Float (double-precision)"))
  (returns (LoftedVelocity :type "Vector Structure"))
  (bind _returnvalue (`KismetMathLibrary.RandomFloatInRange` 0.0 MaxAngle))
  (return (+ (* Velocity (`KismetMathLibrary.DegCos` _returnvalue)) (`KismetMathLibrary.MakeVector` 0.0 0.0 (* (`KismetMathLibrary.VSize` Velocity) (`KismetMathLibrary.DegSin` _returnvalue))))))

(fn `ApplyKickProfile`
  (params (BaseVelocity :type "Vector Structure") (ThrownActor :type "Actor Object Reference") (Mass :type "Float (double-precision)"))
  (returns (KickVelocity :type "Vector Structure"))
  (bind _profile (message `/Game/Blueprint/Interfaces/BPI_ImpactSource.GetPhysicsProfile` ThrownActor))
  (`/Engine/EditorBlueprintResources/StandardMacros.IsValid` _profile
    (:`Is Valid`
      (bind _returnvalue (* (`local.BaseVelocity`) (`/Game/Blueprint/Ball/Data/PDA_PhysicsProfile.KickImpulse` _profile)))
      (bind _loftedvelocity (`self.ApplyKickLoft` (select `bool` (> (`/Game/Blueprint/Ball/Data/PDA_PhysicsProfile.MaxKickSpeed` _profile) 0.0) :`false` _returnvalue :`true` (`KismetMathLibrary.ClampVectorSize` _returnvalue 0.0 (* (`/Game/Blueprint/Ball/Data/PDA_PhysicsProfile.MaxKickSpeed` _profile) Mass))) (`/Game/Blueprint/Ball/Data/PDA_PhysicsProfile.KickMaxLoftAngle` _profile)))
      (return _loftedvelocity))
    (:`Is Not Valid`
      (return (* (`local.BaseVelocity`) (`self.PhysicActorThrowingStrength`))))))

(fn `ClearPhysicActorData`
  (`self.UpdateHeldObjectHolder` false)
  (`WB_PlayerStateComponent.ChangeHolding` (`/Game/Blueprint/Character/BP_GenericCharacter.PlayerStateComponent` (`self.As BP Generic Character`)) (struct :`TagName` "Player.Holding.None"))
  (set `self.Pick Up Actor` null)
  (set `self.Pick Up Actor Component` null)
  (set `self.As BP PO Master Ball 01` null)
  (`KismetSystemLibrary.K2_PauseTimerHandle` (`self.Shooting Strength Timer`))
  (set `self.ShootingStrenghtLerpValue` 0.0)
  (set `self.ShootingStrenghtModifier` 1.0)
  (`self.PauseKickProgressBar`))

(fn `ConfigureGrabFromProfile`
  (params (Component :type "PrimitiveComponent Object Reference"))
  (bind _physicshandle (`/Game/Blueprint/Character/BP_GenericCharacter.PhysicsHandle` (`self.As BP Generic Character`)))
  (set `self.bGrabAtPoint` false)
  (bind _profile (message `/Game/Blueprint/Interfaces/BPI_ImpactSource.GetPhysicsProfile` (`self.GetOwner` Component)))
  (`/Engine/EditorBlueprintResources/StandardMacros.IsValid` _profile
    (:`Is Valid`
      (`PhysicsHandleComponent.SetLinearStiffness` _physicshandle (`/Game/Blueprint/Ball/Data/PDA_PhysicsProfile.GrabLinearStiffness` _profile))
      (`PhysicsHandleComponent.SetLinearDamping` _physicshandle (`/Game/Blueprint/Ball/Data/PDA_PhysicsProfile.GrabLinearDamping` _profile))
      (set `self.bGrabAtPoint` (`BlueprintGameplayTagLibrary.MatchesTag` (`/Game/Blueprint/Ball/Data/PDA_PhysicsProfile.GrabMode` _profile) (struct :`TagName` "Grab.Mode.AtPoint") true)))))

(fn `ForceDrop`
  (params (Impulse :type "Vector Structure"))
  (if (`WB_PlayerStateComponent.IsHoldingAnything` (`/Game/Blueprint/Character/BP_GenericCharacter.PlayerStateComponent` (`self.As BP Generic Character`)))
    (`self.ReleaseHeldComponent`)
    (`self.UpdateHeldObjectHolder` false)
    (`self.Update Master Ball`)
    (`WB_FeedbackLibrary.SetResponsiblePawn` (`self.Pick Up Actor`) (`self.As BP Generic Character`))
    (`self.ClearPhysicActorData`)
    (set `self.Shooting` false)
    (`/Engine/EditorBlueprintResources/StandardMacros.IsValid` (`self.Physic component`)
      (:`Is Valid`
        (`PrimitiveComponent.AddImpulse` (`self.Physic component`) Impulse "None" true)))))

(fn `GrabPhysicComponent`
  (params (Component :type "PrimitiveComponent Object Reference"))
  (bind _as_bp_generic_character (`self.As BP Generic Character`))
  (bind _physicshandle (`/Game/Blueprint/Character/BP_GenericCharacter.PhysicsHandle` _as_bp_generic_character))
  (bind _playerstatecomponent (`/Game/Blueprint/Character/BP_GenericCharacter.PlayerStateComponent` _as_bp_generic_character))
  (bind (_outpointonbody _returnvalue) (`PrimitiveComponent.GetClosestPointOnCollision` Component (`SceneComponent.K2_GetComponentLocation` (`Character.CapsuleComponent` _as_bp_generic_character)) "None"))
  (`self.ConfigureGrabFromProfile` Component)
  (if (`self.bGrabAtPoint`)
    (`PhysicsHandleComponent.GrabComponentAtLocation` _physicshandle Component "None" (select `bool` (< _returnvalue 0.0) :`false` _outpointonbody :`true` (`SceneComponent.K2_GetComponentLocation` Component)))
    (`WB_PlayerStateComponent.SetHeldObjectMass` _playerstatecomponent (`PrimitiveComponent.GetMass` Component))
    (else
      (`PhysicsHandleComponent.GrabComponentAtLocationWithRotation` _physicshandle Component "None" (`SceneComponent.K2_GetComponentLocation` Component) (`SceneComponent.K2_GetComponentRotation` Component))
      (`WB_PlayerStateComponent.SetHeldObjectMass` _playerstatecomponent 0.0))))

(fn `InitializeOwner`
  (bind _asbp_generic_character (cast `/Game/Blueprint/Character/BP_GenericCharacter` (`self.GetOwner`)))
  (bind _output_get (set `self.As BP Generic Character` _asbp_generic_character))
  (bind _asbp_soccer_player (cast `/Game/Blueprint/Character/BP_SoccerPlayer` _output_get))
  (set `self.As BP Soccer Player` _asbp_soccer_player))

(fn `LoseDribbledBall`
  (`self.Update Master Ball`)
  (`self.ClearPhysicActorData`)
  (set `self.Shooting` false))

(fn `PassBall`
  (params (BallVelocity :type "Vector Structure"))
  (`self.ReleaseHeldComponent`)
  (`self.UpdateHeldObjectHolder` false)
  (`self.Update Master Ball`)
  (`PrimitiveComponent.SetPhysicsLinearVelocity` (`self.Physic component`) BallVelocity false "None")
  (`WB_FeedbackLibrary.SetResponsiblePawn` (`self.Pick Up Actor`) (`self.As BP Generic Character`))
  (`WB_BallPossessionSubsystem.MarkBallKicked` (`self.Pick Up Actor`) (`self.As BP Generic Character`))
  (`self.ClearPhysicActorData`)
  (set `self.Shooting` false))

(fn `PauseKickProgressBar`
  (`/Engine/EditorBlueprintResources/StandardMacros.IsValid` (`self.As BP Generic Character`)
    (:`Is Valid`
      (set `/Game/Blueprint/Character/BP_GenericCharacter.KickStrenghtPercent` 0.0 (`self.As BP Generic Character`))
      (`self.SetOwnerKickGauge` 0.0))))

(fn `PickUpHierarchy`
  ; Physic PickUp
  (bind (_outactors _returnvalue) (`KismetSystemLibrary.SphereOverlapActors` (`self.CasterSpherePosition` 50.0) (`self.CasterSphereRadius`) (`|MakeArray` "ObjectTypeQuery4" "ObjectTypeQuery2" :!type "EObjectTypeQuery Enum") null (`|MakeArray` (`self.GetOwner`))))
  (if _returnvalue
    (`self.PickUpPhysicObject` _outactors (`self.GetOwner`))))

(fn `PickUpObjects`
  (params (Array :type "Array of Actor Object Reference") (Owner :type "Actor Object Reference"))
  (locals (L_Owner :type "Actor Object Reference") (L_ArrayActor :type "Actor Object Reference") (L_ArrayComponent :type "StaticMeshComponent Object Reference"))
  (bind _l_arraycomponent (`local.L_ArrayComponent`))
  (bind _pick_up_actor (`self.Pick Up Actor`))
  (set `local.L_Owner` Owner)
  (set `self.Closest Distance` (+ (`self.CasterSphereRadius`) 100.0))
  (for _array_element Array
    (bind _output_get (set `local.L_ArrayActor` _array_element))
    (cast `/Game/Blueprint/Ball/BP_PO_Master_Ball_01` _output_get
      (:`CastFailed`
        (`/Engine/EditorBlueprintResources/StandardMacros.IsValid` _output_get
          (:`Is Valid`
            (for _array_element_2 (`Actor.K2_GetComponentsByClass` _output_get "/Script/Engine.StaticMeshComponent")
              (bind _output_get_2 (set `local.L_ArrayComponent` _array_element_2))
              (bind _returnvalue (`KismetMathLibrary.Vector_Distance` (`SceneComponent.K2_GetComponentLocation` _output_get_2) (`Actor.K2_GetActorLocation` (`local.L_Owner`))))
              (if (<= _returnvalue (`self.Closest Distance`))
                (set `self.Closest Distance` _returnvalue)
                (set `self.Pick Up Actor` (`local.L_ArrayActor`)))))))))
  (`/Engine/EditorBlueprintResources/StandardMacros.IsValid` _pick_up_actor
    (:`Is Valid`
      (bind _asbp_po_master_ball_01 (cast `/Game/Blueprint/Ball/BP_PO_Master_Ball_01` _pick_up_actor)
        (:`then`
          (set `self.As BP PO Master Ball 01` _asbp_po_master_ball_01))
        (:`CastFailed`
          _))
      (for _array_element_3 (`Actor.K2_GetComponentsByClass` _pick_up_actor "/Script/Engine.StaticMeshComponent")
        (bind _output_get_3 (set `local.L_ArrayComponent` _array_element_3))
        (`/Engine/EditorBlueprintResources/StandardMacros.IsValid` _output_get_3
          (:`Is Valid`
            (if (`SceneComponent.IsSimulatingPhysics` _output_get_3 "None")
              (set `self.Pick Up Actor Component` _output_get_3)
              (`PrimitiveComponent.SetUseCCD` _output_get_3 true "None")
              (`PhysicsHandleComponent.GrabComponentAtLocationWithRotation` (`/Game/Blueprint/Character/BP_GenericCharacter.PhysicsHandle` (`self.As BP Generic Character`)) (`local.L_ArrayComponent`) "None" (`SceneComponent.K2_GetComponentLocation` _l_arraycomponent) (`SceneComponent.K2_GetComponentRotation` _l_arraycomponent))
              (`WB_PlayerStateComponent.ChangeHolding` (`/Game/Blueprint/Character/BP_GenericCharacter.PlayerStateComponent` (`self.As BP Generic Character`)) (struct :`TagName` "Player.Holding.Object"))
              (`self.StartHeldObjectMotion`)
              (`self.UpdateHeldObjectHolder` true))))))))

(fn `PickUpPhysicObject`
  (params (Array :type "Array of Actor Object Reference") (Owner :type "Actor Object Reference"))
  (locals (L_Owner :type "Actor Object Reference") (L_ArrayActor :type "Actor Object Reference") (L_ArrayComponent :type "StaticMeshComponent Object Reference"))
  (bind _l_arrayactor (`local.L_ArrayActor`))
  (bind _pick_up_actor (`self.Pick Up Actor`))
  (bind _returnvalue (`Actor.K2_GetActorLocation` (`local.L_Owner`)))
  (set `local.L_Owner` Owner)
  (set `self.Closest Distance` (+ (`self.CasterSphereRadius`) 100.0))
  (for _array_element Array
    (bind _output_get (set `local.L_ArrayActor` _array_element))
    (cast `/Game/Blueprint/Ball/BP_PO_Master_Ball_01` _output_get
      (:`CastFailed`
        (`/Engine/EditorBlueprintResources/StandardMacros.IsValid` _output_get
          (:`Is Valid`
            (for _array_element_2 (`Actor.K2_GetComponentsByClass` _output_get "/Script/Engine.StaticMeshComponent")
              (bind _output_get_2 (set `local.L_ArrayComponent` _array_element_2))
              (bind _returnvalue_2 (`KismetMathLibrary.Vector_Distance` (`PrimitiveComponent.GetClosestPointOnCollision` _output_get_2 _returnvalue "None") _returnvalue))
              (if (and (<= _returnvalue_2 (`self.Closest Distance`)) (not (`Actor.ActorHasTag` _l_arrayactor "NoGrab")))
                (set `self.Closest Distance` _returnvalue_2)
                (set `self.Pick Up Actor` _l_arrayactor))))))))
  (`/Engine/EditorBlueprintResources/StandardMacros.IsValid` _pick_up_actor
    (:`Is Valid`
      (bind _asbp_po_master_ball_01 (cast `/Game/Blueprint/Ball/BP_PO_Master_Ball_01` _pick_up_actor)
        (:`then`
          (set `self.As BP PO Master Ball 01` _asbp_po_master_ball_01))
        (:`CastFailed`
          _))
      (for _array_element_3 (`Actor.K2_GetComponentsByClass` _pick_up_actor "/Script/Engine.StaticMeshComponent")
        (bind _output_get_3 (set `local.L_ArrayComponent` _array_element_3))
        (`/Engine/EditorBlueprintResources/StandardMacros.IsValid` _output_get_3
          (:`Is Valid`
            (if (`SceneComponent.IsSimulatingPhysics` _output_get_3 "None")
              (set `self.Pick Up Actor Component` _output_get_3)
              (`PrimitiveComponent.SetUseCCD` _output_get_3 true "None")
              (`self.GrabPhysicComponent` (`local.L_ArrayComponent`))
              (`WB_PlayerStateComponent.ChangeHolding` (`/Game/Blueprint/Character/BP_GenericCharacter.PlayerStateComponent` (`self.As BP Generic Character`)) (struct :`TagName` "Player.Holding.Object"))
              (`self.StartHeldObjectMotion`)
              (`self.UpdateHeldObjectHolder` true))))))))

(fn `PickUpSoccerBall`
  (params (Array :type "Array of Actor Object Reference") (Owner :type "Actor Object Reference"))
  (locals (L_Owner :type "Actor Object Reference") (L_ArrayActor :type "Actor Object Reference") (L_ArrayComponent :type "StaticMeshComponent Object Reference"))
  (bind _pick_up_actor (`self.Pick Up Actor`))
  (set `local.L_Owner` Owner)
  (set `self.Closest Distance` (+ (`self.CasterSphereRadius`) 100.0))
  (for _array_element Array
    (bind _output_get (set `local.L_ArrayActor` _array_element))
    (bind _asbp_po_master_ball_01 (cast `/Game/Blueprint/Ball/BP_PO_Master_Ball_01` _output_get))
    (`/Engine/EditorBlueprintResources/StandardMacros.IsValid` _asbp_po_master_ball_01
      (:`Is Valid`
        (for _array_element_2 (`Actor.K2_GetComponentsByClass` _output_get "/Script/Engine.StaticMeshComponent")
          (bind _output_get_2 (set `local.L_ArrayComponent` _array_element_2))
          (bind _returnvalue (`KismetMathLibrary.Vector_Distance` (`SceneComponent.K2_GetComponentLocation` _output_get_2) (`Actor.K2_GetActorLocation` (`local.L_Owner`))))
          (if (<= _returnvalue (`self.Closest Distance`))
            (set `self.Closest Distance` _returnvalue)
            (set `self.Pick Up Actor` (`local.L_ArrayActor`)))))))
  (`/Engine/EditorBlueprintResources/StandardMacros.IsValid` _pick_up_actor
    (:`Is Valid`
      (bind _asbp_po_master_ball_01_2 (cast `/Game/Blueprint/Ball/BP_PO_Master_Ball_01` _pick_up_actor)
        (:`then`
          (bind _output_get_3 (set `self.As BP PO Master Ball 01` _asbp_po_master_ball_01_2))
          (`/Engine/EditorBlueprintResources/StandardMacros.IsValid` (`/Game/Blueprint/Ball/BP_PO_Master_Ball_01.Possessor` _output_get_3)
            (:`Is Not Valid`
              (set `/Game/Blueprint/Ball/BP_PO_Master_Ball_01.Possessor` (`self.As BP Soccer Player`) _asbp_po_master_ball_01_2))))
        (:`CastFailed`
          _))
      (for _array_element_3 (`Actor.K2_GetComponentsByClass` _pick_up_actor "/Script/Engine.StaticMeshComponent")
        (bind _output_get_4 (set `local.L_ArrayComponent` _array_element_3))
        (`/Engine/EditorBlueprintResources/StandardMacros.IsValid` _output_get_4
          (:`Is Valid`
            (if (`SceneComponent.IsSimulatingPhysics` _output_get_4 "None")
              (set `self.Pick Up Actor Component` _output_get_4)
              (`PrimitiveComponent.SetUseCCD` _output_get_4 true "None")
              (bind _profile (`/Game/Blueprint/Interfaces/BPI_ImpactSource.GetPhysicsProfile` (`self.As BP PO Master Ball 01`)))
              (bind _returnvalue_2 (`WB_BallDribbleComponent.StartDribble` (`/Game/Blueprint/Character/BP_GenericCharacter.BallDribble` (`self.As BP Generic Character`)) (`self.Pick Up Actor`) (`/Game/Blueprint/Ball/Data/PDA_PhysicsProfile.DribbleProfile` _profile)))
              (if _returnvalue_2
                (`WB_PlayerStateComponent.ChangeHolding` (`/Game/Blueprint/Character/BP_GenericCharacter.PlayerStateComponent` (`self.As BP Generic Character`)) (struct :`TagName` "Player.Holding.Ball"))
                (`self.UpdateHeldObjectHolder` true)
                (else
                  (set `/Game/Blueprint/Ball/BP_PO_Master_Ball_01.Possessor` null (`self.As BP PO Master Ball 01`)))))))))))

(fn `ReleaseHeldComponent`
  (if (`WB_BallDribbleComponent.IsDribbling` (`/Game/Blueprint/Character/BP_GenericCharacter.BallDribble` (`self.As BP Generic Character`)))
    (set `self.Physic component` (`WB_BallDribbleComponent.GetDribbledBody` (`/Game/Blueprint/Character/BP_GenericCharacter.BallDribble` (`self.As BP Generic Character`))))
    (`WB_BallDribbleComponent.StopDribble` (`/Game/Blueprint/Character/BP_GenericCharacter.BallDribble` (`self.As BP Generic Character`)))
    (else
      (set `self.Physic component` (`PhysicsHandleComponent.GetGrabbedComponent` (`/Game/Blueprint/Character/BP_GenericCharacter.PhysicsHandle` (`self.As BP Generic Character`))))
      (`PhysicsHandleComponent.ReleaseComponent` (`/Game/Blueprint/Character/BP_GenericCharacter.PhysicsHandle` (`self.As BP Generic Character`))))))

(fn `SetOwnerKickGauge`
  (params (Percent :type "Float (double-precision)"))
  (bind _returnvalue (`Actor.GetComponentByClass` (`self.GetOwner`) "/Script/WreckingBall.WB_GroundRingComponent"))
  (`/Engine/EditorBlueprintResources/StandardMacros.IsValid` _returnvalue
    (:`Is Valid`
      (`WB_GroundRingComponent.SetKickPercent` _returnvalue Percent))))

(fn `StartHeldObjectMotion`
  (bind _returnvalue (`Actor.GetComponentByClass` (`self.GetOwner`) "/Script/WreckingBall.WB_HeldObjectMotionComponent"))
  (`/Engine/EditorBlueprintResources/StandardMacros.IsValid` (`self.As BP PO Master Ball 01`)
    (:`Is Valid`
      (`WB_HeldObjectMotionComponent.StartHolding` _returnvalue (`self.Pick Up Actor Component`) (`self.bGrabAtPoint`) true))
    (:`Is Not Valid`
      (`WB_HeldObjectMotionComponent.StartHolding` _returnvalue (`self.Pick Up Actor Component`) (`self.bGrabAtPoint`) false))))

(fn `ThrowPhysicActor`
  (bind _pick_up_actor (`self.Pick Up Actor`))
  (bind _as_bp_generic_character (`self.As BP Generic Character`))
  (`self.ReleaseHeldComponent`)
  (`self.UpdateHeldObjectHolder` false)
  (`self.Update Master Ball`)
  (bind _kickvelocity (`self.ApplyKickProfile` (* (`self.ShootingStrenghtModifier`) (+ (`SceneComponent.GetForwardVector` (`Character.CapsuleComponent` (`self.As BP Generic Character`))) (`KismetMathLibrary.MakeVector` 0.0 0.0 (`KismetMathLibrary.SelectFloat` 0.0 0.1 (`self.bGrabAtPoint`))))) (`self.Pick Up Actor`) (`PrimitiveComponent.GetMass` (`self.Pick Up Actor Component`))))
  (`PrimitiveComponent.AddImpulse` (`self.Physic component`) _kickvelocity "None" false)
  (`WB_FeedbackLibrary.SetResponsiblePawn` _pick_up_actor _as_bp_generic_character)
  (bind _asbp_po_master_ball_01 (cast `/Game/Blueprint/Ball/BP_PO_Master_Ball_01` _pick_up_actor))
  (bind _profile (message `/Game/Blueprint/Interfaces/BPI_ImpactSource.GetPhysicsProfile` _asbp_po_master_ball_01))
  (`WB_BallPossessionSubsystem.MarkBallKicked` _asbp_po_master_ball_01 _as_bp_generic_character (`/Game/Blueprint/Ball/Data/PDA_PhysicsProfile.KickedReleaseSpeed` _profile))
  (`NiagaraFunctionLibrary.SpawnSystemAtLocation` "/Game/Art/VFX/KickBlast/NS_KickBlast.NS_KickBlast" (`Actor.K2_GetActorLocation` _asbp_po_master_ball_01)))

(fn `Update Master Ball`
  (bind _pick_up_actor (`self.Pick Up Actor`))
  (`/Engine/EditorBlueprintResources/StandardMacros.IsValid` _pick_up_actor
    (:`Is Valid`
      (bind _asbp_po_master_ball_01 (cast `/Game/Blueprint/Ball/BP_PO_Master_Ball_01` _pick_up_actor))
      (set `/Game/Blueprint/Ball/BP_PO_Master_Ball_01.Possessor` null _asbp_po_master_ball_01)
      (`/Game/Blueprint/Ball/BP_PO_Master_Ball_01.Trigger Kick Scan Timer` _asbp_po_master_ball_01))))

(fn `UpdateHeldObjectHolder`
  (params (IsHeld :type Boolean))
  (bind _pick_up_actor_component (`self.Pick Up Actor Component`))
  (bind _asbp_m_physic_object (cast `/Game/Blueprint/PhysicalObject/BP_M_PhysicObject` (`self.Pick Up Actor`)))
  (if (`local.IsHeld`)
    (`/Game/Blueprint/PhysicalObject/BP_M_PhysicObject.AssignHolder` _asbp_m_physic_object (`self.GetOwner`))
    (else
      (`/Game/Blueprint/PhysicalObject/BP_M_PhysicObject.AssignHolder` _asbp_m_physic_object null)))
  (`/Engine/EditorBlueprintResources/StandardMacros.IsValid` _pick_up_actor_component
    (:`Is Valid`
      (`PrimitiveComponent.IgnoreComponentWhenMoving` (`Character.CapsuleComponent` (`self.As BP Generic Character`)) _pick_up_actor_component (`local.IsHeld`)))))

(fn `UpdateKickProgressBar`
  (params (KickStrenghtPercent :type "Float (double-precision)"))
  (set `/Game/Blueprint/Character/BP_GenericCharacter.KickStrenghtPercent` KickStrenghtPercent (`self.As BP Generic Character`))
  (`self.SetOwnerKickGauge` KickStrenghtPercent))