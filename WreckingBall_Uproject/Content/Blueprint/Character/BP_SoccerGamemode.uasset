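; Game mode for a local-multiplayer soccer match, running it through tag-based phases: countdown, playing, goal pause, ended and results.
; Looping and one-shot timers drive phase changes, broadcast with score updates through dispatchers; goals pause the match clock, trigger celebrate or sulk states, then respawn via SpawnManager.
; It assigns teams from GI_Core slots or index parity, tracks bot-manager player changes, spawns a physics budget manager and offers debug clock controls.
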(event `self.ReceiveBeginPlay`
  ;[0 0.1529 1 0.5] Begin Play
  (`self.SetupMatchPlayers`)
  (`self.SetAllPlayersState` (struct :`TagName` "Player.State.Disabled"))
  (`self.StartMatchCountdown`)
  (`self.InitializePhysicsBudget`))

(event `StartMatchCountdown`
  ;[1 0 0.06535 0.5] Score Update
  (`self.ChangeMatchPhase` (struct :`TagName` "Match.Phase.Countdown"))
  (set `self.CountdownStepsLeft` (`self.CountdownSteps`))
  (`self.OnCountdownTick` (`self.CountdownStepsLeft`))
  (bind _returnvalue (`KismetSystemLibrary.K2_SetTimerDelegate` (delegate `CountdownTick`) 1.0 true))
  (set `self.PhaseTimerHandle` _returnvalue))

(event `CountdownTick`
  ;[0 1 0.07739 0.5] Countdown Tick
  (set `self.CountdownStepsLeft` (- (`self.CountdownStepsLeft`) 1))
  (`self.OnCountdownTick` (`self.CountdownStepsLeft`))
  (if (<= (`self.CountdownStepsLeft`) 0)
    (`KismetSystemLibrary.K2_ClearAndInvalidateTimerHandle` (`self.PhaseTimerHandle`))
    (`self.BeginMatch`)))

(event `BeginMatch`
  ;[0 0.1529 1 0.5] Match Update
  (`self.ChangeMatchPhase` (struct :`TagName` "Match.Phase.Playing"))
  (`/Game/Blueprint/Ball/BP_SpawnManager.Start Spawn` (`self.SpawnManager`))
  (`self.SetAllPlayersState` (struct :`TagName` "Player.State.Free"))
  (bind _returnvalue (`KismetSystemLibrary.K2_SetTimerDelegate` (delegate `MatchTimeElapsed`) (`self.MatchDuration`)))
  (set `self.MatchTimerHandle` _returnvalue)
  (`self.ApplyDebugTimerFreeze`))

(event `MatchTimeElapsed`
  ;[0 1 0.07739 0.5] Match Timer
  (`self.ChangeMatchPhase` (struct :`TagName` "Match.Phase.Ended"))
  (`self.SetAllPlayersState` (struct :`TagName` "Player.State.Disabled"))
  (bind _returnvalue (`KismetSystemLibrary.K2_SetTimerDelegate` (delegate `ShowMatchResults`) (`self.EndAnnouncementDuration`)))
  (set `self.PhaseTimerHandle` _returnvalue))

(event `Update Score`
  (params (`Is Team Red` :type Boolean))
  ;[1 0 0.06535 0.5] Update Score
  (`self.RegisterGoal` `Is Team Red`))

(event `ShowMatchResults`
  ;[1 0 0.06535 0.5] Match Results
  (`self.ChangeMatchPhase` (struct :`TagName` "Match.Phase.Results")))

(event `StartGoalPause`
  ;[0 1 0.07739 0.5] Match Timer - On pause (Goal Scored!)
  (`self.ChangeMatchPhase` (struct :`TagName` "Match.Phase.GoalPause"))
  (`KismetSystemLibrary.K2_PauseTimerHandle` (`self.MatchTimerHandle`))
  (bind _returnvalue (`KismetSystemLibrary.K2_SetTimerDelegate` (delegate `ResumeMatch`) (`self.GoalPauseDuration`)))
  (set `self.PhaseTimerHandle` _returnvalue))

(event `ResumeMatch`
  ;[0 1 0.07739 0.5] Match Timer - On pause (Goal Scored!)
  (`self.ChangeMatchPhase` (struct :`TagName` "Match.Phase.Playing"))
  (`self.SetAllPlayersState` (struct :`TagName` "Player.State.Free"))
  (`/Game/Blueprint/Ball/BP_SpawnManager.Goal Spawn` (`self.SpawnManager`))
  (`KismetSystemLibrary.K2_UnPauseTimerHandle` (`self.MatchTimerHandle`))
  (`self.ApplyDebugTimerFreeze`))

(event `self.BotManagerComponent.OnLocalPlayerAdded`
  (params (PlayerIndex :type Integer) (Pawn :type "Pawn Object Reference"))
  (bind _teamindex (`self.GetTeamForPlayer` PlayerIndex))
  (`self.RegisterMatchPlayer` PlayerIndex _teamindex))

(event `self.BotManagerComponent.OnLocalPlayerRemoving`
  (params (PlayerIndex :type Integer) (Pawn :type "Pawn Object Reference"))
  (bind _asbp_soccer_player (cast `/Game/Blueprint/Character/BP_SoccerPlayer` Pawn))
  (`/Game/Blueprint/Character/BPC_GrabObject.ForceDrop` (`/Game/Blueprint/Character/BP_GenericCharacter.BPC_GrabPhysicObject` _asbp_soccer_player) (0.0 0.0 0.0))
  (`KismetArrayLibrary.Array_RemoveItem` (`self.Players`) _asbp_soccer_player))

(fn `ApplyDebugTimerFreeze`
  (if (`self.DebugTimerFrozen`)
    (`KismetSystemLibrary.K2_PauseTimerHandle` (`self.MatchTimerHandle`))))

(fn `ChangeMatchPhase`
  (params (NewPhase :type "GameplayTag Structure"))
  (bind _output_get (set `self.MatchPhase` NewPhase))
  (`self.OnMatchPhaseChanged` _output_get))

(fn `DebugRemoveMatchTime`
  (locals (RemainingBefore :type "Float (double-precision)"))
  (if (`BlueprintGameplayTagLibrary.MatchesTag` (`self.MatchPhase`) (struct :`TagName` "Match.Phase.Playing") true)
    (set `local.RemainingBefore` (`KismetSystemLibrary.K2_GetTimerRemainingTimeHandle` (`self.MatchTimerHandle`)))
    (if (> (`local.RemainingBefore`) (`self.DebugTimeStep`))
      (`KismetSystemLibrary.K2_ClearAndInvalidateTimerHandle` (`self.MatchTimerHandle`))
      (bind _returnvalue (`KismetSystemLibrary.K2_SetTimerDelegate` (`|CreateDelegate` :!event `MatchTimeElapsed`) (`KismetMathLibrary.FMax` (- (`local.RemainingBefore`) (`self.DebugTimeStep`)) (`self.DebugTimeStep`))))
      (set `self.MatchTimerHandle` _returnvalue)
      (`self.ApplyDebugTimerFreeze`))))

(fn `DebugToggleMatchTimer`
  (set `self.DebugTimerFrozen` (not (`self.DebugTimerFrozen`)))
  (if (`self.DebugTimerFrozen`)
    (`KismetSystemLibrary.K2_PauseTimerHandle` (`self.MatchTimerHandle`))
    (elif (`BlueprintGameplayTagLibrary.MatchesTag` (`self.MatchPhase`) (struct :`TagName` "Match.Phase.Playing") true)
      (`KismetSystemLibrary.K2_UnPauseTimerHandle` (`self.MatchTimerHandle`)))))

(fn `GetCurrentMatchPhase`
  (returns (Phase :type "GameplayTag Structure"))
  (return (`self.MatchPhase`)))

(fn `GetMatchResult`
  (returns (Result :type "GameplayTag Structure"))
  (if (> (`self.ScoreRed`) (`self.ScoreBlue`))
    (return (struct :`TagName` "Match.Result.RedWin"))
    (elif (< (`self.ScoreRed`) (`self.ScoreBlue`))
      (return (struct :`TagName` "Match.Result.BlueWin"))
      (else
        (return (struct :`TagName` "Match.Result.Tie"))))))

(fn `GetScores`
  (returns (RedScore :type Integer) (BlueScore :type Integer))
  (return (`self.ScoreRed`) (`self.ScoreBlue`)))

(fn `GetTeamForPlayer`
  (params (PlayerIndex :type Integer))
  (returns (TeamIndex :type Integer))
  (bind _asgi_core (cast `/Game/Blueprint/Core/GI_Core` (`GameplayStatics.GetGameInstance`))
    (:`then`
      (bind _slotindex (`/Game/Blueprint/Core/GI_Core.FindSlotByControllerId` _asgi_core (`GameplayStatics.GetPlayerControllerID` (`GameplayStatics.GetPlayerController` PlayerIndex))))
      (if (>= _slotindex 0)
        (bind _teamindex (`/Game/Blueprint/Core/GI_Core.GetSlotTeam` _asgi_core _slotindex))
        (return _teamindex)
        (else
          (return (mod PlayerIndex 2)))))
    (:`CastFailed`
      (return (mod PlayerIndex 2)))))

(fn `GetTimeRemaining`
  (returns (Seconds :type "Float (double-precision)"))
  (if (or (`BlueprintGameplayTagLibrary.MatchesTag` (`self.MatchPhase`) (struct :`TagName` "Match.Phase.Playing") true) (`BlueprintGameplayTagLibrary.MatchesTag` (`self.MatchPhase`) (struct :`TagName` "Match.Phase.GoalPause") true))
    (return (`KismetSystemLibrary.K2_GetTimerRemainingTimeHandle` (`self.MatchTimerHandle`)))
    (elif (or (`BlueprintGameplayTagLibrary.MatchesTag` (`self.MatchPhase`) (struct :`TagName` "Match.Phase.Ended") true) (`BlueprintGameplayTagLibrary.MatchesTag` (`self.MatchPhase`) (struct :`TagName` "Match.Phase.Results") true))
      (return 0.0)
      (else
        (return (`self.MatchDuration`))))))

(fn `InitializePhysicsBudget`
  (`|SpawnActorFromClass` "/Game/Blueprint/Impact/Budget/BP_PhysicsBudgetManager.BP_PhysicsBudgetManager_C" (`KismetMathLibrary.MakeTransform` (0.0 0.0 0.0)) "AlwaysSpawn" "MultiplyWithRoot" null null))

(fn `RegisterGoal`
  (params (ScoringTeamIsRed :type Boolean))
  (if (`BlueprintGameplayTagLibrary.MatchesTag` (`self.MatchPhase`) (struct :`TagName` "Match.Phase.Playing") true)
    (set `self.ScoreRed` (+ (`self.ScoreRed`) (select `bool` (`local.ScoringTeamIsRed`) :`true` 1)))
    (set `self.ScoreBlue` (+ (`self.ScoreBlue`) (select `bool` (`local.ScoringTeamIsRed`) :`false` 1)))
    (`self.OnScoreChanged` (`local.ScoringTeamIsRed`) (`self.ScoreRed`) (`self.ScoreBlue`))
    (`self.StartGoalCelebration` (`local.ScoringTeamIsRed`))
    (`self.StartGoalPause`)))

(fn `RegisterMatchPlayer`
  (params (PlayerIndex :type Integer) (TeamIndex :type Integer))
  (bind _asbp_soccer_player (cast `/Game/Blueprint/Character/BP_SoccerPlayer` (`GameplayStatics.GetPlayerCharacter` PlayerIndex)))
  (if (== TeamIndex 1)
    (`PrimitiveComponent.SetMaterial` (`Character.Mesh` _asbp_soccer_player) 0 "/Game/Art/Material/Instance_Materials/Color/MI_TeamBlue.MI_TeamBlue")
    (else
      (`PrimitiveComponent.SetMaterial` (`Character.Mesh` _asbp_soccer_player) 0 "/Game/Art/Material/Instance_Materials/Color/MI_TeamRed.MI_TeamRed")))
  (set `WB_PlayerHitComponent.TeamIndex` TeamIndex (`/Game/Blueprint/Character/BP_GenericCharacter.PlayerHitComponent` _asbp_soccer_player))
  (`KismetArrayLibrary.Array_AddUnique` (`self.Players`) _asbp_soccer_player))

(fn `SetAllPlayersState`
  (params (NewState :type "GameplayTag Structure"))
  (for _array_element (`self.Players`)
    (`/Game/Blueprint/Character/BPC_GrabObject.CancelShootCharge` (`/Game/Blueprint/Character/BP_GenericCharacter.BPC_GrabPhysicObject` _array_element))
    (`WB_PlayerStateComponent.ChangePlayerState` (`/Game/Blueprint/Character/BP_GenericCharacter.PlayerStateComponent` _array_element) (`local.NewState`))))

(fn `SetupMatchPlayers`
  (if (< (`GameplayStatics.GetNumLocalPlayerControllers`) 2)
    (`GameplayStatics.CreatePlayer` -1))
  (set `self.PlayerTwo` (`GameplayStatics.GetPlayerController` 1))
  (for _index (range (`GameplayStatics.GetNumLocalPlayerControllers`))
    (bind _teamindex (`self.GetTeamForPlayer` _index))
    (`self.RegisterMatchPlayer` _index _teamindex)))

(fn `StartGoalCelebration`
  (params (ScoringTeamIsRed :type Boolean))
  (for _index (range (`GameplayStatics.GetNumLocalPlayerControllers`))
    (bind _asbp_generic_character (cast `/Game/Blueprint/Character/BP_GenericCharacter` (`GameplayStatics.GetPlayerCharacter` _index)))
    (`/Game/Blueprint/Character/BPC_GrabObject.DropHeldItem` (`/Game/Blueprint/Character/BP_GenericCharacter.BPC_GrabPhysicObject` _asbp_generic_character))
    (bind _teamindex (`self.GetTeamForPlayer` _index))
    (if (== (!= _teamindex 1) (`local.ScoringTeamIsRed`))
      (bind _playerstatecomponent (`/Game/Blueprint/Character/BP_GenericCharacter.PlayerStateComponent` _asbp_generic_character))
      (bind _celebrationduration (`WB_PlayerStateProfile.CelebrationDuration` (`WB_PlayerStateComponent.GetActiveProfile` _playerstatecomponent)))
      (`WB_PlayerStateComponent.ChangePlayerStateForDuration` _playerstatecomponent (struct :`TagName` "Player.State.Celebrating") _celebrationduration)
      (else
        (`WB_PlayerStateComponent.ChangePlayerStateForDuration` _playerstatecomponent (struct :`TagName` "Player.State.Sulking") _celebrationduration)))))

(fn `UserConstructionScript`)