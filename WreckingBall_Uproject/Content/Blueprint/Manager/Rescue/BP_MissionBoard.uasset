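; Mission board for the rescue mode that displays up to five target actors and tracks their rescue through overlaps.
; On BeginPlay it fills the WBP_RescueBoard widget, builds the objective list and passes the insurance policy worth to BP_RescueGM.
; Overlap begin and end toggle targets between complete and pending, adjusting the completed count.
; When completed plus failed reaches the total on an overlap begin, it calls UpdateRescue on the game mode.
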(event `self.ReceiveBeginPlay`
  ;[0 0.1529 1 0.5] BeginPlay
  (`self.InitiateBlackboard`)
  (`self.InitializeObjective`)
  (`self.Cast to Game Mode`))

(event `OverlapBeginBoardUpdate`
  (params (`Overlap Actor` :type "Actor Object Reference"))
  ;[1 0 0.06535 0.5] Overlap
  (for _array_element (`self.Target To Rescue`)
    (if (== _array_element `Overlap Actor`)
      (`/Game/Blueprint/Manager/Rescue/WBP_RescueBoard.Target Complete` (`self.WBP Rescue Board`) `Overlap Actor`)
      (`/Engine/EditorBlueprintResources/StandardMacros.IncrementInt` (`self.Completed Objective`)
        (:`  `
          (if (== (+ (`self.Completed Objective`) (`self.Failed Objective`)) (`self.Total Objective`))
            (`/Game/Blueprint/Manager/BP_RescueGM.Update Rescue` (`self.As BP Rescue GM`) true)))))))

(event `OverlapEndBoardUpdate`
  (params (`Overlap Actor` :type "Actor Object Reference"))
  ;[1 0 0.06535 0.5] Overlap
  (for _array_element (`self.Target To Rescue`)
    (if (== _array_element `Overlap Actor`)
      (`/Game/Blueprint/Manager/Rescue/WBP_RescueBoard.Target Pending` (`self.WBP Rescue Board`) `Overlap Actor`)
      (`/Engine/EditorBlueprintResources/StandardMacros.DecrementInt` (`self.Completed Objective`)))))

(fn `Cast to Game Mode`
  (bind _asbp_rescue_gm (cast `/Game/Blueprint/Manager/BP_RescueGM` (`GameplayStatics.GetGameMode`)))
  (bind _output_get (set `self.As BP Rescue GM` _asbp_rescue_gm))
  (set `/Game/Blueprint/Manager/BP_RescueGM.Insurance Policy Worth` (`self.InsurancePolicy Worth`) _output_get))

(fn `InitializeObjective`
  (bind _output_get (set `self.Target To Rescue` (`|MakeArray` (`self.Target Actor 01`) (`self.Target Actor 02`) (`self.Target Actor 03`) (`self.Target Actor 04`) (`self.Target Actor 05`))))
  (for (_array_element _array_index) _output_get
    (`/Engine/EditorBlueprintResources/StandardMacros.IsValid` _array_element
      (:`Is Not Valid`
        (`KismetArrayLibrary.Array_Remove` (`self.Target To Rescue`) _array_index))))
  (bind _output_get_2 (set `self.Total Objective` (- (`KismetArrayLibrary.Array_Length` (`self.Target To Rescue`)) 1)))
  (`KismetSystemLibrary.PrintString` (`KismetStringLibrary.Conv_IntToString` _output_get_2) true true (struct :`R` 1.0 :`B` 0.887529 :`A` 1.0) 8.0))

(fn `InitiateBlackboard`
  (bind _target_actor_01 (`self.Target Actor 01`))
  (bind _target_actor_05 (`self.Target Actor 05`))
  (bind _target_actor_03 (`self.Target Actor 03`))
  (bind _target_actor_04 (`self.Target Actor 04`))
  (bind _target_actor_02 (`self.Target Actor 02`))
  (bind _aswbp_rescue_board (cast `/Game/Blueprint/Manager/Rescue/WBP_RescueBoard` (`WidgetComponent.GetWidget` (`self.WBP_RescueBoard`))))
  (set `self.WBP Rescue Board` _aswbp_rescue_board)
  (set `/Game/Blueprint/Manager/Rescue/WBP_RescueBoard.RescueTarget` (`|MakeArray` (select `bool` (`KismetSystemLibrary.IsValid` _target_actor_01) :`true` _target_actor_01) (select `bool` (`KismetSystemLibrary.IsValid` _target_actor_02) :`true` _target_actor_02) (select `bool` (`KismetSystemLibrary.IsValid` _target_actor_03) :`true` _target_actor_03) (select `bool` (`KismetSystemLibrary.IsValid` _target_actor_04) :`true` _target_actor_04) (select `bool` (`KismetSystemLibrary.IsValid` _target_actor_05) :`true` _target_actor_05)) _aswbp_rescue_board)
  (set `/Game/Blueprint/Manager/Rescue/WBP_RescueBoard.Display All At Once` (`self.IsDisplayedAllAtOnce`) _aswbp_rescue_board)
  (`/Game/Blueprint/Manager/Rescue/WBP_RescueBoard.DisplayBoard` _aswbp_rescue_board))

(fn `UserConstructionScript`)