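; Game manager for a rescue level that tallies insurance claims on damaged actors and plays random background music.
; InsuranceClaim sums counts and costs by claim and item category, then updates the WBP_InsuranceCount widget with a cha-ching sound.
; UpdateRescue, on completion, blocks further claims, stops music and input, shows the final receipt, then opens a level after a delay.
; The audio-finished binding is unconnected, so tracks do not chain.
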(event `self.ReceiveBeginPlay`
  ;[0 0.1529 1 0.5] Begin Play
  (`self.Play audio`)
  (bind _asbp_generic_character (cast `/Game/Blueprint/Character/Master/BP_GenericCharacter` (`GameplayStatics.GetPlayerCharacter` 0)))
  (set `self.As BP Generic Character` _asbp_generic_character)
  (bind _returnvalue (`|CreateWidget` "/Game/Blueprint/Manager/Insurance/WBP_InsuranceCount.WBP_InsuranceCount_C" (`GameplayStatics.GetPlayerController` 0)))
  (bind _output_get (set `self.Insurance Claim Widget` _returnvalue))
  (`UserWidget.AddToPlayerScreen` _output_get 0))

(event `Play audio`
  ;[1 0 0.06535 0.5] Play Audio
  (bind _returnvalue (`AddComponent|NODE_AddAudioComponent-0`))
  (bind _output_get (set `self.AudioComponentMusic` _returnvalue))
  (`AudioComponent.SetSound` _output_get (`KismetArrayLibrary.Array_Random` (`self.Music`)))
  (`AudioComponent.Play` _returnvalue 0.0)
  (bind _returnvalue_2 (message `AnimationDataModel.GetPlayLength` (`AudioComponent.Sound` _returnvalue)))
  (`KismetSystemLibrary.PrintString` (`KismetStringLibrary.Conv_DoubleToString` _returnvalue_2)))

(event `OnAudioFinished_Event`
  ;[1 0 0.06535 0.5] Play Audio
  (`self.Play audio`))

(event `InsuranceClaim`
  (params (DamagedActor :type "/Game/Blueprint/CombustibleObject/BP_Master_CombustibleObject Object Reference") (InsuranceClaim :type "/Game/Blueprint/Manager/Insurance/STR_InsuranceClaims Structure") (ClaimCategory :type "/Game/Blueprint/Manager/Insurance/E_ClaimCategory Enum" :default "NewEnumerator0"))
  ;[1 0 0.06535 0.5] Insurance Claim
  (if (not (`self.Gameset`))
    (`KismetArrayLibrary.Array_AddUnique` (`self.DamagedActors`) DamagedActor)
    (`self.CalculateClaimCategoryCost` InsuranceClaim ClaimCategory)
    (`self.CalculateItemCategoryCost` InsuranceClaim)
    (`self.DisplayNewClaim` InsuranceClaim ClaimCategory)
    (`self.CalculateTotalCost` InsuranceClaim)
    (`GameplayStatics.PlaySound2D` "/Game/Audio/NotLegitAudio/SFX/Cash/SFX_Cha-Ching.SFX_Cha-Ching" 1.0 1.0 0.0 null null)))

(event `Update Rescue`
  (params (`Is Complete` :type Boolean))
  (bind _returnvalue (`GameplayStatics.GetPlayerController` 0))
  (if `Is Complete`
    (set `self.Gameset` true)
    (`AudioComponent.Stop` (`self.AudioComponentMusic`))
    (`self.DisableInput` _returnvalue _returnvalue)
    (`/Game/Blueprint/Manager/Insurance/WBP_InsuranceCount.Final Receit` (`self.Insurance Claim Widget`))
    (`KismetSystemLibrary.Delay` 15.0)
    (`GameplayStatics.OpenLevelBySoftObjectPtr` (`self.Level`))))

(fn `CalculateClaimCategoryCost`
  (params (`Insurance Claim` :type "/Game/Blueprint/Manager/Insurance/STR_InsuranceClaims Structure") (ClaimCategory :type "/Game/Blueprint/Manager/Insurance/E_ClaimCategory Enum" :default "NewEnumerator0"))
  (bind (_itemcategory _itemcost) (break `/Game/Blueprint/Manager/Insurance/STR_InsuranceClaims` `Insurance Claim`))
  (set `self.Total Item Cost` (+ (`self.Total Item Cost`) _itemcost))
  (switch `/Game/Blueprint/Manager/Insurance/E_ClaimCategory` ClaimCategory
    (:`NewEnumerator0`
      (`/Engine/EditorBlueprintResources/StandardMacros.IncrementInt` (`self.ItemClaimedForFire`)
        (:`  `
          (set `self.ItemCostForFire` (+ (`self.ItemCostForFire`) _itemcost)))))
    (:`NewEnumerator1`
      (`/Engine/EditorBlueprintResources/StandardMacros.IncrementInt` (`self.ItemClaimedForFlood`)
        (:`  `
          (set `self.ItemCostForFlood` (+ (`self.ItemCostForFlood`) _itemcost)))))
    (:`NewEnumerator2`
      (`/Engine/EditorBlueprintResources/StandardMacros.IncrementInt` (`self.ItemClaimedForDemolition`)
        (:`  `
          (set `self.ItemCostForDemolition` (+ (`self.ItemCostForDemolition`) _itemcost)))))
    (:`NewEnumerator3`
      (`/Engine/EditorBlueprintResources/StandardMacros.IncrementInt` (`self.ItemClaimedForTheft`)
        (:`  `
          (set `self.ItemCostForTheft` (+ (`self.ItemCostForTheft`) _itemcost)))))
    (:`NewEnumerator7`
      (`/Engine/EditorBlueprintResources/StandardMacros.IncrementInt` (`self.ItemClaimedForCivicProperty`)
        (:`  `
          (set `self.ItemCostForTheft` (+ (`self.ItemCostForCivicProperty`) _itemcost)))))))

(fn `CalculateItemCategoryCost`
  (params (`Insurance Claim` :type "/Game/Blueprint/Manager/Insurance/STR_InsuranceClaims Structure"))
  (bind (_itemcategory _itemcost) (break `/Game/Blueprint/Manager/Insurance/STR_InsuranceClaims` `Insurance Claim`))
  (switch `/Game/Blueprint/Manager/Insurance/E_ItemCategory` _itemcategory
    (:`NewEnumerator0`
      (`/Engine/EditorBlueprintResources/StandardMacros.IncrementInt` (`self.ClaimedForStructuralItem`)
        (:`  `
          (set `self.CostForStructuralItem` (+ _itemcost (`self.CostForStructuralItem`))))))
    (:`NewEnumerator1`
      (`/Engine/EditorBlueprintResources/StandardMacros.IncrementInt` (`self.ClaimedForPersonalGoods`)
        (:`  `
          (set `self.CostForPersonalGoods` (+ _itemcost (`self.CostForPersonalGoods`))))))
    (:`NewEnumerator2`
      (`/Engine/EditorBlueprintResources/StandardMacros.IncrementInt` (`self.ClaimedForFurnitures`)
        (:`  `
          (set `self.CostForFurniture` (+ _itemcost (`self.CostForFurniture`))))))
    (:`NewEnumerator3`
      (`/Engine/EditorBlueprintResources/StandardMacros.IncrementInt` (`self.ClaimedForHomeAppliances`)
        (:`  `
          (set `self.CostForHomeAppliances` (+ _itemcost (`self.CostForHomeAppliances`))))))
    (:`NewEnumerator4`
      (`/Engine/EditorBlueprintResources/StandardMacros.IncrementInt` (`self.ClaimedForArts`)
        (:`  `
          (set `self.CostForArts` (+ _itemcost (`self.CostForArts`))))))
    (:`NewEnumerator6`
      (`/Engine/EditorBlueprintResources/StandardMacros.IncrementInt` (`self.ClaimedForOutdooring`)
        (:`  `
          (set `self.CostForOutdooring` (+ _itemcost (`self.CostForOutdooring`))))))
    (:`NewEnumerator7`
      (`/Engine/EditorBlueprintResources/StandardMacros.IncrementInt` (`self.ClaimedForVehicles`)
        (:`  `
          (set `self.CostForVehicles` (+ _itemcost (`self.CostForVehicles`))))))
    (:`NewEnumerator8`
      (`/Engine/EditorBlueprintResources/StandardMacros.IncrementInt` (`self.ClaimedForCasualty`)
        (:`  `
          (set `self.CostForCasualty` (+ _itemcost (`self.CostForCasualty`))))))))

(fn `CalculateTotalCost`
  (params (`Insurance Claim` :type "/Game/Blueprint/Manager/Insurance/STR_InsuranceClaims Structure"))
  (bind _output_get (set `self.Total Item Cost` (+ (`self.Total Item Cost`) (`.ItemCost_8_F5EA57B1496839F6C003E6B674DEB6C8` (break `/Game/Blueprint/Manager/Insurance/STR_InsuranceClaims` `Insurance Claim`)))))
  (set `/Game/Blueprint/Manager/Insurance/WBP_InsuranceCount.Total Insurance Claim Cost` _output_get (`self.Insurance Claim Widget`)))

(fn `DisplayNewClaim`
  (params (`Insurance Claim` :type "/Game/Blueprint/Manager/Insurance/STR_InsuranceClaims Structure") (`Claim Category` :type "/Game/Blueprint/Manager/Insurance/E_ClaimCategory Enum" :default "NewEnumerator0"))
  (bind (_itemcategory _itemcost) (break `/Game/Blueprint/Manager/Insurance/STR_InsuranceClaims` `Insurance Claim`))
  (`/Game/Blueprint/Manager/Insurance/WBP_InsuranceCount.New Claim` (`self.Insurance Claim Widget`) `Claim Category` _itemcategory _itemcost))

(fn `UserConstructionScript`)