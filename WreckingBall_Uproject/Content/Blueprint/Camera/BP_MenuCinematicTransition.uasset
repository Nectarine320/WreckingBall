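; BP_MenuCinematicTransition is a placeable actor that defines a cinematic transition between two menu states, identified by FromState and ToState gameplay tags, with an array of sequences.
; The construction script sets a Label text showing both state tags and the sequence count.
; On BeginPlay it prints a misconfiguration warning with its display name when either tag is invalid.
; Nothing in these graphs plays the sequences.
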(event `self.ReceiveBeginPlay`
  (if (or (not (`BlueprintGameplayTagLibrary.IsGameplayTagValid` (`self.FromState`))) (not (`BlueprintGameplayTagLibrary.IsGameplayTagValid` (`self.ToState`))))
    (`KismetSystemLibrary.PrintString` (`KismetStringLibrary.Concat_StrStr` "BP_MenuCinematicTransition mal configure (FromState ou ToState vide) : " (`KismetSystemLibrary.GetDisplayName` self)) true true (struct :`G` 0.66 :`B` 1.0 :`A` 1.0) 10.0)))

(fn `UserConstructionScript`
  (`TextRenderComponent.K2_SetText` (`self.Label`) (`KismetTextLibrary.Conv_StringToText` (`KismetStringLibrary.Concat_StrStr` (`KismetStringLibrary.Concat_StrStr` (`KismetStringLibrary.Concat_StrStr` (`KismetStringLibrary.Concat_StrStr` (`KismetStringLibrary.Concat_StrStr` (`KismetStringLibrary.Conv_NameToString` (`BlueprintGameplayTagLibrary.GetTagName` (`self.FromState`))) "  ->  ") (`KismetStringLibrary.Conv_NameToString` (`BlueprintGameplayTagLibrary.GetTagName` (`self.ToState`)))) "   (sequences: ") (`KismetStringLibrary.Conv_IntToString` (`KismetArrayLibrary.Array_Length` (`self.Sequences`)))) ")"))))