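; Soccer match camera actor that follows the active ball and registers itself as the default camera on the soccer player camera manager.
; A camera profile configures the spring arm and camera at construction and sets arm length every tick.
; Each tick, while the gamemode's ball has collision enabled, the profile computes a target from ball, view and last carrier direction, and the actor eases toward it at the profile's follow speed.
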(event `self.ReceiveBeginPlay`
  (bind _ascamm_soccer_player (cast `/Game/Blueprint/Camera/CAMM_SoccerPlayer` (`GameplayStatics.GetPlayerCameraManager` 0)))
  (bind _output_get (set `self.As CAMM Soccer Player` _ascamm_soccer_player))
  (set `/Game/Blueprint/Camera/CAMM_SoccerPlayer.Default Camera` self _output_get)
  (bind _asbp_soccer_gamemode (cast `/Game/Blueprint/Character/BP_SoccerGamemode` (`GameplayStatics.GetGameMode`)))
  (set `self.As BP Soccer Gamemode` _asbp_soccer_gamemode))

(event `self.ReceiveTick`
  (params (DeltaSeconds :type "Float (single-precision)"))
  (`self.Update CameraLocation`)
  (`self.Update CameraDistance`))

(fn `Update CameraDistance`
  (set `SpringArmComponent.TargetArmLength` (`WB_SoccerCameraProfile.ArmLength` (`self.CameraProfile`)) (`self.SpringArm`)))

(fn `Update CameraLocation`
  (bind _activeball (`/Game/Blueprint/Character/BP_SoccerGamemode.ActiveBall` (`self.As BP Soccer Gamemode`)))
  (`/Engine/EditorBlueprintResources/StandardMacros.IsValid` _activeball
    (:`Is Valid`
      (if (`self.GetActorEnableCollision` _activeball)
        (bind (_outcarrierdirection _returnvalue) (`WB_SoccerCameraProfile.ComputeCameraTarget` (`self.CameraProfile`) _activeball (`self.Camera`) (`self.LastCarrierDirection`)))
        (set `self.LastCarrierDirection` _outcarrierdirection)
        (`self.K2_SetActorLocation` (`KismetMathLibrary.VInterpTo` (`self.K2_GetActorLocation`) _returnvalue (`GameplayStatics.GetWorldDeltaSeconds`) (`WB_SoccerCameraProfile.BallFollowSpeed` (`self.CameraProfile`))))))))

(fn `UserConstructionScript`
  (`WB_SoccerCameraProfile.ApplyCameraProfile` (`self.CameraProfile`) (`self.SpringArm`) (`self.Camera`)))