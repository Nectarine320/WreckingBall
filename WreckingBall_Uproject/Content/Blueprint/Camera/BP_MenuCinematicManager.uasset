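; Front-end menu manager that switches between gameplay-tag menu states through cinematic transitions, listening to state requests from BP_FrontEndGameMode.
; A request finds the transition linking current and target states, playing its sequences forward, or in reverse for the opposite direction.
; The menu layer clears at transition start; once every sequence finishes, it pushes the new state's widget and broadcasts the change.
; Overlapping requests are ignored; switching without a cinematic is optional.
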(event `self.ReceiveBeginPlay`
  (set `self.CurrentState` (`self.InitialState`))
  (for _array_element (`self.Transitions`)
    (for _array_element_2 (`/Game/Blueprint/Camera/BP_MenuCinematicTransition.Sequences` _array_element)
      (add `MovieSceneSequencePlayer.OnFinished` (`LevelSequenceActor.SequencePlayer` _array_element_2) (delegate `OnSequenceFinished`))))
  (if (`self.bPushInitialStateWidget`)
    (`self.ShowStateWidget` (`self.InitialState`)))
  (bind _asbp_front_end_game_mode (cast `/Game/Blueprint/UI/FrontEnd/BP_FrontEndGameMode` (`GameplayStatics.GetGameMode`))
    (:`then`
      (add `/Game/Blueprint/UI/FrontEnd/BP_FrontEndGameMode.OnMenuStateRequested` _asbp_front_end_game_mode (`|CreateDelegate` :!event `RequestMenuState`)))
    (:`CastFailed`
      (`KismetSystemLibrary.PrintString` "BP_MenuCinematicManager: le Game Mode n'est pas BP_FrontEndGameMode, aucune requete de menu ne sera recue"))))

(event `OnSequenceFinished`
  (if (`self.bIsTransitioning`)
    (set `self.PendingSequenceCount` (- (`self.PendingSequenceCount`) 1))
    (if (<= (`self.PendingSequenceCount`) 0)
      (`self.FinishTransition`))))

(fn `FinishTransition`
  (bind _pendingstate (`self.PendingState`))
  (set `self.bIsTransitioning` false)
  (set `self.CurrentState` _pendingstate)
  (`self.ShowStateWidget` _pendingstate)
  (`self.OnMenuStateChanged` _pendingstate))

(fn `RequestMenuState`
  (params (TargetState :type "GameplayTag Structure"))
  (bind _currentstate (`self.CurrentState`))
  (if (or (`self.bIsTransitioning`) (`BlueprintGameplayTagLibrary.MatchesTag` TargetState _currentstate true))
    (`KismetSystemLibrary.PrintString` "BP_MenuCinematicManager: requete ignoree (transition en cours ou deja dans cet etat)" false)
    (else
      (set `self.ActiveTransition` null)
      (set `self.PendingState` TargetState)
      (for _array_element (`self.Transitions`)
        (bind _fromstate (`/Game/Blueprint/Camera/BP_MenuCinematicTransition.FromState` _array_element))
        (bind _tostate (`/Game/Blueprint/Camera/BP_MenuCinematicTransition.ToState` _array_element))
        (if (and (`BlueprintGameplayTagLibrary.MatchesTag` _fromstate _currentstate true) (`BlueprintGameplayTagLibrary.MatchesTag` _tostate TargetState true))
          (set `self.ActiveTransition` _array_element)
          (set `self.bPlayReverse` false)
          (break)
          (elif (and (`BlueprintGameplayTagLibrary.MatchesTag` _fromstate TargetState true) (`BlueprintGameplayTagLibrary.MatchesTag` _tostate _currentstate true))
            (set `self.ActiveTransition` _array_element)
            (set `self.bPlayReverse` true)
            (break))))
      (`/Engine/EditorBlueprintResources/StandardMacros.IsValid` (`self.ActiveTransition`)
        (:`Is Valid`
          (`self.StartTransition`))
        (:`Is Not Valid`
          (if (`self.bAllowDirectSwitchWithoutCinematic`)
            (`self.StartTransition`)
            (else
              (`KismetSystemLibrary.PrintString` "BP_MenuCinematicManager: aucune transition trouvee entre l'etat courant et l'etat demande. Ajoute un BP_MenuCinematicTransition dans Transitions."))))))))

(fn `ShowStateWidget`
  (params (State :type "GameplayTag Structure"))
  (bind (_value _returnvalue) (`BlueprintMapLibrary.Map_Find` (`self.StateWidgets`) State))
  (if _returnvalue
    (`/Game/Blueprint/UI/BPFL_UI.PushContentToLayer` (`GameplayStatics.GetPlayerController` 0) (`self.MenuLayer`) _value)))

(fn `StartTransition`
  (bind _activetransition (`self.ActiveTransition`))
  (bind _sequences (`/Game/Blueprint/Camera/BP_MenuCinematicTransition.Sequences` _activetransition))
  (set `self.bIsTransitioning` true)
  (`/Game/Blueprint/UI/BPFL_UI.ClearLayer` (`GameplayStatics.GetPlayerController` 0) (`self.MenuLayer`))
  (set `self.PendingSequenceCount` 0)
  (`/Engine/EditorBlueprintResources/StandardMacros.IsValid` _activetransition
    (:`Is Valid`
      (set `self.PendingSequenceCount` (`KismetArrayLibrary.Array_Length` _sequences))
      (if (> (`self.PendingSequenceCount`) 0)
        (for _array_element _sequences
          (if (`self.bPlayReverse`)
            (bind _sequenceplayer (`LevelSequenceActor.SequencePlayer` _array_element))
            (`MovieSceneSequencePlayer.PlayReverse` _sequenceplayer)
            (else
              (`MovieSceneSequencePlayer.Play` _sequenceplayer))))
        (else
          (`self.FinishTransition`))))
    (:`Is Not Valid`
      (`self.FinishTransition`))))

(fn `UserConstructionScript`)