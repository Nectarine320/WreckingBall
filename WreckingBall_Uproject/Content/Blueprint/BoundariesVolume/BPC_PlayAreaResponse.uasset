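; Actor component that handles its owner leaving the play area, responding by gameplay tag: remove, return to start or respawn.
; HandleLeftPlayArea ignores exits still overlapping a matching BP_PlayAreaVolume, otherwise starts a delay timer, hiding and freezing non-Remove owners.
; Remove destroys the owner unless it has re-entered by timeout.
; Respawn picks randomly among the three closest tag-matched BP_RespawnPoints, preferring unoccupied ones and falling back to the start location.
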(event `self.ReceiveBeginPlay`
  ;[0 0.1529 1 0.5] Begin Play
  (`self.InitializeResponse`))

(event `StartOutOfBoundsResponse`
  ;[0 1 0.07739 0.5] Tick - When ball is out.
  (bind _returnvalue (`KismetSystemLibrary.K2_SetTimerDelegate` (delegate `FinishOutOfBoundsResponse`) (`self.ResponseDelay`)))
  (set `self.ResponseTimer` _returnvalue))

(event `FinishOutOfBoundsResponse`
  ;[0 1 0.07739 0.5] Tick - When ball is out.
  (`self.FinishResponse`))

(fn `CacheRespawnPoints`
  (bind _outactors (`GameplayStatics.GetAllActorsOfClass` "/Game/Blueprint/BoundariesVolume/BP_RespawnPoint.BP_RespawnPoint_C"))
  (for _array_element _outactors
    (if (`BlueprintGameplayTagLibrary.MatchesTag` (`/Game/Blueprint/BoundariesVolume/BP_RespawnPoint.PointTag` _array_element) (`self.RespawnPointTag`) true)
      (`KismetArrayLibrary.Array_Add` (`self.RespawnPoints`) _array_element))))

(fn `FinishResponse`
  (if (`BlueprintGameplayTagLibrary.MatchesTag` (`self.ResponseTag`) (struct :`TagName` "OutOfBounds.Response.Remove") true)
    (bind _isinside (`self.IsInsideWatchedArea`))
    (if _isinside
      (set `self.IsResponding` false)
      (`self.OnResponseFinished` self (`self.ResponseTag`))
      (else
        (`self.OnResponseFinished` self (`self.ResponseTag`))
        (`Actor.K2_DestroyActor` (`self.GetOwner` self))))
    (else
      (`self.MoveOwnerForResponse`)
      (`self.SetOwnerActive` true)
      (set `self.IsResponding` false)
      (`self.OnResponseFinished` self (`self.ResponseTag`)))))

(fn `GetClosestPointIndex`
  (params (Points :type "Array of /Game/Blueprint/BoundariesVolume/BP_RespawnPoint Object Reference") (FromLocation :type "Vector Structure"))
  (returns (Index :type Integer))
  (locals (BestIndex :type Integer) (BestDistance :type "Float (double-precision)"))
  (set `local.BestIndex` -1)
  (set `local.BestDistance` 1000000000.0)
  (for _index (range (`KismetArrayLibrary.Array_Length` Points))
    (bind _returnvalue (`KismetMathLibrary.Vector_Distance` (`Actor.K2_GetActorLocation` (`|GetArrayItem` Points _index)) FromLocation))
    (if (< _returnvalue (`local.BestDistance`))
      (set `local.BestDistance` _returnvalue)
      (set `local.BestIndex` _index)))
  (return (`local.BestIndex`)))

(fn `HandleLeftPlayArea`
  (params (Location :type "Vector Structure"))
  (bind _isinside (`self.IsInsideWatchedArea`))
  (if (not (or (`self.IsResponding`) _isinside))
    (set `self.IsResponding` true)
    (set `self.ExitLocation` Location)
    (`self.OnResponseStarted` self (`self.ResponseTag`))
    (if (not (`BlueprintGameplayTagLibrary.MatchesTag` (`self.ResponseTag`) (struct :`TagName` "OutOfBounds.Response.Remove") true))
      (`self.SetOwnerActive` false))
    (`self.StartOutOfBoundsResponse`)))

(fn `InitializeResponse`
  (set `self.StartTransform` (`Actor.GetTransform` (`self.GetOwner` self))))

(fn `IsInsideWatchedArea`
  (returns (IsInside :type Boolean))
  (for _array_element (`Actor.GetOverlappingActors` (`self.GetOwner` self) "/Game/Blueprint/BoundariesVolume/BP_PlayAreaVolume.BP_PlayAreaVolume_C")
    (if (`BlueprintGameplayTagLibrary.MatchesTag` (`/Game/Blueprint/BoundariesVolume/BP_PlayAreaVolume.AreaTag` _array_element) (`self.WatchedAreaTag`) true)
      (return true)))
  (return false))

(fn `IsPointFree`
  (params (Point :type "/Game/Blueprint/BoundariesVolume/BP_RespawnPoint Object Reference"))
  (returns (IsFree :type Boolean))
  (bind (_outactors _returnvalue) (`KismetSystemLibrary.SphereOverlapActors` (`Actor.K2_GetActorLocation` Point) (`self.FreePointRadius`) (`|MakeArray` "ObjectTypeQuery3" "ObjectTypeQuery4" :!type "EObjectTypeQuery Enum") null (`|MakeArray` (`self.GetOwner` self))))
  (return (not _returnvalue)))

(fn `MoveOwnerForResponse`
  (if (`BlueprintGameplayTagLibrary.MatchesTag` (`self.ResponseTag`) (struct :`TagName` "OutOfBounds.Response.ReturnToStart") true)
    (`Actor.K2_SetActorTransform` (`self.GetOwner` self) (`self.StartTransform`) false true)
    (else
      (bind _location (`self.PickRespawnLocation` (`self.ExitLocation`)))
      (`Actor.K2_SetActorLocation` (`self.GetOwner` self) _location false true))))

(fn `PickRespawnLocation`
  (params (FromLocation :type "Vector Structure"))
  (returns (Location :type "Vector Structure"))
  (locals (Candidates :type "Array of /Game/Blueprint/BoundariesVolume/BP_RespawnPoint Object Reference") (Closest :type "Array of /Game/Blueprint/BoundariesVolume/BP_RespawnPoint Object Reference"))
  (if (`KismetArrayLibrary.Array_IsEmpty` (`self.RespawnPoints`))
    (`self.CacheRespawnPoints`))
  (if (`KismetArrayLibrary.Array_IsEmpty` (`self.RespawnPoints`))
    (return (+ (.location (`self.StartTransform`)) (`KismetMathLibrary.MakeVector` 0.0 0.0 (`self.RespawnDropHeight`))))
    (else
      (for _array_element (`self.RespawnPoints`)
        (bind _isfree (`self.IsPointFree` _array_element))
        (if _isfree
          (`KismetArrayLibrary.Array_Add` (`local.Candidates`) _array_element)))
      (if (`KismetArrayLibrary.Array_IsEmpty` (`local.Candidates`))
        (set `local.Candidates` (`self.RespawnPoints`)))
      (for _ (range 3)
        (if (not (`KismetArrayLibrary.Array_IsEmpty` (`local.Candidates`)))
          (bind _index (`self.GetClosestPointIndex` (`local.Candidates`) FromLocation))
          (`KismetArrayLibrary.Array_Add` (`local.Closest`) (`|GetArrayItem` (`local.Candidates`) _index))
          (`KismetArrayLibrary.Array_Remove` (`local.Candidates`) _index)))
      (return (+ (`Actor.K2_GetActorLocation` (`|GetArrayItem` (`local.Closest`) (`KismetMathLibrary.RandomIntegerInRange` 0 (- (`KismetArrayLibrary.Array_Length` (`local.Closest`)) 1)))) (`KismetMathLibrary.MakeVector` 0.0 0.0 (`self.RespawnDropHeight`)))))))

(fn `SetOwnerActive`
  (params (Active :type Boolean))
  (bind _returnvalue (`self.GetOwner` self))
  (bind _returnvalue_2 (and Active (`self.WasSimulatingPhysics`)))
  (bind _rootcomponent (`Actor.RootComponent` _returnvalue))
  (if (not Active)
    (set `self.WasSimulatingPhysics` (`SceneComponent.IsSimulatingPhysics` _rootcomponent "None")))
  (`Actor.SetActorHiddenInGame` _returnvalue (not Active))
  (`Actor.SetActorEnableCollision` _returnvalue Active)
  (bind _asprimitive_component (cast `PrimitiveComponent` _rootcomponent))
  (`PrimitiveComponent.SetSimulatePhysics` _asprimitive_component _returnvalue_2)
  (if _returnvalue_2
    (`PrimitiveComponent.SetPhysicsLinearVelocity` _asprimitive_component (`KismetMathLibrary.MakeVector` 0.0) false "None")
    (`PrimitiveComponent.SetPhysicsAngularVelocityInDegrees` _asprimitive_component (`KismetMathLibrary.MakeVector` 0.0) false "None")))