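; BP_PlayAreaVolume is a tagged boundary volume that reports when actors, such as the ball, leave a play area.
; On end overlap, it finds the leaving actor's BPC_PlayAreaResponse components and calls HandleLeftPlayArea with the actor's location on those whose WatchedAreaTag exactly matches its AreaTag.
; The construction script sets the area's shape color according to whether the tag is PlayArea.Ball.
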(event `self.ReceiveActorEndOverlap`
  (params (OtherActor :type "Actor Object Reference"))
  ; Update when ball is out.
  (`self.NotifyLeftPlayArea` OtherActor))

(fn `NotifyLeftPlayArea`
  (params (LeavingActor :type "Actor Object Reference"))
  (for _array_element (`self.K2_GetComponentsByClass` LeavingActor "/Game/Blueprint/BoundariesVolume/BPC_PlayAreaResponse.BPC_PlayAreaResponse_C")
    (if (`BlueprintGameplayTagLibrary.MatchesTag` (`/Game/Blueprint/BoundariesVolume/BPC_PlayAreaResponse.WatchedAreaTag` _array_element) (`self.AreaTag`) true)
      (`/Game/Blueprint/BoundariesVolume/BPC_PlayAreaResponse.HandleLeftPlayArea` _array_element (`self.K2_GetActorLocation` LeavingActor)))))

(fn `UserConstructionScript`
  (if (`BlueprintGameplayTagLibrary.MatchesTag` (`self.AreaTag`) (struct :`TagName` "PlayArea.Ball") true)
    (set `ShapeComponent.ShapeColor` (struct :`B` 255 :`G` 120 :`R` 40 :`A` 255) (`self.Area`))
    (else
      (set `ShapeComponent.ShapeColor` (struct :`B` 160 :`G` 160 :`R` 160 :`A` 255) (`self.Area`)))))