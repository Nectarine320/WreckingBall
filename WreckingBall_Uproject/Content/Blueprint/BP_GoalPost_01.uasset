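; Team goal post for a soccer mode that detects the ball entering its box and awards the score to the opposing team.
; A ball overlap calls Goal on the ball and UpdateScore on the soccer game mode, gated by a DoOnce until EnableGoal re-arms it.
; The construction script uses IsRedTeam to set the post's team material and the goal component's defending team index.
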(event `self.ReceiveBeginPlay`
  (bind _asbp_soccer_gamemode (cast `/Game/Blueprint/Character/BP_SoccerGamemode` (`GameplayStatics.GetGameMode`)))
  (set `self. BP Soccer Gamemode` _asbp_soccer_gamemode))

(event `self.Box.OnComponentBeginOverlap`
  (params (OverlappedComponent :type "PrimitiveComponent Object Reference") (OtherActor :type "Actor Object Reference") (OtherComp :type "PrimitiveComponent Object Reference") (OtherBodyIndex :type Integer) (bFromSweep :type Boolean) (SweepResult :type "HitResult Structure (by ref)"))
  (bind _asbp_po_master_ball_01 (cast `/Game/Blueprint/Ball/BP_PO_Master_Ball_01` OtherActor))
  (`/Engine/EditorBlueprintResources/StandardMacros.DoOnce` false :!label _label
    (:`Completed`
      (`/Game/Blueprint/Ball/BP_PO_Master_Ball_01.Goal` _asbp_po_master_ball_01 self)
      (`/Game/Blueprint/Character/BP_SoccerGamemode.Update Score` (`self. BP Soccer Gamemode`) (not (`self.Is Red Team`))))))

(event `Enable Goal`
  (goto _label :!via `Reset`))

(fn `UserConstructionScript`
  (`PrimitiveComponent.SetMaterial` (`self.SM_GoalPost`) 1 (select `bool` (`self.Is Red Team`) :`false` "/Game/Art/Material/Instance_Materials/Color/MI_TeamBlue.MI_TeamBlue" :`true` "/Game/Art/Material/Instance_Materials/Color/MI_TeamRed.MI_TeamRed" :!type "MaterialInterface Object Reference"))
  (set `WB_TeamGoalComponent.DefendingTeamIndex` (select `bool` (`self.Is Red Team`) :`false` 1) (`self.TeamGoalComponent`)))