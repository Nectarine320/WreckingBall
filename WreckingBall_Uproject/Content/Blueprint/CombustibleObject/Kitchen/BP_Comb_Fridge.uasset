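; BP_Comb_Fridge is a combustible kitchen fridge assembled from three child-actor parts: a body, a bottom door and a top door.
; On BeginPlay it casts each child actor to BP_M_PhysicObject and stores the references.
; Two physics constraints then join the body's combustible mesh to each door's mesh at runtime, so the doors are physically attached to the fridge.
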(event `self.ReceiveBeginPlay`
  (bind _asbp_master_combustible_object (cast `/Game/Blueprint/CombustibleObject/BP_M_PhysicObject` (`ChildActorComponent.ChildActor` (`self.BP_Comb_FridgePart_01`))))
  (set `self.As BP Fridge` _asbp_master_combustible_object)
  (bind _asbp_master_combustible_object_2 (cast `/Game/Blueprint/CombustibleObject/BP_M_PhysicObject` (`ChildActorComponent.ChildActor` (`self.BP_Comb_FridgePart_02`))))
  (set `self.As BP Fridge Door Bot` _asbp_master_combustible_object_2)
  (bind _asbp_master_combustible_object_3 (cast `/Game/Blueprint/CombustibleObject/BP_M_PhysicObject` (`ChildActorComponent.ChildActor` (`self.BP_Comb_FridgePart_03`))))
  (set `self.As BP Fridge Door Top` _asbp_master_combustible_object_3)
  (`PhysicsConstraintComponent.SetConstrainedComponents` (`self.PhysicsConstraint`) (`/Game/Blueprint/CombustibleObject/BP_M_PhysicObject.SM_CombustibleObject` (`self.As BP Fridge`)) "None" (`/Game/Blueprint/CombustibleObject/BP_M_PhysicObject.SM_CombustibleObject` (`self.As BP Fridge Door Bot`)) "None")
  (`PhysicsConstraintComponent.SetConstrainedComponents` (`self.PhysicsConstraint1`) (`/Game/Blueprint/CombustibleObject/BP_M_PhysicObject.SM_CombustibleObject` (`self.As BP Fridge`)) "None" (`/Game/Blueprint/CombustibleObject/BP_M_PhysicObject.SM_CombustibleObject` (`self.As BP Fridge Door Top`)) "None"))

(fn `UserConstructionScript`)