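; BP_Comb_Oven is a kitchen oven in the combustible object set, assembled from a body and a door.
; Two child actor components supply the parts, each cast to BP_M_PhysicObject on BeginPlay.
; A PhysicsConstraint then binds their SMCombustibleObject components at runtime, linking the door to the oven body as separate physics objects.
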(event `self.ReceiveBeginPlay`
  (bind _asbp_master_combustible_object (cast `/Game/Blueprint/CombustibleObject/BP_M_PhysicObject` (`ChildActorComponent.ChildActor` (`self.BP_Comb_OverPart_01`))))
  (set `self.As BP Oven` _asbp_master_combustible_object)
  (bind _asbp_master_combustible_object_2 (cast `/Game/Blueprint/CombustibleObject/BP_M_PhysicObject` (`ChildActorComponent.ChildActor` (`self.BP_Comb_OverPart_02`))))
  (set `self.As BP Oven Door` _asbp_master_combustible_object_2)
  (`PhysicsConstraintComponent.SetConstrainedComponents` (`self.PhysicsConstraint`) (`/Game/Blueprint/CombustibleObject/BP_M_PhysicObject.SM_CombustibleObject` (`self.As BP Oven`)) "None" (`/Game/Blueprint/CombustibleObject/BP_M_PhysicObject.SM_CombustibleObject` (`self.As BP Oven Door`)) "None"))

(fn `UserConstructionScript`)