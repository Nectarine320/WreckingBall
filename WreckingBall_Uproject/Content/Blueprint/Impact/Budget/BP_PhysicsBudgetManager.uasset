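; BP_PhysicsBudgetManager caps how many collapsed walls keep their physics debris in the world at once.
; RegisterCollapsedWall adds each wall once to a CollapsedWalls queue and, when a valid Budget exists, evicts entries until the count fits its MaxCollapsedWalls.
; ClearOldestWall removes the first entry and calls HideDebrisAfterLifetime on it if still valid, so the earliest collapses are cleared first.
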(fn `ClearOldestWall`
  (locals (OldestWall :type "/Game/Blueprint/Impact/Destructible/BP_Destructible_Wall_Base Object Reference"))
  (set `local.OldestWall` (`|GetArrayItem` (`self.CollapsedWalls`)))
  (`KismetArrayLibrary.Array_Remove` (`self.CollapsedWalls`))
  (`/Engine/EditorBlueprintResources/StandardMacros.IsValid` (`local.OldestWall`)
    (:`Is Valid`
      (`/Game/Blueprint/Impact/Destructible/BP_Destructible_Wall_Base.HideDebrisAfterLifetime` (`local.OldestWall`)))))

(fn `RegisterCollapsedWall`
  (params (Wall :type "/Game/Blueprint/Impact/Destructible/BP_Destructible_Wall_Base Object Reference"))
  (`KismetArrayLibrary.Array_AddUnique` (`self.CollapsedWalls`) Wall)
  (`/Engine/EditorBlueprintResources/StandardMacros.IsValid` (`self.Budget`)
    (:`Is Valid`
      (while (> (`KismetArrayLibrary.Array_Length` (`self.CollapsedWalls`)) (`/Game/Blueprint/Impact/Budget/PDA_PhysicsBudget.MaxCollapsedWalls` (`self.Budget`)))
        (`self.ClearOldestWall`)))))

(fn `UserConstructionScript`)