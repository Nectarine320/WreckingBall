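; Blueprint function library for destruction that converts an impact into damage and kinetic energy.
; Impact speed is either full velocity magnitude or its component along the hit normal, depending on impact type.
; Kinetic energy comes from mass and that speed converted to m/s, then a float curve maps it to damage, scaled by a multiplier.
; Damage is zero below the minimum speed or without a valid curve, but energy is always returned.
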(fn `ComputeImpactDamage`
  (params (ImpactData :type "/Game/Blueprint/Impact/STR_ImpactData Structure") (MassKg :type "Float (double-precision)") (DamageMultiplier :type "Float (double-precision)") (MinImpactSpeed :type "Float (double-precision)") (EnergyToDamageCurve :type "CurveFloat Object Reference"))
  (returns (Damage :type "Float (double-precision)") (Energy :type "Float (double-precision)"))
  (bind (_location _normal _velocity) (break `/Game/Blueprint/Impact/STR_ImpactData` ImpactData))
  (bind (_location_2 _normal_2 _velocity_2 _source _instigator _impacttype) (break `/Game/Blueprint/Impact/STR_ImpactData` (`local.ImpactData`)))
  (bind _returnvalue (`KismetMathLibrary.SelectFloat` (`KismetMathLibrary.VSize` _velocity_2) (`KismetMathLibrary.Abs` (`KismetMathLibrary.Dot_VectorVector` _velocity (`KismetMathLibrary.Normal` _normal))) (`|EnumEquality` _impacttype "NewEnumerator1")))
  (bind _returnvalue_2 (* (* 0.5 MassKg) (`KismetMathLibrary.Square` (/ _returnvalue 100.0))))
  (`/Engine/EditorBlueprintResources/StandardMacros.IsValid` EnergyToDamageCurve
    (:`Is Valid`
      (if (>= _returnvalue (`local.MinImpactSpeed`))
        (return (* (`CurveFloat.GetFloatValue` EnergyToDamageCurve _returnvalue_2) (`local.DamageMultiplier`)) _returnvalue_2)
        (else
          (return 0.0 _returnvalue_2))))
    (:`Is Not Valid`
      (return 0.0 _returnvalue_2))))