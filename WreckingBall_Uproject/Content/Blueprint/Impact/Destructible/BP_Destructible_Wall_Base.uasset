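; Base destructible wall with two Geometry Collection sides around a static middle mesh, configured by a wall profile data asset.
; Blocker hits feed the parent impact pipeline, with the impact normal picking the side for damage eligibility, surface feedback and crack decals.
; On destruction it clears decals, collapses destructible sides and tagged trims, and swaps the middle mesh.
; Blocker collision turns off only when both sides are destructible and the profile allows it.
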(event `self.Blockers.OnBlockerHit`
  (params (HitComponent :type "PrimitiveComponent Object Reference") (OtherActor :type "Actor Object Reference") (OtherComp :type "PrimitiveComponent Object Reference") (NormalImpulse :type "Vector Structure") (Hit :type "HitResult Structure (by ref)"))
  ;[1 0 0.06535 0.5] On Hit trigger
  (bind _impactdata (`self.BuildImpactDataFromHit` OtherActor Hit OtherComp NormalImpulse))
  (`/Game/Blueprint/Interfaces/BPI_ImpactReceiver.ApplyImpact` _impactdata))

(event `CollapseSides`
  ;[2 1.759 0.1667 0.5] Simulation - Collapse plaster
  (`self.CollapseSide` 1.0)
  (`self.CollapseSide` -1.0))

(fn `ApplyDestroyedMiddleMesh`
  (`/Engine/EditorBlueprintResources/StandardMacros.IsValid` (`self.MiddleMeshDestroyed`)
    (:`Is Valid`
      (`StaticMeshComponent.SetStaticMesh` (`self.SM_MiddleMesh`) (`self.MiddleMeshDestroyed`))
      (`WB_DestructibleLibrary.ApplyMaterialOverrides` (`self.SM_MiddleMesh`) (`self.MiddleMaterialOverrides`))
      (`WB_DestructibleLibrary.ApplyMaterialOverrides` (`self.SM_MiddleMesh`) (`self.MiddleDestroyedMaterialOverrides`)))))

(fn `ApplyWallProfile`
  (locals (CurrentWallProfile :type "/Game/Blueprint/Impact/Destructible/PDA_DestructibleWallProfile Object Reference"))
  (set `local.CurrentWallProfile` (`self.GetWallProfile`))
  (`WB_DestructibleLibrary.SyncMaterialOverrides` (`self.GC_SideA`) (`self.SideAMaterialOverrides`))
  (`WB_DestructibleLibrary.SyncMaterialOverrides` (`self.GC_SideB`) (`self.SideBMaterialOverrides`))
  (`WB_DestructibleLibrary.SyncMaterialOverrides` (`self.SM_MiddleMesh`) (`self.MiddleMaterialOverrides`)))

(fn `BreakSideAtImpact`
  (params (ImpactData :type "/Game/Blueprint/Impact/STR_ImpactData Structure") (Damage :type "Float (double-precision)"))
  (bind (_location _normal) (break `/Game/Blueprint/Impact/STR_ImpactData` (`local.ImpactData`)))
  (bind (_location_2 _normal_2) (break `/Game/Blueprint/Impact/STR_ImpactData` (`local.ImpactData`)))
  (`/Engine/EditorBlueprintResources/StandardMacros.IsValid` (`self.GetWallProfile`)
    (:`Is Valid`
      (switch `/Game/Blueprint/Impact/E_Wallside` (`self.GetImpactSide` (`local.ImpactData`))
        (:`NewEnumerator1`
          (bind _returnvalue (`GameplayStatics.SpawnDecalAttached` (`/Game/Blueprint/Impact/Destructible/PDA_DestructibleWallProfile.CrackDecalMaterial` (`self.GetWallProfile`)) (`KismetMathLibrary.MakeVector` 20.0 (`self.LocalBreakHalfSize`) (`self.LocalBreakHalfSize`)) (`self.SideAPivot`) "None" _location (`KismetMathLibrary.Conv_VectorToRotator` _normal) "KeepWorldPosition"))
          (`KismetArrayLibrary.Array_Add` (`self.CrackDecals`) _returnvalue))
        (:`NewEnumerator2`
          (bind _returnvalue_2 (`GameplayStatics.SpawnDecalAttached` (`/Game/Blueprint/Impact/Destructible/PDA_DestructibleWallProfile.CrackDecalMaterial` (`self.GetWallProfile`)) (`KismetMathLibrary.MakeVector` 20.0 (`self.LocalBreakHalfSize`) (`self.LocalBreakHalfSize`)) (`self.SideBPivot`) "None" _location_2 (`KismetMathLibrary.Conv_VectorToRotator` _normal_2) "KeepWorldPosition"))
          (`KismetArrayLibrary.Array_Add` (`self.CrackDecals`) _returnvalue_2))))))

(fn `CanTakeDamageFrom`
  (params (ImpactNormal :type "Vector Structure"))
  (returns (CanTakeDamage :type Boolean))
  (bind _returnvalue (`WB_DestructibleLibrary.GetSideFromNormal` self (`local.ImpactNormal`)))
  (if (== _returnvalue 0)
    (bind _destructible (`self.IsSideDestructible` 1.0))
    (bind _destructible_2 (`self.IsSideDestructible` -1.0))
    (return (or _destructible _destructible_2))
    (else
      (bind _destructible_3 (`self.IsSideDestructible` (`KismetMathLibrary.Conv_IntToDouble` _returnvalue)))
      (return _destructible_3))))

(fn `ClearCrackDecals`
  (for _array_element (`self.CrackDecals`)
    (`ActorComponent.K2_DestroyComponent` _array_element))
  (`KismetArrayLibrary.Array_Clear` (`self.CrackDecals`)))

(fn `CollapseSide`
  (params (SideSign :type "Float (double-precision)"))
  (bind _wallprofile (`self.GetWallProfile`))
  (bind _destructible (`self.IsSideDestructible` (`local.SideSign`)))
  (if _destructible
    (`WB_DestructibleLibrary.CollapseGeometryCollection` (select `bool` (>= (`local.SideSign`) 0.0) :`false` (`self.GC_SideB`) :`true` (`self.GC_SideA`)) (`self.GetActorBounds` false) (`/Game/Blueprint/Impact/Destructible/PDA_DestructibleWallProfile.CollapseImpulseRadius` _wallprofile) (`self.CollapseImpulseStrength`) (`/Game/Blueprint/Impact/Destructible/PDA_DestructibleWallProfile.DebrisLifetime` _wallprofile))))

(fn `CollapseTrims`
  (bind _destructible (`self.IsSideDestructible` 1.0))
  (bind _destructible_2 (`self.IsSideDestructible` -1.0))
  (if (or _destructible _destructible_2)
    (for _array_element (`self.GetComponentsByTag` "/Script/GeometryCollectionEngine.GeometryCollectionComponent" (`self.TrimTag`))
      (`WB_DestructibleLibrary.CollapseGeometryCollection` _array_element (`self.GetActorBounds` self false false) (`/Game/Blueprint/Impact/Destructible/PDA_DestructibleWallProfile.CollapseImpulseRadius` (`self.GetWallProfile`)) (`self.CollapseImpulseStrength`) (`/Game/Blueprint/Impact/Destructible/PDA_DestructibleWallProfile.DebrisLifetime` (`self.GetWallProfile`))))))

(fn `DisableBlockersIfOpen`
  (bind _destructible (`self.IsSideDestructible` 1.0))
  (bind _destructible_2 (`self.IsSideDestructible` -1.0))
  (if (and (and _destructible _destructible_2) (`/Game/Blueprint/Impact/Destructible/PDA_DestructibleWallProfile.DisableBlockerOnDestroyed` (`self.GetWallProfile`)))
    (`WB_DestructibleBlockersComponent.SetBlockersCollisionEnabled` (`self.Blockers`) "NoCollision")))

(fn `GetAttachSurfaceForSide`
  (params (SideSign :type "Float (double-precision)"))
  (returns (Surface :type "SceneComponent Object Reference"))
  (return (select `bool` (>= SideSign 0.0) :`false` (`self.SideBPivot`) :`true` (`self.SideAPivot`))))

(fn `GetImpactSide`
  (params (ImpactData :type "/Game/Blueprint/Impact/STR_ImpactData Structure"))
  (returns (Side :type "/Game/Blueprint/Impact/E_Wallside Enum"))
  (bind _returnvalue (`KismetMathLibrary.Dot_VectorVector` (`.Normal_5_12160DF741D20ABA0B31FFB05AB1541D` (break `/Game/Blueprint/Impact/STR_ImpactData` (`local.ImpactData`))) (`self.GetActorRightVector`)))
  (if (> _returnvalue 0.5)
    (return "NewEnumerator1")
    (elif (< _returnvalue -0.5)
      (return "NewEnumerator2")
      (else
        (return "NewEnumerator0")))))

(fn `GetWallProfile`
  (returns (WallProfile :type "/Game/Blueprint/Impact/Destructible/PDA_DestructibleWallProfile Object Reference"))
  (bind _aspda_destructible_wall_profile (cast `/Game/Blueprint/Impact/Destructible/PDA_DestructibleWallProfile` (`self.Profile`))
    (:`then`
      (return _aspda_destructible_wall_profile))
    (:`CastFailed`
      (return null))))

(fn `InitializeDestructible`
  (returns (Handled :type Boolean))
  (`parent.InitializeDestructible`)
  (add `self.OnDamaged` (`|CreateDelegate` :!event `BreakSideAtImpact`))
  (return true))

(fn `IsSideDestructible`
  (params (SideSign :type "Float (double-precision)"))
  (returns (Destructible :type Boolean))
  (bind _wallprofile (`self.GetWallProfile`))
  (`/Engine/EditorBlueprintResources/StandardMacros.IsValid` _wallprofile
    (:`Is Valid`
      (return (select `bool` (>= (`local.SideSign`) 0.0) :`false` (`/Game/Blueprint/Impact/Destructible/PDA_DestructibleWallProfile.SideBDestructible` _wallprofile) :`true` (`/Game/Blueprint/Impact/Destructible/PDA_DestructibleWallProfile.SideADestructible` _wallprofile))))
    (:`Is Not Valid`
      (return true))))

(fn `OnEnterDamaged`
  (params (ImpactData :type "/Game/Blueprint/Impact/STR_ImpactData Structure"))
  (returns (Handled :type Boolean))
  (`parent.OnEnterDamaged` ImpactData)
  (set `self.LastHitSide` (`self.GetImpactSide` (`local.ImpactData`)))
  (if (`self.DebugPrint`)
    (`KismetSystemLibrary.PrintString` (`KismetStringLibrary.Concat_StrStr` "Wall side hit: " (`|GetEnumeratorNameAsString` (`self.LastHitSide`))) true true (struct :`G` 0.66 :`B` 1.0 :`A` 1.0) 4.0))
  (return true))

(fn `OnEnterDestroyed`
  (params (ImpactData :type "/Game/Blueprint/Impact/STR_ImpactData Structure"))
  (returns (Handled :type Boolean))
  (`parent.OnEnterDestroyed` ImpactData)
  (`/Engine/EditorBlueprintResources/StandardMacros.IsValid` (`self.GetWallProfile`)
    (:`Is Valid`
      (`self.ClearCrackDecals`)
      (`self.CollapseSides`)
      (`self.CollapseTrims`)
      (`self.ApplyDestroyedMiddleMesh`)
      (`self.DisableBlockersIfOpen`)
      (return true))
    (:`Is Not Valid`
      (return true))))

(fn `PlayImpactFeedback`
  (params (ImpactData :type "/Game/Blueprint/Impact/STR_ImpactData Structure") (IsHeavy :type Boolean))
  (returns (Handled :type Boolean))
  (bind (_location _normal _velocity _source _instigator _impacttype _surfacetype) (break `/Game/Blueprint/Impact/STR_ImpactData` ImpactData))
  (bind _wallprofile (`self.GetWallProfile`))
  (bind _handled (`parent.PlayImpactFeedback` (make `/Game/Blueprint/Impact/STR_ImpactData` _location _normal _velocity _source _instigator _impacttype (`WB_DestructibleLibrary.GetWallSideSurface` null _normal (`/Game/Blueprint/Impact/Destructible/PDA_DestructibleWallProfile.SideAPhysicalMaterial` _wallprofile) (`/Game/Blueprint/Impact/Destructible/PDA_DestructibleWallProfile.SideBPhysicalMaterial` _wallprofile) _surfacetype)) IsHeavy))
  (return _handled))

(fn `UserConstructionScript`
  (`parent.UserConstructionScript`)
  (`self.ApplyWallProfile`))