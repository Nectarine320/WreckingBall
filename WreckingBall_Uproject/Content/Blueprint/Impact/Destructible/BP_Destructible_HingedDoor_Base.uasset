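; Base Blueprint for a destructible hinged door that turns impacts into lock damage and tears the door off when destroyed.
; Blocker hits are converted to impact data and applied through the destructible impact system.
; Damage events pass damage, location and normal to the HingedDoor component to weaken the lock.
; Entering the destroyed state runs the parent logic, then tears the door off at the impact point.
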(event `self.ReceiveBeginPlay`
  (`parent.ReceiveBeginPlay`)
  (add `self.OnDamaged` (`|CreateDelegate` :!event `HandleDoorDamaged`)))

(event `self.Blockers.OnBlockerHit`
  (params (HitComponent :type "PrimitiveComponent Object Reference") (OtherActor :type "Actor Object Reference") (OtherComp :type "PrimitiveComponent Object Reference") (NormalImpulse :type "Vector Structure") (Hit :type "HitResult Structure (by ref)"))
  (bind _impactdata (`self.BuildImpactDataFromHit` OtherActor Hit OtherComp NormalImpulse))
  (`/Game/Blueprint/Interfaces/BPI_ImpactReceiver.ApplyImpact` _impactdata))

(fn `HandleDoorDamaged`
  (params (ImpactData :type "/Game/Blueprint/Impact/STR_ImpactData Structure") (Damage :type "Float (double-precision)"))
  (bind (_location _normal) (break `/Game/Blueprint/Impact/STR_ImpactData` ImpactData))
  (`WB_HingedDoorComponent.ApplyLockDamage` (`self.HingedDoor`) (`local.Damage`) _location _normal))

(fn `OnEnterDestroyed`
  (params (ImpactData :type "/Game/Blueprint/Impact/STR_ImpactData Structure"))
  (returns (Handled :type Boolean))
  (bind (_location _normal) (break `/Game/Blueprint/Impact/STR_ImpactData` ImpactData))
  (`parent.OnEnterDestroyed` ImpactData)
  (`WB_HingedDoorComponent.TearOff` (`self.HingedDoor`) _location _normal)
  (return true))

(fn `UserConstructionScript`
  (`parent.UserConstructionScript`))