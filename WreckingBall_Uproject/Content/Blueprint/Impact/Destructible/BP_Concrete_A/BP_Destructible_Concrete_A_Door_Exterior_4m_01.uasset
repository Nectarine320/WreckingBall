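; Destructible 4m exterior concrete door piece that carries a hinged door as a child actor and exposes per-instance settings for it.
; After the parent construction script, it pushes the starts-locked flag onto the child door's hinged door component.
; It then syncs material overrides onto the child door's mesh.
; All of this runs at construction; the event graph holds only disabled stubs.
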(fn `ApplyDoorLock`
  (bind _aswb_hinged_door_component (cast `WB_HingedDoorComponent` (`self.GetComponentByClass` (`ChildActorComponent.ChildActor` (`self.Dependent_Door`)) "/Script/WreckingBall.WB_HingedDoorComponent")))
  (set `WB_HingedDoorComponent.bStartsLocked` (`self.DoorStartsLocked`) _aswb_hinged_door_component))

(fn `ApplyDoorMaterials`
  (bind _asbp_destructible_hinged_door_base (cast `/Game/Blueprint/Impact/Destructible/BP_Destructible_HingedDoor_Base` (`ChildActorComponent.ChildActor` (`self.Dependent_Door`))))
  (`WB_DestructibleLibrary.SyncMaterialOverrides` (`/Game/Blueprint/Impact/Destructible/BP_Destructible_HingedDoor_Base.DoorMesh` _asbp_destructible_hinged_door_base) (`self.DoorMaterialOverrides`)))

(fn `UserConstructionScript`
  (`parent.UserConstructionScript`)
  (`self.ApplyDoorLock`)
  (`self.ApplyDoorMaterials`))