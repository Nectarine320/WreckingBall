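; Base Blueprint for destructible objects that lose health from physical impacts and move through Intact, Damaged and Destroyed states.
; ApplyImpact gates hits by per-source cooldown and side checks, then derives damage from the source's physics profile via an energy curve, with a dash override.
; Accepted hits update state, notify dependents and play heavy feedback and wobble; weak hits get light feedback.
; Stub functions like CanTakeDamageFrom and OnEnterDamaged serve as child hooks.
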(event `self.ReceiveBeginPlay`
  ;[0 0.1529 1 0.5] Being Play
  (`self.InitializeDestructible`))

(fn `ApplyImpact`
  (params (ImpactData :type "/Game/Blueprint/Impact/STR_ImpactData Structure"))
  (returns (Accepted :type Boolean))
  (locals (Damage :type "Float (double-precision)") (SourceProfile :type "/Game/Blueprint/Ball/Data/PDA_PhysicsProfile Object Reference"))
  (bind (_location _normal) (break `/Game/Blueprint/Impact/STR_ImpactData` (`local.ImpactData`)))
  (bind (_location_2 _normal_2 _velocity _source _instigator _impacttype) (break `/Game/Blueprint/Impact/STR_ImpactData` (`local.ImpactData`)))
  (if (`WB_DestructibleLibrary.IsDestructionEnabled`)
    (`/Engine/EditorBlueprintResources/StandardMacros.IsValid` (`self.Profile`)
      (:`Is Valid`
        (if (`|EnumInequality` (`self.CurrentState`) "NewEnumerator2")
          (bind (_sourceprofile _candamage) (`self.GetSourceProfile` (`.Source_19_C3FB2C5644D3FDFB63B35D9730502CB7` (break `/Game/Blueprint/Impact/STR_ImpactData` (`local.ImpactData`)))))
          (set `local.SourceProfile` _sourceprofile)
          (if _candamage
            (bind _registered (`self.TryRegisterHit` (`.Source_19_C3FB2C5644D3FDFB63B35D9730502CB7` (break `/Game/Blueprint/Impact/STR_ImpactData` (`local.ImpactData`)))))
            (if _registered
              (bind _cantakedamage (`self.CanTakeDamageFrom` (`.Normal_5_12160DF741D20ABA0B31FFB05AB1541D` (break `/Game/Blueprint/Impact/STR_ImpactData` (`local.ImpactData`)))))
              (if _cantakedamage
                (`/Engine/EditorBlueprintResources/StandardMacros.IsValid` (`local.SourceProfile`)
                  (:`Is Valid`
                    (set `local.Damage` (`WB_PlayerCommandComponent.ResolveDashImpactDamage` (`|EnumEquality` _impacttype "NewEnumerator1") _source _velocity (`/Game/Blueprint/Impact/BPFL_Destruction.ComputeImpactDamage` (`local.ImpactData`) (`/Game/Blueprint/Ball/Data/PDA_PhysicsProfile.MassKg` (`local.SourceProfile`)) (`/Game/Blueprint/Ball/Data/PDA_PhysicsProfile.DamageMultiplier` (`local.SourceProfile`)) (`/Game/Blueprint/Ball/Data/PDA_PhysicsProfile.MinImpactSpeed` (`local.SourceProfile`)) (`/Game/Blueprint/Impact/Destructible/PDA_DestructibleProfile.EnergyToDamageCurve` (`self.Profile`)))))
                    (if (>= (`local.Damage`) (`/Game/Blueprint/Impact/Destructible/PDA_DestructibleProfile.MinDamagePerHit` (`self.Profile`)))
                      (bind _newhealth (`self.ComputeNewHealth` (`local.Damage`) (`/Game/Blueprint/Ball/Data/PDA_PhysicsProfile.MaxStatesPerHit` (`local.SourceProfile`))))
                      (set `self.CurrentHealth` (`KismetMathLibrary.FMax` _newhealth))
                      (`self.PlayImpactFeedback` (`local.ImpactData`) true)
                      (`self.OnDamaged` (`local.ImpactData`) (`local.Damage`))
                      (`self.ReactToDamage` _location _normal (`local.Damage`))
                      (bind _state (`self.GetStateForHealth` (`self.CurrentHealth`)))
                      (`self.SetDestructibleState` _state (`local.ImpactData`))
                      (`self.PrintImpactDebug` (`local.Damage`) (`local.ImpactData`))
                      (`WB_FeedbackLibrary.PlayFeedback` (struct :`TagName` "Feedback.Impact.Accepted") (`.Source_19_C3FB2C5644D3FDFB63B35D9730502CB7` (break `/Game/Blueprint/Impact/STR_ImpactData` (`local.ImpactData`))))
                      (return true)
                      (else
                        (`self.PlayImpactFeedback` (`local.ImpactData`))
                        (`self.PlayMinorHitWobble` (`local.ImpactData`) (`local.Damage`))
                        (`self.PrintImpactDebug` (`local.Damage`) (`local.ImpactData`))
                        (return false))))
                  (:`Is Not Valid`
                    _)))
              (`self.PlayImpactFeedback` (`local.ImpactData`))
              (return false)
              (else
                (return false)))
            (else
              (return false)))
          (else
            (return false))))
      (:`Is Not Valid`
        _)))
  (return false))

(fn `BuildImpactDataFromHit`
  (params (OtherActor :type "Actor Object Reference") (Hit :type "HitResult Structure") (OtherComp :type "PrimitiveComponent Object Reference") (NormalImpulse :type "Vector Structure"))
  (returns (ImpactData :type "/Game/Blueprint/Impact/STR_ImpactData Structure"))
  (bind _otheractor (`local.OtherActor`))
  (bind _otheractor_2 (`local.OtherActor`))
  (bind _otheractor_3 (`local.OtherActor`))
  (bind _returnvalue (`self.GetVelocity` (`local.OtherActor`)))
  (bind (_bblockinghit _binitialoverlap _time _distance _location _impactpoint _normal _impactnormal) (`GameplayStatics.BreakHitResult` (`local.Hit`)))
  (bind (_bblockinghit_2 _binitialoverlap_2 _time_2 _distance_2 _location_2 _impactpoint_2 _normal_2 _impactnormal_2) (`GameplayStatics.BreakHitResult` (`local.Hit`)))
  (bind (_bblockinghit_3 _binitialoverlap_3 _time_3 _distance_3 _location_3 _impactpoint_3 _normal_3 _impactnormal_3) (`GameplayStatics.BreakHitResult` (`local.Hit`)))
  (bind _returnvalue_2 (/ (`local.NormalImpulse`) (`KismetMathLibrary.FMax` (`PrimitiveComponent.GetMass` (`local.OtherComp`)) 0.01)))
  (bind _returnvalue_3 (+ _returnvalue _returnvalue_2))
  (bind _returnvalue_4 (- _returnvalue _returnvalue_2))
  (`/Engine/EditorBlueprintResources/StandardMacros.IsValid` (`local.OtherComp`)
    (:`Is Valid`
      (if (`SceneComponent.IsSimulatingPhysics` (`local.OtherComp`) "None")
        (return (make `/Game/Blueprint/Impact/STR_ImpactData` _impactpoint (`WB_DestructibleLibrary.OrientNormalTowardSource` _impactnormal _impactpoint _otheractor) (select `bool` (> (`KismetMathLibrary.VSize` _returnvalue_4) (`KismetMathLibrary.VSize` _returnvalue_3)) :`false` _returnvalue_4 :`true` _returnvalue_3) _otheractor null "NewEnumerator0" (`GameplayStatics.GetSurfaceType` (`local.Hit`))))
        (else
          (return (make `/Game/Blueprint/Impact/STR_ImpactData` _impactpoint_2 (`WB_DestructibleLibrary.OrientNormalTowardSource` _impactnormal_2 _impactpoint_2 _otheractor_2) (`self.GetVelocity` (`local.OtherActor`)) _otheractor_2 null "NewEnumerator0" (`GameplayStatics.GetSurfaceType` (`local.Hit`)))))))
    (:`Is Not Valid`
      (return (make `/Game/Blueprint/Impact/STR_ImpactData` _impactpoint_3 (`WB_DestructibleLibrary.OrientNormalTowardSource` _impactnormal_3 _impactpoint_3 _otheractor_3) (`self.GetVelocity` (`local.OtherActor`)) _otheractor_3 null "NewEnumerator0" (`GameplayStatics.GetSurfaceType` (`local.Hit`)))))))

(fn `CanTakeDamageFrom`
  (params (ImpactNormal :type "Vector Structure"))
  (returns (CanTakeDamage :type Boolean))
  (return true))

(fn `ComputeNewHealth`
  (params (Damage :type "Float (double-precision)") (MaxStatesPerHit :type Integer))
  (returns (NewHealth :type "Float (double-precision)"))
  (bind _returnvalue (- (`self.CurrentHealth`) Damage))
  (switch `/Game/Blueprint/Impact/E_DestructibleState` (`self.CurrentState`)
    (:`NewEnumerator0`
      (if (< MaxStatesPerHit 2)
        (return (`KismetMathLibrary.FMax` _returnvalue 1.0))
        (else
          (return _returnvalue))))
    (:`NewEnumerator1`
      (return _returnvalue))
    (:`NewEnumerator2`
      (return _returnvalue))))

(fn `GetAttachSurfaceForSide`
  (params (SideSign :type "Float (double-precision)"))
  (returns (Surface :type "SceneComponent Object Reference"))
  (return (`self.RootComponent`)))

(fn `GetFeedbackFX`
  (params (Feedback :type "/Game/Blueprint/Impact/PDA_ImpactFeedback Object Reference") (Surface :type "EPhysicalSurface Enum" :default "SurfaceType_Default") (IsHeavy :type Boolean))
  (returns (FX :type "NiagaraSystem Object Reference"))
  (bind (_value _returnvalue) (`BlueprintMapLibrary.Map_Find` (`/Game/Blueprint/Impact/PDA_ImpactFeedback.HeavyFX` (`local.Feedback`)) (`local.Surface`)))
  (bind (_value_2 _returnvalue_2) (`BlueprintMapLibrary.Map_Find` (`/Game/Blueprint/Impact/PDA_ImpactFeedback.LightFX` (`local.Feedback`)) (`local.Surface`)))
  (`/Engine/EditorBlueprintResources/StandardMacros.IsValid` (`local.Feedback`)
    (:`Is Valid`
      (if (`local.IsHeavy`)
        (return (select `bool` _returnvalue :`false` (`BlueprintMapLibrary.Map_Find` (`/Game/Blueprint/Impact/PDA_ImpactFeedback.HeavyFX` (`local.Feedback`)) "SurfaceType_Default") :`true` _value))
        (else
          (return (select `bool` _returnvalue_2 :`false` (`BlueprintMapLibrary.Map_Find` (`/Game/Blueprint/Impact/PDA_ImpactFeedback.LightFX` (`local.Feedback`)) "SurfaceType_Default") :`true` _value_2)))))
    (:`Is Not Valid`
      (return null))))

(fn `GetFeedbackSound`
  (params (Feedback :type "/Game/Blueprint/Impact/PDA_ImpactFeedback Object Reference") (Surface :type "EPhysicalSurface Enum" :default "SurfaceType_Default") (IsHeavy :type Boolean))
  (returns (Sound :type "SoundBase Object Reference"))
  (bind (_value _returnvalue) (`BlueprintMapLibrary.Map_Find` (`/Game/Blueprint/Impact/PDA_ImpactFeedback.HeavySounds` (`local.Feedback`)) (`local.Surface`)))
  (bind (_value_2 _returnvalue_2) (`BlueprintMapLibrary.Map_Find` (`/Game/Blueprint/Impact/PDA_ImpactFeedback.LightSounds` (`local.Feedback`)) (`local.Surface`)))
  (`/Engine/EditorBlueprintResources/StandardMacros.IsValid` (`local.Feedback`)
    (:`Is Valid`
      (if (`local.IsHeavy`)
        (return (select `bool` _returnvalue :`false` (`BlueprintMapLibrary.Map_Find` (`/Game/Blueprint/Impact/PDA_ImpactFeedback.HeavySounds` (`local.Feedback`)) "SurfaceType_Default") :`true` _value))
        (else
          (return (select `bool` _returnvalue_2 :`false` (`BlueprintMapLibrary.Map_Find` (`/Game/Blueprint/Impact/PDA_ImpactFeedback.LightSounds` (`local.Feedback`)) "SurfaceType_Default") :`true` _value_2)))))
    (:`Is Not Valid`
      (return null))))

(fn `GetSourceProfile`
  (params (Source :type "Actor Object Reference"))
  (returns (SourceProfile :type "/Game/Blueprint/Ball/Data/PDA_PhysicsProfile Object Reference") (CanDamage :type Boolean))
  (if (`KismetSystemLibrary.DoesImplementInterface` Source "/Game/Blueprint/Interfaces/BPI_ImpactSource.BPI_ImpactSource_C")
    (bind _candamage (message `/Game/Blueprint/Interfaces/BPI_ImpactSource.CanDealImpactDamage` Source))
    (bind _profile (message `/Game/Blueprint/Interfaces/BPI_ImpactSource.GetPhysicsProfile` Source))
    (return _profile _candamage)
    (else
      (return (`self.DebugFallbackSourceProfile`) true))))

(fn `GetStateForHealth`
  (params (Health :type "Float (double-precision)"))
  (returns (State :type "/Game/Blueprint/Impact/E_DestructibleState Enum"))
  (if (<= (`local.Health`) 0.0)
    (return "NewEnumerator2")
    (elif (< (* (/ (`local.Health`) (* (`/Game/Blueprint/Impact/Destructible/PDA_DestructibleProfile.MaxHealth` (`self.Profile`)) (`self.HealthMultiplier`))) 100.0) (`/Game/Blueprint/Impact/Destructible/PDA_DestructibleProfile.DamagedThresholdPercent` (`self.Profile`)))
      (return "NewEnumerator1")
      (else
        (return "NewEnumerator0")))))

(fn `InitializeDestructible`
  (returns (Handled :type Boolean))
  (bind _profile (`self.Profile`))
  (set `self.CurrentState` "NewEnumerator0")
  (`/Engine/EditorBlueprintResources/StandardMacros.IsValid` _profile
    (:`Is Valid`
      (set `self.CurrentHealth` (* (`/Game/Blueprint/Impact/Destructible/PDA_DestructibleProfile.MaxHealth` _profile) (`self.HealthMultiplier`)))
      (return true))
    (:`Is Not Valid`
      (return false))))

(fn `IsSideDestructible`
  (params (SideSign :type "Float (double-precision)"))
  (returns (Destructible :type Boolean))
  (return true))

(fn `OnEnterDamaged`
  (params (ImpactData :type "/Game/Blueprint/Impact/STR_ImpactData Structure"))
  (returns (Handled :type Boolean))
  (return false))

(fn `OnEnterDestroyed`
  (params (ImpactData :type "/Game/Blueprint/Impact/STR_ImpactData Structure"))
  (returns (Handled :type Boolean))
  (`WB_DestructibleLibrary.NotifyDependentsDestroyed` self)
  (`WB_FeedbackLibrary.PlayFeedback` (struct :`TagName` "Feedback.Destruction") (`.Source_19_C3FB2C5644D3FDFB63B35D9730502CB7` (break `/Game/Blueprint/Impact/STR_ImpactData` (`local.ImpactData`))))
  (return false))

(fn `PlayImpactFeedback`
  (params (ImpactData :type "/Game/Blueprint/Impact/STR_ImpactData Structure") (IsHeavy :type Boolean))
  (returns (Handled :type Boolean))
  (bind (_location _normal _velocity _source _instigator _impacttype _surfacetype) (break `/Game/Blueprint/Impact/STR_ImpactData` (`local.ImpactData`)))
  (bind (_location_2 _normal_2 _velocity_2 _source_2 _instigator_2 _impacttype_2 _surfacetype_2) (break `/Game/Blueprint/Impact/STR_ImpactData` (`local.ImpactData`)))
  (bind (_location_3 _normal_3) (break `/Game/Blueprint/Impact/STR_ImpactData` (`local.ImpactData`)))
  (bind _impactfeedback (`/Game/Blueprint/Impact/Destructible/PDA_DestructibleProfile.ImpactFeedback` (`self.Profile`)))
  (`/Engine/EditorBlueprintResources/StandardMacros.IsValid` (`self.Profile`)
    (:`Is Valid`
      (bind _sound (`self.GetFeedbackSound` (`/Game/Blueprint/Impact/Destructible/PDA_DestructibleProfile.ImpactFeedback` (`self.Profile`)) (select `bool` (`|EnumEquality` _surfacetype "SurfaceType_Default") :`false` _surfacetype :`true` (`/Game/Blueprint/Impact/Destructible/PDA_DestructibleProfile.SurfaceType` (`self.Profile`))) (`local.IsHeavy`)))
      (`GameplayStatics.PlaySoundAtLocation` _sound (`.Location_2_D59D6FBE46C7A7483A69D18B3893A402` (break `/Game/Blueprint/Impact/STR_ImpactData` (`local.ImpactData`))) (struct) (`KismetMathLibrary.RandomFloatInRange` (`/Game/Blueprint/Impact/PDA_ImpactFeedback.VolumeMin` _impactfeedback) (`/Game/Blueprint/Impact/PDA_ImpactFeedback.VolumeMax` _impactfeedback)) (`KismetMathLibrary.RandomFloatInRange` (`/Game/Blueprint/Impact/PDA_ImpactFeedback.PitchMin` _impactfeedback) (`/Game/Blueprint/Impact/PDA_ImpactFeedback.PitchMax` _impactfeedback)) 0.0 (`/Game/Blueprint/Impact/PDA_ImpactFeedback.SoundAttenuation` _impactfeedback) (`/Game/Blueprint/Impact/PDA_ImpactFeedback.SoundConcurrency` _impactfeedback) null null)
      (bind _fx (`self.GetFeedbackFX` (`/Game/Blueprint/Impact/Destructible/PDA_DestructibleProfile.ImpactFeedback` (`self.Profile`)) (select `bool` (`|EnumEquality` _surfacetype_2 "SurfaceType_Default") :`false` _surfacetype_2 :`true` (`/Game/Blueprint/Impact/Destructible/PDA_DestructibleProfile.SurfaceType` (`self.Profile`))) (`local.IsHeavy`)))
      (`NiagaraFunctionLibrary.SpawnSystemAtLocation` _fx _location_3 (`KismetMathLibrary.MakeRotFromX` _normal_3) (1.0 1.0 1.0) true true "AutoRelease")
      (return true))
    (:`Is Not Valid`
      (return false))))

(fn `PlayMinorHitWobble`
  (params (ImpactData :type "/Game/Blueprint/Impact/STR_ImpactData Structure") (Damage :type "Float (double-precision)"))
  (bind _returnvalue (`self.GetComponentByClass` "/Script/WreckingBall.WB_WobbleComponent"))
  (`/Engine/EditorBlueprintResources/StandardMacros.IsValid` _returnvalue
    (:`Is Valid`
      (`WB_WobbleComponent.StartMinorHitWobbleFromNormal` _returnvalue (`.Normal_5_12160DF741D20ABA0B31FFB05AB1541D` (break `/Game/Blueprint/Impact/STR_ImpactData` (`local.ImpactData`))) (`local.Damage`) (`/Game/Blueprint/Impact/Destructible/PDA_DestructibleProfile.Wobble` (`self.Profile`))))))

(fn `PrintImpactDebug`
  (params (Damage :type "Float (double-precision)") (ImpactData :type "/Game/Blueprint/Impact/STR_ImpactData Structure"))
  (bind (_location _normal _velocity) (break `/Game/Blueprint/Impact/STR_ImpactData` (`local.ImpactData`)))
  (if (`self.DebugPrint`)
    (bind _sourceprofile (`self.GetSourceProfile` (`.Source_19_C3FB2C5644D3FDFB63B35D9730502CB7` (break `/Game/Blueprint/Impact/STR_ImpactData` (`local.ImpactData`)))))
    (bind _masskg (`/Game/Blueprint/Ball/Data/PDA_PhysicsProfile.MassKg` _sourceprofile))
    (`KismetSystemLibrary.PrintString` (`KismetStringLibrary.Concat_StrStr` (`KismetStringLibrary.Concat_StrStr` (`KismetStringLibrary.Concat_StrStr` (`KismetStringLibrary.Concat_StrStr` (`KismetStringLibrary.Concat_StrStr` (`KismetStringLibrary.Concat_StrStr` (`KismetStringLibrary.Concat_StrStr` (`KismetStringLibrary.Concat_StrStr` (`KismetStringLibrary.Concat_StrStr` (`KismetStringLibrary.Concat_StrStr` (`KismetStringLibrary.Concat_StrStr` (`KismetStringLibrary.Concat_StrStr` (`KismetSystemLibrary.GetDisplayName` self) " | mass ") (`KismetStringLibrary.Conv_IntToString` (`KismetMathLibrary.Round` _masskg))) " kg | energy ") (`KismetStringLibrary.Conv_IntToString` (`KismetMathLibrary.Round` (`.Energy` (`/Game/Blueprint/Impact/BPFL_Destruction.ComputeImpactDamage` (`local.ImpactData`) _masskg (`/Game/Blueprint/Ball/Data/PDA_PhysicsProfile.DamageMultiplier` _sourceprofile) (`/Game/Blueprint/Ball/Data/PDA_PhysicsProfile.MinImpactSpeed` _sourceprofile) (`/Game/Blueprint/Impact/Destructible/PDA_DestructibleProfile.EnergyToDamageCurve` (`self.Profile`))))))) " J | speed ") (`KismetStringLibrary.Conv_IntToString` (`KismetMathLibrary.Round` (`KismetMathLibrary.Abs` (`KismetMathLibrary.Dot_VectorVector` _velocity (`KismetMathLibrary.Normal` _normal)))))) " cm/s | damage ") (`KismetStringLibrary.Conv_IntToString` (`KismetMathLibrary.Round` (`local.Damage`)))) (`KismetMathLibrary.SelectString` " | ACCEPTED" " | REFUSED" (>= (`local.Damage`) (`/Game/Blueprint/Impact/Destructible/PDA_DestructibleProfile.MinDamagePerHit` (`self.Profile`))))) " | health ") (`KismetStringLibrary.Conv_IntToString` (`KismetMathLibrary.Round` (`self.CurrentHealth`)))) (`KismetStringLibrary.Concat_StrStr` " | " (`|GetEnumeratorNameAsString` (`self.CurrentState`)))) true true (struct :`G` 0.66 :`B` 1.0 :`A` 1.0) 4.0)))

(fn `ReactToDamage`
  (params (ImpactLocation :type "Vector Structure") (ImpactNormal :type "Vector Structure") (Damage :type "Float (double-precision)"))
  (bind _returnvalue (`self.GetComponentByClass` "/Script/WreckingBall.WB_WobbleComponent"))
  (`WB_DestructibleLibrary.NotifyDependentsDamaged` self (`local.ImpactLocation`) (`local.ImpactNormal`) (`local.Damage`))
  (`/Engine/EditorBlueprintResources/StandardMacros.IsValid` _returnvalue
    (:`Is Valid`
      (`WB_WobbleComponent.StartWobbleFromNormal` _returnvalue (`local.ImpactNormal`) (`local.Damage`) (`/Game/Blueprint/Impact/Destructible/PDA_DestructibleProfile.Wobble` (`self.Profile`))))))

(fn `SetDestructibleState`
  (params (NewState :type "/Game/Blueprint/Impact/E_DestructibleState Enum" :default "NewEnumerator0") (ImpactData :type "/Game/Blueprint/Impact/STR_ImpactData Structure"))
  (if (`|EnumInequality` (`local.NewState`) (`self.CurrentState`))
    (set `self.CurrentState` (`local.NewState`))
    (`self.OnStateChanged` (`local.NewState`) (`local.ImpactData`))
    (switch `/Game/Blueprint/Impact/E_DestructibleState` (`local.NewState`)
      (:`NewEnumerator1`
        (`self.OnEnterDamaged` (`local.ImpactData`)))
      (:`NewEnumerator2`
        (`self.OnEnterDestroyed` (`local.ImpactData`))
        (`self.OnBroken` self (`local.ImpactData`))))))

(fn `TryRegisterHit`
  (params (Source :type "Actor Object Reference"))
  (returns (Registered :type Boolean))
  (bind _returnvalue (`KismetSystemLibrary.GetGameTimeInSeconds`))
  (bind (_value _returnvalue_2) (`BlueprintMapLibrary.Map_Find` (`self.LastHitTimes`) Source))
  (if (and _returnvalue_2 (< (- _returnvalue _value) (`/Game/Blueprint/Impact/Destructible/PDA_DestructibleProfile.HitCooldown` (`self.Profile`))))
    (return false)
    (else
      (`BlueprintMapLibrary.Map_Add` (`self.LastHitTimes`) Source _returnvalue)
      (return true))))

(fn `UserConstructionScript`)