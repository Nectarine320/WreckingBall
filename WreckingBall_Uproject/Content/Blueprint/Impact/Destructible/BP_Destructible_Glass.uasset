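; Destructible glass Blueprint that shatters when destroyed by an impact or by the loss of the parent it depends on.
; Blocker hits become impact data fed to the inherited impact logic, while parent damage starts a profile-driven wobble.
; Entering the destroyed state hides the glass mesh, disables blocker collision and spawns the glass profile's shatter effect at the impact location, oriented along impact velocity.
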(event `self.Blockers.OnBlockerHit`
  (params (HitComponent :type "PrimitiveComponent Object Reference") (OtherActor :type "Actor Object Reference") (OtherComp :type "PrimitiveComponent Object Reference") (NormalImpulse :type "Vector Structure") (Hit :type "HitResult Structure (by ref)"))
  (bind _impactdata (`self.BuildImpactDataFromHit` OtherActor Hit OtherComp NormalImpulse))
  (`/Game/Blueprint/Interfaces/BPI_ImpactReceiver.ApplyImpact` _impactdata))

(event `self.Dependent.ParentDestroyed`
  (params (Parent :type "Actor Object Reference"))
  (`self.ShatterFromParentDestroyed`))

(event `self.Dependent.ParentDamaged`
  (params (Parent :type "Actor Object Reference") (ImpactLocation :type "Vector Structure") (ImpactNormal :type "Vector Structure") (Damage :type "Float (single-precision)"))
  (`WB_WobbleComponent.StartWobbleFromNormal` (`self.Wobble`) ImpactNormal Damage (`/Game/Blueprint/Impact/Destructible/PDA_DestructibleProfile.Wobble` (`self.Profile`))))

(fn `OnEnterDestroyed`
  (params (ImpactData :type "/Game/Blueprint/Impact/STR_ImpactData Structure"))
  (returns (Handled :type Boolean))
  (bind (_location _normal _velocity) (break `/Game/Blueprint/Impact/STR_ImpactData` ImpactData))
  (`parent.OnEnterDestroyed` ImpactData)
  (`self.ShatterGlass` _location _velocity)
  (return true))

(fn `ShatterFromParentDestroyed`
  (`self.SetDestructibleState` "NewEnumerator2" (make `/Game/Blueprint/Impact/STR_ImpactData` (`self.K2_GetActorLocation`) (0.0 0.0 0.0) (0.0 0.0 0.0) null null "NewEnumerator0" "SurfaceType5")))

(fn `ShatterGlass`
  (params (ImpactLocation :type "Vector Structure") (ImpactDirection :type "Vector Structure"))
  (`SceneComponent.SetVisibility` (`self.GlassMesh`) false false)
  (`WB_DestructibleBlockersComponent.SetBlockersCollisionEnabled` (`self.Blockers`) "NoCollision")
  (bind _aspda_destructible_glass_profile (cast `/Game/Blueprint/Impact/Destructible/PDA_DestructibleGlassProfile` (`self.Profile`)))
  (`NiagaraFunctionLibrary.SpawnSystemAtLocation` (`/Game/Blueprint/Impact/Destructible/PDA_DestructibleGlassProfile.ShatterFX` _aspda_destructible_glass_profile) (`local.ImpactLocation`) (`KismetMathLibrary.MakeRotFromX` (`local.ImpactDirection`))))

(fn `UserConstructionScript`
  (`parent.UserConstructionScript`))