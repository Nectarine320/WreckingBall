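; BP_Destructible_Column is a destructible column with a static beam mesh and a Geometry Collection cover, configured by a column profile data asset.
; Construction applies the profile's meshes and material overrides.
; Blocker hits become impact data for inherited impact handling.
; Entering the destroyed state collapses the cover with a profile-tuned impulse from the blocker's location and can disable blocker collision, while the beam mesh is left untouched.
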(event `self.Blocker.OnComponentHit`
  (params (HitComponent :type "PrimitiveComponent Object Reference") (OtherActor :type "Actor Object Reference") (OtherComp :type "PrimitiveComponent Object Reference") (NormalImpulse :type "Vector Structure") (Hit :type "HitResult Structure (by ref)"))
  ;[1 0 0.06535 0.5] On Hit Blocker
  (bind _impactdata (`self.BuildImpactDataFromHit` OtherActor Hit OtherComp NormalImpulse))
  (`/Game/Blueprint/Interfaces/BPI_ImpactReceiver.ApplyImpact` _impactdata))

(fn `ApplyColumnProfile`
  (bind _aspda_destructible_column_profile (cast `/Game/Blueprint/Impact/Destructible/PDA_DestructibleColumnProfile` (`self.Profile`)))
  (`StaticMeshComponent.SetStaticMesh` (`self.SM_BeamMesh`) (`/Game/Blueprint/Impact/Destructible/PDA_DestructibleColumnProfile.BeamMesh` _aspda_destructible_column_profile))
  (`GeometryCollectionComponent.SetRestCollection` (`self.GC_Cover`) (`/Game/Blueprint/Impact/Destructible/PDA_DestructibleColumnProfile.CoverGeometryCollection` _aspda_destructible_column_profile) false)
  (`WB_DestructibleLibrary.ApplyMaterialOverrides` (`self.SM_BeamMesh`) (`/Game/Blueprint/Impact/Destructible/PDA_DestructibleColumnProfile.BeamMaterials` _aspda_destructible_column_profile))
  (`WB_DestructibleLibrary.ApplyMaterialOverrides` (`self.GC_Cover`) (`/Game/Blueprint/Impact/Destructible/PDA_DestructibleColumnProfile.CoverMaterials` _aspda_destructible_column_profile)))

(fn `CollapseCover`
  (bind _aspda_destructible_column_profile (cast `/Game/Blueprint/Impact/Destructible/PDA_DestructibleColumnProfile` (`self.Profile`)))
  (`WB_DestructibleLibrary.CollapseGeometryCollection` (`self.GC_Cover`) (`SceneComponent.K2_GetComponentLocation` (`self.Blocker`)) (`/Game/Blueprint/Impact/Destructible/PDA_DestructibleColumnProfile.CollapseImpulseRadius` _aspda_destructible_column_profile) (`/Game/Blueprint/Impact/Destructible/PDA_DestructibleColumnProfile.CollapseImpulseStrength` _aspda_destructible_column_profile) (`/Game/Blueprint/Impact/Destructible/PDA_DestructibleColumnProfile.DebrisLifetime` _aspda_destructible_column_profile))
  (if (`/Game/Blueprint/Impact/Destructible/PDA_DestructibleColumnProfile.DisableBlockerOnDestroyed` _aspda_destructible_column_profile)
    (`PrimitiveComponent.SetCollisionEnabled` (`self.Blocker`) "NoCollision")))

(fn `GetAttachSurfaceForSide`
  (params (SideSign :type "Float (double-precision)"))
  (returns (Surface :type "SceneComponent Object Reference"))
  (return (`self.Pivot`)))

(fn `OnEnterDestroyed`
  (params (ImpactData :type "/Game/Blueprint/Impact/STR_ImpactData Structure"))
  (returns (Handled :type Boolean))
  (`parent.OnEnterDestroyed` ImpactData)
  (`self.CollapseCover`)
  (return true))

(fn `UserConstructionScript`
  (`parent.UserConstructionScript`)
  (`self.ApplyColumnProfile`))