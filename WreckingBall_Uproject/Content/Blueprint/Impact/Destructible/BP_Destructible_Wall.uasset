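; Destructible wall actor with a middle mesh and two geometry collection plaster sides, configured from a wall profile data asset.
; Construction applies the profile's meshes and side material overrides, then fits the Blocker box to the middle mesh or a default size.
; Blocker hits feed the inherited impact system.
; Entering Damaged records the side hit via normal dot right vector; Destroyed hides both plaster sides and optionally disables Blocker collision.
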(event `self.Blocker.OnComponentHit`
  (params (HitComponent :type "PrimitiveComponent Object Reference") (OtherActor :type "Actor Object Reference") (OtherComp :type "PrimitiveComponent Object Reference") (NormalImpulse :type "Vector Structure") (Hit :type "HitResult Structure (by ref)"))
  ;[1 0 0.06535 0.5] On Hit trigger
  (bind _impactdata (`self.BuildImpactDataFromHit` OtherActor Hit OtherComp NormalImpulse))
  (`/Game/Blueprint/Interfaces/BPI_ImpactReceiver.ApplyImpact` _impactdata))

(fn `ApplySideMaterial`
  (params (SideCollection :type "GeometryCollectionComponent Object Reference") (Material :type "MaterialInterface Object Reference"))
  (`/Engine/EditorBlueprintResources/StandardMacros.IsValid` Material
    (:`Is Valid`
      (`PrimitiveComponent.SetMaterial` (`local.SideCollection`) 0 (`local.Material`)))))

(fn `ApplyWallProfile`
  (locals (CurrentWallProfile :type "/Game/Blueprint/Impact/Destructible/PDA_DestructibleWallProfile Object Reference"))
  (set `local.CurrentWallProfile` (`self.GetWallProfile`))
  (`/Engine/EditorBlueprintResources/StandardMacros.IsValid` (`local.CurrentWallProfile`)
    (:`Is Valid`
      (`StaticMeshComponent.SetStaticMesh` (`self.Middle`) (`/Game/Blueprint/Impact/Destructible/PDA_DestructibleWallProfile.MiddleMesh` (`local.CurrentWallProfile`)))
      (`GeometryCollectionComponent.SetRestCollection` (`self.GC_PlasterSideA`) (`/Game/Blueprint/Impact/Destructible/PDA_DestructibleWallProfile.SideAGeometryCollection` (`local.CurrentWallProfile`)) false)
      (`GeometryCollectionComponent.SetRestCollection` (`self.GC_PlasterSideB`) (`/Game/Blueprint/Impact/Destructible/PDA_DestructibleWallProfile.SideBGeometryCollection` (`local.CurrentWallProfile`)) false)
      (`self.ApplySideMaterial` (`self.GC_PlasterSideA`) (`self.SideAMaterial`))
      (`self.ApplySideMaterial` (`self.GC_PlasterSideB`) (`self.SideBMaterial`))
      (`self.FitBlockerToWall` (`/Game/Blueprint/Impact/Destructible/PDA_DestructibleWallProfile.MiddleMesh` (`local.CurrentWallProfile`))))
    (:`Is Not Valid`
      (`self.FitBlockerToWall` null))))

(fn `FitBlockerToWall`
  (params (MiddleMesh :type "StaticMesh Object Reference"))
  (bind (_min _max) (break `Box` (`StaticMesh.GetBoundingBox` (`local.MiddleMesh`))))
  (bind (_min_2 _max_2) (break `Box` (`StaticMesh.GetBoundingBox` (`local.MiddleMesh`))))
  (`/Engine/EditorBlueprintResources/StandardMacros.IsValid` MiddleMesh
    (:`Is Valid`
      (`SceneComponent.K2_SetRelativeLocation` (`self.Blocker`) (* (+ _min _max) (0.5 0.5 0.5)) false false)
      (`BoxComponent.SetBoxExtent` (`self.Blocker`) (`KismetMathLibrary.MakeVector` (.x (* (- _max_2 _min_2) (0.5 0.5 0.5))) (`KismetMathLibrary.FMax` (.y (* (- _max_2 _min_2) (0.5 0.5 0.5))) (.y (`self.DefaultWallHalfSize`))) (.z (* (- _max_2 _min_2) (0.5 0.5 0.5)))) true))
    (:`Is Not Valid`
      (`SceneComponent.K2_SetRelativeLocation` (`self.Blocker`) (`KismetMathLibrary.MakeVector` 0.0 0.0 (.z (`self.DefaultWallHalfSize`))) false false)
      (`BoxComponent.SetBoxExtent` (`self.Blocker`) (`self.DefaultWallHalfSize`) true))))

(fn `GetImpactSide`
  (params (ImpactData :type "/Game/Blueprint/Impact/STR_ImpactData Structure"))
  (returns (Side :type "/Game/Blueprint/Impact/E_Wallside Enum"))
  (bind _returnvalue (`KismetMathLibrary.Dot_VectorVector` (`.Normal_5_12160DF741D20ABA0B31FFB05AB1541D` (break `/Game/Blueprint/Impact/STR_ImpactData` (`local.ImpactData`))) (`self.GetActorRightVector`)))
  (if (> _returnvalue 0.5)
    (return "NewEnumerator1")
    (elif (< _returnvalue -0.5)
      (return "NewEnumerator2")
      (else
        (return "NewEnumerator0")))))

(fn `GetWallProfile`
  (returns (WallProfile :type "/Game/Blueprint/Impact/Destructible/PDA_DestructibleWallProfile Object Reference"))
  (bind _aspda_destructible_wall_profile (cast `/Game/Blueprint/Impact/Destructible/PDA_DestructibleWallProfile` (`self.Profile`))
    (:`then`
      (return _aspda_destructible_wall_profile))
    (:`CastFailed`
      (return null))))

(fn `OnEnterDamaged`
  (params (ImpactData :type "/Game/Blueprint/Impact/STR_ImpactData Structure"))
  (returns (Handled :type Boolean))
  (`parent.OnEnterDamaged` ImpactData)
  (set `self.LastHitSide` (`self.GetImpactSide` (`local.ImpactData`)))
  (if (`self.DebugPrint`)
    (`KismetSystemLibrary.PrintString` (`KismetStringLibrary.Concat_StrStr` "Wall side hit: " (`|GetEnumeratorNameAsString` (`self.LastHitSide`))) true true (struct :`G` 0.66 :`B` 1.0 :`A` 1.0) 4.0))
  (return true))

(fn `OnEnterDestroyed`
  (params (ImpactData :type "/Game/Blueprint/Impact/STR_ImpactData Structure"))
  (returns (Handled :type Boolean))
  (bind _wallprofile (`self.GetWallProfile`))
  (`parent.OnEnterDestroyed` ImpactData)
  (`SceneComponent.SetVisibility` (`self.GC_PlasterSideA`) false false)
  (`SceneComponent.SetVisibility` (`self.GC_PlasterSideB`) false false)
  (`/Engine/EditorBlueprintResources/StandardMacros.IsValid` _wallprofile
    (:`Is Valid`
      (if (`/Game/Blueprint/Impact/Destructible/PDA_DestructibleWallProfile.DisableBlockerOnDestroyed` _wallprofile)
        (`PrimitiveComponent.SetCollisionEnabled` (`self.Blocker`) "NoCollision"))
      (return true))
    (:`Is Not Valid`
      (return true))))

(fn `UserConstructionScript`
  (`parent.UserConstructionScript`)
  (`self.ApplyWallProfile`))