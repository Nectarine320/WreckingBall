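; BP_LevelTeleporter is an interactable portal that opens its assigned level when the player overlaps it.
; It starts hidden with capsule collision off and shows the level name on a text component.
; Each GenericInteraction call toggles visibility, capsule collision and a siren sound, tracked by LevelLoaded, which reflects only the active state.
; Travel uses Open Level by object reference; the level-streaming nodes are unconnected.
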(event `self.ReceiveBeginPlay`
  ;[0 0.1529 1 0.5] Begin Play
  (`TextRenderComponent.K2_SetText` (`self.LevelTxt`) (`KismetTextLibrary.Conv_StringToText` (`KismetSystemLibrary.Conv_SoftObjectReferenceToString` (`self.Level`))))
  (`PrimitiveComponent.SetCollisionEnabled` (`self.Capsule`) "NoCollision")
  (bind _returnvalue (`AddComponent|NODE_AddAudioComponent-0`))
  (set `self.SFX SirenOn` _returnvalue)
  (`self.SetActorHiddenInGame` true))

(event `/Game/Blueprint/Interactable/BPI_Interactable.GenericInteraction`
  (params (Instigator :type "Actor Object Reference") (Owner :type "Actor Object Reference"))
  ;[1 0 0.06535 0.5] Message Recieve
  (if (`self.Level Loaded`)
    (set `self.Level Loaded` false)
    (`PrimitiveComponent.SetCollisionEnabled` (`self.Capsule`) "NoCollision")
    (`ActorComponent.Deactivate` (`self.SFX SirenOn`))
    (`self.SetActorHiddenInGame` true)
    (else
      (set `self.Level Loaded` true)
      (`PrimitiveComponent.SetCollisionEnabled` (`self.Capsule`) "QueryAndPhysics")
      (`ActorComponent.Activate` (`self.SFX SirenOn`) false)
      (`self.SetActorHiddenInGame` false))))

(event `self.Capsule.OnComponentBeginOverlap`
  (params (OverlappedComponent :type "PrimitiveComponent Object Reference") (OtherActor :type "Actor Object Reference") (OtherComp :type "PrimitiveComponent Object Reference") (OtherBodyIndex :type Integer) (bFromSweep :type Boolean) (SweepResult :type "HitResult Structure (by ref)"))
  ;[1 0 0.06535 0.5] Player Overlap
  (if (== OtherActor (`GameplayStatics.GetPlayerCharacter` 0))
    (`GameplayStatics.OpenLevelBySoftObjectPtr` (`self.Level`))))

(fn `UserConstructionScript`)