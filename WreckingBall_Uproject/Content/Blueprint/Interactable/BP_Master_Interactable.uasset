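; BP_Master_Interactable is an interactable Blueprint, named as a master, that shows a prompt widget to nearby characters.
; Begin and end overlaps on InteractCollisionBox toggle the widget's visibility when the other actor is a BP_GenericCharacter.
; An unconnected loop would send GenericInteractionMessage, with itself as owner, to valid Messengers implementing BPI_Interactable, but it never runs.
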(event `self.InteractCollisionBox.OnComponentBeginOverlap`
  (params (OverlappedComponent :type "PrimitiveComponent Object Reference") (OtherActor :type "Actor Object Reference") (OtherComp :type "PrimitiveComponent Object Reference") (OtherBodyIndex :type Integer) (bFromSweep :type Boolean) (SweepResult :type "HitResult Structure (by ref)"))
  ;[0.5781 0 0 0.5] Overlap Component
  (cast `/Game/Blueprint/Character/BP_GenericCharacter` OtherActor)
  (`SceneComponent.SetVisibility` (`self.Widget`) true false))

(event `self.InteractCollisionBox.OnComponentEndOverlap`
  (params (OverlappedComponent :type "PrimitiveComponent Object Reference") (OtherActor :type "Actor Object Reference") (OtherComp :type "PrimitiveComponent Object Reference") (OtherBodyIndex :type Integer))
  ;[0.5781 0 0 0.5] Overlap Component
  (cast `/Game/Blueprint/Character/BP_GenericCharacter` OtherActor)
  (`SceneComponent.SetVisibility` (`self.Widget`) false false))

(fn `UserConstructionScript`)