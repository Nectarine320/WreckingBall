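; BP_Elevator is an interactable elevator whose platform travels between top and bottom destination components, toggled by GenericInteraction according to IsTop.
; A timeline, played forward or reversed, lerps the platform between the two points with clamped height, updating IsTop when it finishes.
; BeginPlay sets the timeline's start from IsTop and scales its play rate inversely to travel distance.
; The construction script snaps the platform to its starting end.
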(event `self.ReceiveBeginPlay`
  (bind _returnvalue (/ 1.0 (`KismetMathLibrary.Vector_Distance` (* (`SceneComponent.RelativeLocation` (`self.BottomDestination`)) 0.005) (* (`SceneComponent.RelativeLocation` (`self.TopDestination`)) 0.005))))
  ;[0 0.1529 1 0.5] BeginPlay
  (`TimelineComponent.SetNewTime` (`self.ElevatorTimeline`) (`KismetMathLibrary.SelectFloat` 1.0 0.0 (`self.Is Top`)))
  (`TimelineComponent.SetPlayRate` (`self.ElevatorTimeline`) _returnvalue)
  (`KismetSystemLibrary.PrintString` (`KismetStringLibrary.Concat_StrStr` (`KismetStringLibrary.Conv_DoubleToString` _returnvalue) "SECONDS")))

(event `MoveUp`
  (bind (_returnvalue_x _returnvalue_y _returnvalue_z) (`KismetMathLibrary.BreakVector` (`SceneComponent.K2_GetComponentLocation` (`self.BottomDestination`))))
  (bind (_returnvalue_x_2 _returnvalue_y_2 _returnvalue_z_2) (`KismetMathLibrary.BreakVector` (`SceneComponent.K2_GetComponentLocation` (`self.TopDestination`))))
  ;[2 1.759 0.1667 0.5] Moving Elevator Animation
  (set `self.Is Moving` true)
  (bind (_direction _transitionlerp) (`Timeline|ElevatorTimeline` :!label _label)
    (:`Update`
      (`SceneComponent.K2_SetWorldLocation` (`self.SM_Platform`) (`KismetMathLibrary.MakeVector` (.x (`KismetMathLibrary.VLerp` (`SceneComponent.K2_GetComponentLocation` (`self.TopDestination`)) (`SceneComponent.K2_GetComponentLocation` (`self.BottomDestination`)) _transitionlerp)) (.y (`KismetMathLibrary.VLerp` (`SceneComponent.K2_GetComponentLocation` (`self.TopDestination`)) (`SceneComponent.K2_GetComponentLocation` (`self.BottomDestination`)) _transitionlerp)) (`KismetMathLibrary.FClamp` (.z (`KismetMathLibrary.VLerp` (`SceneComponent.K2_GetComponentLocation` (`self.TopDestination`)) (`SceneComponent.K2_GetComponentLocation` (`self.BottomDestination`)) _transitionlerp)) (- _returnvalue_z 10.0) (+ _returnvalue_z_2 10.0))) false false))
    (:`Finished`
      (set `self.Is Moving` false)
      (switch `ETimelineDirection` _direction
        (:`Forward`
          (set `self.Is Top` true))
        (:`Backward`
          (set `self.Is Top` false))))))

(event `/Game/Blueprint/Interactable/BPI_Interactable.GenericInteraction`
  (params (Instigator :type "Actor Object Reference") (Owner :type "Actor Object Reference"))
  ;[1 0 0.06535 0.5] Message Recieved
  (if (`self.Is Top`)
    (`self.MoveDown`)
    (else
      (`self.MoveUp`))))

(event `MoveDown`
  ;[2 1.759 0.1667 0.5] Moving Elevator Animation
  (set `self.Is Moving` true)
  (goto _label :!via `Reverse`))

(fn `UserConstructionScript`
  (bind _bottomdestination (`self.BottomDestination`))
  (bind _topdestination (`self.TopDestination`))
  (bind (_relativelocation_x _relativelocation_y _relativelocation_z) (`KismetMathLibrary.BreakVector` (`SceneComponent.RelativeLocation` _bottomdestination)))
  (bind (_relativelocation_x_2 _relativelocation_y_2 _relativelocation_z_2) (`KismetMathLibrary.BreakVector` (`SceneComponent.RelativeLocation` _topdestination)))
  (bind _returnvalue (select `bool` (`self.Is Top`) :`false` (`SceneComponent.RelativeLocation` (`self.BottomDestination`)) :`true` (`SceneComponent.RelativeLocation` (`self.TopDestination`))))
  (`SceneComponent.K2_SetRelativeLocation` _bottomdestination (`KismetMathLibrary.MakeVector` 0.0 0.0 _relativelocation_z) false false)
  (`SceneComponent.K2_SetRelativeLocation` _topdestination (`KismetMathLibrary.MakeVector` 0.0 0.0 _relativelocation_z_2) false false)
  (`SceneComponent.K2_SetRelativeLocation` (`self.SM_Platform`) _returnvalue false false)
  (`KismetSystemLibrary.PrintString` (`KismetStringLibrary.Conv_VectorToString` _returnvalue) true false))