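; Master physics ball that players can possess, that damages destructibles and scores at goalposts, where it stops and destroys itself.
; A kick triggers a looping timer that sphere-traces along its velocity, sending impact messages and destructible hits until it slows and deregisters.
; Physics collisions above the speed threshold also notify destructibles.
; BeginPlay applies a physics preset, registers a profile-driven Niagara trail and binds the play-area response.
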(event `InitializePlayAreaResponse`
  (add `/Game/Blueprint/BoundariesVolume/BPC_PlayAreaResponse.OnResponseStarted` (`self.PlayAreaResponse`) (`|CreateDelegate` :!event `ReleaseBallOnLeftPlayArea`)))

(event `self.ReceiveBeginPlay`
  ;[0 0.1529 1 0.5] Begin Play / Initializer
  (`self.Kick Scan Initialization`)
  (`self.ApplyPhysicsPreset`)
  (`self.InitializePlayAreaResponse`)
  (`self.InitializeBallTrail`))

(event `Goal`
  (params (Goalpost :type "/Game/Blueprint/BP_GoalPost_01 Object Reference (by ref)"))
  ;[1 0 0.06535 0.5] Goal
  (set `self.Goalpost` Goalpost)
  (`GameplayStatics.PlaySound2D` (`self.SFX_Burst`) 1.0 1.0 0.0 null null)
  (`KismetSystemLibrary.Delay` 0.25)
  (`PrimitiveComponent.SetPhysicsLinearVelocity` (`self.SM_PhysicObject`) (0.0 0.0 0.0) false "None")
  (`/Game/Blueprint/BP_GoalPost_01.Enable Goal` (`self.Goalpost`))
  (`self.K2_DestroyActor`))

(event `Trigger Kick Scan Timer`
  ;[1 0 0.06535 0.5] Trigger Kick Scan
  (`KismetSystemLibrary.K2_UnPauseTimerHandle` (`self.Kick Scan Timer`)))

(event `Kick Scan Initialization`
  ;[0 0.1529 1 0.5] Kick Scan Initialization
  (bind _returnvalue (`KismetSystemLibrary.K2_SetTimerDelegate` (delegate `Kick Scan`) 0.033 true true))
  (bind _output_get (set `self.Kick Scan Timer` _returnvalue))
  (`KismetSystemLibrary.K2_PauseTimerHandle` _output_get))

(event `Kick Scan`
  (bind _returnvalue (`self.K2_GetActorLocation`))
  ;[0 1 0.07739 0.5] Kick Scan Timer
  (if (< (`self.Min Vector value to check`) (`KismetMathLibrary.VSize` (`self.GetVelocity`)))
    (bind _outhits (`KismetSystemLibrary.SphereTraceMulti` _returnvalue (+ _returnvalue (* (`self.BallScanDistance`) (`SceneComponent.GetComponentVelocity` (`self.SM_PhysicObject`)))) (`self.BallScanRadius`) "TraceTypeQuery1" false (`|MakeArray` self :!type "Actor Object Reference") "None" true (struct :`R` 1.0 :`A` 1.0) (struct :`G` 1.0 :`A` 1.0) 1.0))
    (for _array_element _outhits
      (bind _output_get (set `self.Out Hit` _array_element))
      (bind (_bblockinghit _binitialoverlap _time _distance _location _impactpoint _normal _impactnormal _physmat _hitactor) (`GameplayStatics.BreakHitResult` _output_get))
      (if _bblockinghit
        (`self.ApplyScanImpact` (`self.Out Hit`))
        (bind _asbp_master_destructible (cast `/Game/Blueprint/Destructible/BP_MasterDestructible` _hitactor))
        (bind _output_get_2 (set `self.As BP Master Destructible` _asbp_master_destructible))
        (`/Game/Blueprint/Destructible/BP_MasterDestructible.Hit recieved` _output_get_2 self _impactnormal)))
    (else
      (`KismetSystemLibrary.K2_PauseTimerHandle` (`self.Kick Scan Timer`))
      (`self.Remove Id from Destructible List`))))

(event `self.ReceiveHit`
  (params (MyComp :type "PrimitiveComponent Object Reference") (Other :type "Actor Object Reference") (OtherComp :type "PrimitiveComponent Object Reference") (bSelfMoved :type Boolean) (HitLocation :type "Vector Structure") (HitNormal :type "Vector Structure") (NormalImpulse :type "Vector Structure") (Hit :type "HitResult Structure (by ref)"))
  (bind _output_get (set `self.Hit` Hit))
  (bind (_bblockinghit _binitialoverlap _time _distance _location _impactpoint _normal _impactnormal _physmat _hitactor) (`GameplayStatics.BreakHitResult` _output_get))
  (if _bblockinghit
    (if (< (`self.Min Vector value to check`) (`KismetMathLibrary.VSize` (`self.GetVelocity`)))
      (bind _asbp_master_destructible (cast `/Game/Blueprint/Destructible/BP_MasterDestructible` _hitactor))
      (bind _output_get_2 (set `self.As BP Master Destructible` _asbp_master_destructible))
      (`/Game/Blueprint/Destructible/BP_MasterDestructible.Hit recieved` _output_get_2 self _impactnormal))))

(fn `ApplyScanImpact`
  (params (Hit :type "HitResult Structure"))
  (bind (_bblockinghit _binitialoverlap _time _distance _location _impactpoint _normal _impactnormal _physmat _hitactor) (`GameplayStatics.BreakHitResult` Hit))
  (message `/Game/Blueprint/Interfaces/BPI_ImpactReceiver.ApplyImpact` _hitactor (make `/Game/Blueprint/Impact/STR_ImpactData` _impactpoint _impactnormal (`self.GetVelocity`) self null "NewEnumerator2" (`GameplayStatics.GetSurfaceType` Hit))))

(fn `InitializeBallTrail`
  (bind _returnvalue (`NiagaraFunctionLibrary.SpawnSystemAttached` "/Game/Art/VFX/BallTrail/NS_BallTrail.NS_BallTrail" (`self.SM_PhysicObject`) "None" (0.0 0.0 0.0) (struct) "SnapToTarget"))
  (bind _profile (`self.GetPhysicsProfile`))
  (`/Engine/EditorBlueprintResources/StandardMacros.IsValid` _profile
    (:`Is Valid`
      (`WB_BallPossessionSubsystem.RegisterBallTrail` self _returnvalue (`/Game/Blueprint/Ball/Data/PDA_PhysicsProfile.TrailStartSpeed` _profile) (`/Game/Blueprint/Ball/Data/PDA_PhysicsProfile.TrailStopSpeed` _profile) (`/Game/Blueprint/Ball/Data/PDA_PhysicsProfile.TrailImpactSpeed` _profile)))))

(fn `ReleaseBallOnLeftPlayArea`
  (params (ResponseTag :type "GameplayTag Structure"))
  (`GameplayStatics.PlaySound2D` (`self.SFX_Burst`) 1.0 1.0 0.0 null null)
  (`self.Remove Player Possession`))

(fn `Remove Id from Destructible List`
  (bind _as_bp_master_destructible (`self.As BP Master Destructible`))
  (`/Engine/EditorBlueprintResources/StandardMacros.IsValid` _as_bp_master_destructible
    (:`Is Valid`
      (`/Game/Blueprint/Destructible/BP_MasterDestructible.Remove From List` _as_bp_master_destructible self))))

(fn `Remove Player Possession`
  (bind _possessor (`self.Possessor`))
  (`/Engine/EditorBlueprintResources/StandardMacros.IsValid` _possessor
    (:`Is Valid`
      (`/Game/Blueprint/Character/BP_SoccerPlayer.Ball Depossession` _possessor)
      (set `self.Possessor` null))))

(fn `UserConstructionScript`
  (`parent.UserConstructionScript`))