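; BP_BallPreviewStudio is an actor that builds the row of ball preview pedestals, one per player slot.
; On BeginPlay it spawns BP_BallPedestal actors evenly spaced along its local Y axis, tags each with its slot index and stores them for lookup.
; It switches each pedestal's capture on or off, optionally limited to slots that GI_Core reports as Player.Slot.Joined.
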(event `self.ReceiveBeginPlay`
  ;[0 0.1529 1 0.5] Begin Play
  (`self.InitializeStudio`))

(fn `GetPedestal`
  (params (SlotIndex :type Integer))
  (returns (Pedestal :type "/Game/Blueprint/Ball/Preview/BP_BallPedestal Object Reference"))
  (if (`KismetArrayLibrary.Array_IsValidIndex` (`self.Pedestals`) (`local.SlotIndex`))
    (return (`|GetArrayItem` (`self.Pedestals`) (`local.SlotIndex`)))
    (else
      (return null))))

(fn `InitializeStudio`
  (`KismetArrayLibrary.Array_Clear` (`self.Pedestals`))
  (for _index (range (`self.PedestalCount`))
    (`self.SpawnPedestal` _index)))

(fn `IsSlotJoined`
  (params (SlotIndex :type Integer))
  (returns (IsJoined :type Boolean))
  (bind _asgi_core (cast `/Game/Blueprint/Core/GI_Core` (`GameplayStatics.GetGameInstance`))
    (:`then`
      (bind _state (`/Game/Blueprint/Core/GI_Core.GetSlotState` _asgi_core (`local.SlotIndex`)))
      (return (`BlueprintGameplayTagLibrary.MatchesTag` _state (struct :`TagName` "Player.Slot.Joined") true)))
    (:`CastFailed`
      (return false))))

(fn `SetAllCapturesActive`
  (params (Active :type Boolean) (OnlyJoinedSlots :type Boolean))
  (for _index (range (`KismetArrayLibrary.Array_Length` (`self.Pedestals`)))
    (`self.UpdateSlotCapture` _index (`local.Active`) (`local.OnlyJoinedSlots`))))

(fn `SpawnPedestal`
  (params (SlotIndex :type Integer))
  (locals (SpawnedPedestal :type "/Game/Blueprint/Ball/Preview/BP_BallPedestal Object Reference"))
  (bind _returnvalue (`|SpawnActorFromClass` "/Game/Blueprint/Ball/Preview/BP_BallPedestal.BP_BallPedestal_C" (`KismetMathLibrary.MakeTransform` (`KismetMathLibrary.TransformLocation` (`self.GetTransform`) (`KismetMathLibrary.MakeVector` 0.0 (* (`KismetMathLibrary.Conv_IntToDouble` (`local.SlotIndex`)) (`self.PedestalSpacing`)))) (`self.K2_GetActorRotation`)) "AlwaysSpawn" "MultiplyWithRoot" null null))
  (set `local.SpawnedPedestal` _returnvalue)
  (set `/Game/Blueprint/Ball/Preview/BP_BallPedestal.SlotIndex` (`local.SlotIndex`) (`local.SpawnedPedestal`))
  (`KismetArrayLibrary.Array_Add` (`self.Pedestals`) (`local.SpawnedPedestal`)))

(fn `UpdateSlotCapture`
  (params (SlotIndex :type Integer) (Active :type Boolean) (OnlyJoinedSlots :type Boolean))
  (locals (ShouldCapture :type Boolean))
  (bind _isjoined (`self.IsSlotJoined` (`local.SlotIndex`)))
  (set `local.ShouldCapture` (and (`local.Active`) (or (not (`local.OnlyJoinedSlots`)) _isjoined)))
  (bind _pedestal (`self.GetPedestal` (`local.SlotIndex`)))
  (`/Game/Blueprint/Ball/Preview/BP_BallPedestal.SetCaptureActive` _pedestal (`local.ShouldCapture`)))

(fn `UserConstructionScript`)