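; Preview pedestal that renders a spinning ball of a given type into a runtime-created render target.
; SetBall applies the type's preview mesh and material, then centers the mesh and scales its pivot to a uniform preview diameter.
; A show-only scene capture isolates the ball, and one toggle switches capture, visibility, light and spin, clearing the target when off.
; A timed confirm spin temporarily adds yaw speed to the idle rotation.
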(event `self.ReceiveBeginPlay`
  ;[0 0.1529 1 0.5] Begin Play
  (`self.InitializeIdleSpin`)
  (`self.InitializeCapture`))

(fn `FitBall`
  (locals (LargestSide :type "Float (double-precision)"))
  (bind (_min _max) (`StaticMeshComponent.GetLocalBounds` (`self.BallMesh`)))
  (bind (_min_2 _max_2) (`StaticMeshComponent.GetLocalBounds` (`self.BallMesh`)))
  (bind _returnvalue (/ (`self.PreviewBallDiameter`) (`local.LargestSide`)))
  (`SceneComponent.K2_SetRelativeLocation` (`self.BallMesh`) (* (+ _min _max) (`KismetMathLibrary.MakeVector` -0.5 -0.5 -0.5)) false false)
  (set `local.LargestSide` (`KismetMathLibrary.GetMaxElement` (- _max_2 _min_2)))
  (if (> (`local.LargestSide`) 0.0)
    (`SceneComponent.SetRelativeScale3D` (`self.BallPivot`) (`KismetMathLibrary.MakeVector` _returnvalue _returnvalue _returnvalue))))

(fn `GetRenderTarget`
  (returns (RenderTarget :type "TextureRenderTarget2D Object Reference"))
  (return (`self.CaptureRenderTarget`)))

(fn `InitializeCapture`
  (bind _returnvalue (`KismetRenderingLibrary.CreateRenderTarget2D` (`self.RenderTargetSize`) (`self.RenderTargetSize`)))
  (set `self.CaptureRenderTarget` _returnvalue)
  (set `SceneCaptureComponent2D.TextureTarget` (`self.CaptureRenderTarget`) (`self.Capture`))
  (`SceneCaptureComponent.ClearShowOnlyComponents` (`self.Capture`))
  (`SceneCaptureComponent.ShowOnlyComponent` (`self.Capture`) (`self.BallMesh`))
  (`self.SetCaptureActive` false))

(fn `InitializeIdleSpin`
  (`MovementComponent.SetUpdatedComponent` (`self.IdleSpin`) (`self.BallPivot`))
  (set `self.IdleRotationRate` (`RotatingMovementComponent.RotationRate` (`self.IdleSpin`))))

(fn `SetBall`
  (params (BallType :type "/Game/Blueprint/Ball/Data/PDA_BallType Object Reference"))
  (`/Engine/EditorBlueprintResources/StandardMacros.IsValid` (`local.BallType`)
    (:`Is Valid`
      (`StaticMeshComponent.SetStaticMesh` (`self.BallMesh`) (`/Game/Blueprint/Ball/Data/PDA_BallType.PreviewMesh` (`local.BallType`)))
      (`PrimitiveComponent.SetMaterial` (`self.BallMesh`) 0 (`/Game/Blueprint/Ball/Data/PDA_BallType.PreviewMaterial` (`local.BallType`)))
      (`self.FitBall`))))

(fn `SetCaptureActive`
  (params (Active :type Boolean))
  (set `SceneCaptureComponent.bCaptureEveryFrame` (`local.Active`) (`self.Capture`))
  (`SceneComponent.SetVisibility` (`self.BallMesh`) (`local.Active`) false)
  (`SceneComponent.SetVisibility` (`self.Light`) (`local.Active`) false)
  (`ActorComponent.SetActive` (`self.IdleSpin`) (`local.Active`) false)
  (if (not (`local.Active`))
    (`KismetRenderingLibrary.ClearRenderTarget2D` (`self.CaptureRenderTarget`))))

(fn `StartConfirmSpin`
  (params (Degrees :type "Float (double-precision)") (Duration :type "Float (double-precision)"))
  (bind _idlerotationrate (`self.IdleRotationRate`))
  (`KismetSystemLibrary.K2_ClearAndInvalidateTimerHandle` (`self.ConfirmSpinTimer`))
  (set `RotatingMovementComponent.RotationRate` (`KismetMathLibrary.MakeRotator` (.roll _idlerotationrate) (.pitch _idlerotationrate) (+ (.yaw _idlerotationrate) (/ (`local.Degrees`) (`local.Duration`)))) (`self.IdleSpin`))
  (bind _returnvalue (`KismetSystemLibrary.K2_SetTimerDelegate` (`|CreateDelegate` :!event `StopConfirmSpin`) (`local.Duration`)))
  (set `self.ConfirmSpinTimer` _returnvalue))

(fn `StopConfirmSpin`
  (`KismetSystemLibrary.K2_ClearAndInvalidateTimerHandle` (`self.ConfirmSpinTimer`))
  (set `RotatingMovementComponent.RotationRate` (`self.IdleRotationRate`) (`self.IdleSpin`)))

(fn `UserConstructionScript`)