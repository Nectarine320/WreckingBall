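; Spawn manager for the soccer mode that creates match balls near a start point and registers each as the gamemode's active ball.
; StartSpawn and GoalSpawn spawn a weighted ball type picked by the game instance, falling back to a default type or the standard soccer ball class.
; Ball classes load blocking, and spawns land on random reachable nearby points.
; A debug function force-drops and destroys existing balls, then spawns the next debug type.
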(event `self.ReceiveBeginPlay`
  ;[0 0.1529 1 0.5] Begin Play
  (bind _asbp_soccer_gamemode (cast `/Game/Blueprint/Character/BP_SoccerGamemode` (`GameplayStatics.GetGameMode`)))
  (set `/Game/Blueprint/Character/BP_SoccerGamemode.SpawnManager` self _asbp_soccer_gamemode))

(event `Start Spawn`
  ;[1 0 0.06535 0.5] Trigger Spawning
  (`self.SpawnMatchBall`))

(event `Goal Spawn`
  ;[1 0 0.06535 0.5] Trigger Spawning
  (`self.SpawnMatchBall`))

(fn `DebugCycleBall`
  (bind _debugballtypes (`self.DebugBallTypes`))
  (bind _returnvalue (`KismetArrayLibrary.Array_Length` _debugballtypes))
  (bind _output (`|GetArrayItem` _debugballtypes (`self.DebugBallIndex`)))
  (if (> _returnvalue 0)
    (set `self.DebugBallIndex` -1)
    (bind _outactors (`GameplayStatics.GetAllActorsOfClass` "/Game/Blueprint/Ball/BP_PO_Master_Ball_01.BP_PO_Master_Ball_01_C"))
    (for _array_element _outactors
      (for _index (range (+ (- _returnvalue 1) 1))
        (bind _returnvalue_2 (`KismetSystemLibrary.LoadClassAsset_Blocking` (`/Game/Blueprint/Ball/Data/PDA_BallType.BallClass` (`|GetArrayItem` _debugballtypes _index))))
        (if (`KismetMathLibrary.ClassIsChildOf` (`GameplayStatics.GetObjectClass` _array_element) _returnvalue_2)
          (set `self.DebugBallIndex` _index)))
      (bind _possessor (`/Game/Blueprint/Ball/BP_PO_Master_Ball_01.Possessor` _array_element))
      (`/Engine/EditorBlueprintResources/StandardMacros.IsValid` _possessor
        (:`Is Valid`
          (`/Game/Blueprint/Character/BPC_GrabObject.ForceDrop` (`/Game/Blueprint/Character/BP_GenericCharacter.BPC_GrabPhysicObject` _possessor) (`KismetMathLibrary.MakeVector` 0.0))
          (`self.K2_DestroyActor` _array_element))
        (:`Is Not Valid`
          (`self.K2_DestroyActor` _array_element))))
    (set `self.DebugBallIndex` (mod (+ (`self.DebugBallIndex`) 1) _returnvalue))
    (bind _returnvalue_3 (`KismetSystemLibrary.LoadClassAsset_Blocking` (`/Game/Blueprint/Ball/Data/PDA_BallType.BallClass` _output)))
    (bind _asbp_po_master_ball_01 (castclass `/Game/Blueprint/Ball/BP_PO_Master_Ball_01` _returnvalue_3))
    (bind _returnvalue_4 (`|SpawnActorFromClass` _asbp_po_master_ball_01 (`KismetMathLibrary.MakeTransform` (`NavigationSystemV1.K2_GetRandomReachablePointInRadius` (`SceneComponent.K2_GetComponentLocation` (`self.Start SpawnPoint`)) 75.0 null null)) "AdjustIfPossibleButAlwaysSpawn" "MultiplyWithRoot" null null))
    (`self.RegisterSpawnedBall` _returnvalue_4)
    (`KismetSystemLibrary.PrintString` (`KismetTextLibrary.Conv_TextToString` (`/Game/Blueprint/Ball/Data/PDA_BallType.DisplayName` _output)))))

(fn `GetMatchBallType`
  (returns (BallType :type "/Game/Blueprint/Ball/Data/PDA_BallType Object Reference"))
  (bind _asgi_core (cast `/Game/Blueprint/Core/GI_Core` (`GameplayStatics.GetGameInstance`))
    (:`then`
      (bind _balltype (`/Game/Blueprint/Core/GI_Core.PickWeightedBallType` _asgi_core))
      (`/Engine/EditorBlueprintResources/StandardMacros.IsValid` _balltype
        (:`Is Valid`
          (return _balltype))
        (:`Is Not Valid`
          (return (`self.DefaultBallType`)))))
    (:`CastFailed`
      (return (`self.DefaultBallType`)))))

(fn `RegisterSpawnedBall`
  (params (Ball :type "Actor Object Reference"))
  (bind _asbp_soccer_gamemode (cast `/Game/Blueprint/Character/BP_SoccerGamemode` (`GameplayStatics.GetGameMode`)))
  (`/Game/Blueprint/Character/BP_SoccerGamemode.SetActiveBall` _asbp_soccer_gamemode Ball))

(fn `SpawnMatchBall`
  (bind _balltype (`self.GetMatchBallType`))
  (bind _returnvalue (`KismetSystemLibrary.LoadClassAsset_Blocking` (`/Game/Blueprint/Ball/Data/PDA_BallType.BallClass` _balltype)))
  (bind _asbp_po_master_ball_01 (castclass `/Game/Blueprint/Ball/BP_PO_Master_Ball_01` _returnvalue)
    (:`then`
      (bind _returnvalue_2 (`|SpawnActorFromClass` _asbp_po_master_ball_01 (`KismetMathLibrary.MakeTransform` (`NavigationSystemV1.K2_GetRandomReachablePointInRadius` (`SceneComponent.K2_GetComponentLocation` (`self.Start SpawnPoint`)) 75.0 null null)) "Undefined" "MultiplyWithRoot" self null))
      (`self.RegisterSpawnedBall` _returnvalue_2))
    (:`CastFailed`
      (bind _returnvalue_3 (`|SpawnActorFromClass` "/Game/Blueprint/Ball/BP_PO_SoccerBall_01.BP_PO_SoccerBall_01_C" (`KismetMathLibrary.MakeTransform` (`NavigationSystemV1.K2_GetRandomReachablePointInRadius` (`SceneComponent.K2_GetComponentLocation` (`self.Start SpawnPoint`)) 75.0 null null)) "Undefined" "MultiplyWithRoot" self null))
      (`self.RegisterSpawnedBall` _returnvalue_3))))

(fn `UserConstructionScript`)