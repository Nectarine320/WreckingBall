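; Spawn manager actor for soccer balls that registers itself with BP_SoccerGamemode on BeginPlay.
; StartSpawn spawns a master ball at a random reachable navmesh point near StartSpawnPoint.
; OutOfBound finds the child of OutOfBoundSpawnPoint closest to the exit location, then spawns a ball of the same class at a random reachable point around it.
; The construction script keeps OutOfBoundSpawnPoint at zero relative location.
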(event `self.ReceiveBeginPlay`
  (bind _asbp_soccer_gamemode (cast `/Game/Blueprint/Character/BP_SoccerGamemode` (`GameplayStatics.GetGameMode`)))
  (set `/Game/Blueprint/Character/BP_SoccerGamemode.SpawnManager` self _asbp_soccer_gamemode))

(event `Start Spawn`
  (`|SpawnActorFromClass` "/Game/Blueprint/PhysicalObject/Ball/BP_PO_Master_Ball_01.BP_PO_Master_Ball_01_C" (`KismetMathLibrary.MakeTransform` (`NavigationSystemV1.K2_GetRandomReachablePointInRadius` (`SceneComponent.K2_GetComponentLocation` (`self.Start SpawnPoint`)) 75.0 null null)) "Undefined" "MultiplyWithRoot" self null))

(event `OutOfBound`
  (params (OutOfBoundLocation :type "Vector Structure") (BP_Ball :type "/Game/Blueprint/PhysicalObject/Ball/BP_PO_Master_Ball_01 Object Reference"))
  (bind _output_get (set `self.BP Ball` BP_Ball))
  (set `self.ClosestDistance` (`self.FartestDistance`))
  (set `self.Closest Actor` null)
  (for _array_element (`SceneComponent.GetChildrenComponents` (`self.OutOfBoundSpawn Point`) false)
    (bind _returnvalue (`KismetMathLibrary.Vector_Distance` OutOfBoundLocation (`SceneComponent.K2_GetComponentLocation` _array_element)))
    (if (<= _returnvalue (`self.ClosestDistance`))
      (set `self.ClosestDistance` _returnvalue)
      (set `self.Closest Actor` _array_element)))
  (`|SpawnActorFromClass` (`GameplayStatics.GetObjectClass` _output_get) (`KismetMathLibrary.MakeTransform` (`NavigationSystemV1.K2_GetRandomReachablePointInRadius` (`SceneComponent.K2_GetComponentLocation` (`self.Closest Actor`)) 150.0 null null)) "Undefined" "MultiplyWithRoot" self null))

(fn `UserConstructionScript`
  (`SceneComponent.K2_SetRelativeLocation` (`self.OutOfBoundSpawn Point`) (0.0 0.0 0.0) false false))