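; Master ball physical object that handles going out of bounds and scoring goals, each with a burst sound and short delays.
; OutOfBound reports the ball and its location to the owning BP_SpawnManager, releases any possessing player and destroys the ball.
; Goal zeroes the mesh's physics velocity, moves actor and mesh to a fixed point above the world origin, then calls EnableGoal on the goalpost.
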(event `self.ReceiveBeginPlay`
  ;[0 0.1529 1 0.5] Begin Play / Initializer
)

(event `OutOfBound`
  (`GameplayStatics.PlaySound2D` (`self.SFX_Burst`) 1.0 1.0 0.0 null null)
  (bind _output_get (set `self.OutOfBoundLocation` (`self.K2_GetActorLocation`)))
  (`KismetSystemLibrary.Delay` 0.25)
  (bind _asbp_spawn_manager (cast `/Game/Blueprint/PhysicalObject/Ball/BP_SpawnManager` (`self.GetOwner`)))
  (`/Game/Blueprint/PhysicalObject/Ball/BP_SpawnManager.OutOfBound` _asbp_spawn_manager _output_get self)
  (`self.Remove Player Possession`)
  (`self.K2_DestroyActor`))

(event `Goal`
  (params (Goalpost :type "/Game/Blueprint/BP_GoalPost_01 Object Reference (by ref)"))
  (set `self.Goalpost` Goalpost)
  (`GameplayStatics.PlaySound2D` (`self.SFX_Burst`) 1.0 1.0 0.0 null null)
  (`KismetSystemLibrary.Delay` 0.25)
  (`PrimitiveComponent.SetPhysicsLinearVelocity` (`self.SM_Ball`) (0.0 0.0 0.0) false "None")
  (`KismetSystemLibrary.Delay` 0.5)
  (`self.K2_SetActorLocation` (0.0 0.0 350.0))
  (`SceneComponent.K2_SetWorldLocation` (`self.SM_Ball`) (0.0 0.0 350.0) true true)
  (`/Game/Blueprint/BP_GoalPost_01.Enable Goal` (`self.Goalpost`)))

(fn `Remove Player Possession`
  (bind _possessor (`self.Possessor`))
  (`/Engine/EditorBlueprintResources/StandardMacros.IsValid` _possessor
    (:`Is Valid`
      (`/Game/Blueprint/Character/BP_SoccerPlayer.Ball Depossession` _possessor)
      (set `self.Possessor` null))))

(fn `UserConstructionScript`
  (`parent.UserConstructionScript`))