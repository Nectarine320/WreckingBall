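; A grouped kitchen fridge prop built from three child-actor parts: the body, a bottom door and a top door.
; On BeginPlay it casts each child actor to BP_M_PhysicObject and stores a reference to it.
; It then binds two physics constraints at runtime, linking each door's mesh to the body mesh so the parts act as one jointed physics object.
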(event `self.ReceiveBeginPlay`
  (bind _asbp_m_physic_object (cast `/Game/Blueprint/PhysicalObject/BP_M_PhysicObject` (`ChildActorComponent.ChildActor` (`self.BP_Comb_FridgePart_01`))))
  (set `self.As BP Fridge` _asbp_m_physic_object)
  (bind _asbp_m_physic_object_2 (cast `/Game/Blueprint/PhysicalObject/BP_M_PhysicObject` (`ChildActorComponent.ChildActor` (`self.BP_Comb_FridgePart_02`))))
  (set `self.As BP Fridge Door Bot` _asbp_m_physic_object_2)
  (bind _asbp_m_physic_object_3 (cast `/Game/Blueprint/PhysicalObject/BP_M_PhysicObject` (`ChildActorComponent.ChildActor` (`self.BP_Comb_FridgePart_03`))))
  (set `self.As BP Fridge Door Top` _asbp_m_physic_object_3)
  (`PhysicsConstraintComponent.SetConstrainedComponents` (`self.PhysicsConstraint`) (`/Game/Blueprint/PhysicalObject/BP_M_PhysicObject.SM_PhysicObject` (`self.As BP Fridge`)) "None" (`/Game/Blueprint/PhysicalObject/BP_M_PhysicObject.SM_PhysicObject` (`self.As BP Fridge Door Bot`)) "None")
  (`PhysicsConstraintComponent.SetConstrainedComponents` (`self.PhysicsConstraint1`) (`/Game/Blueprint/PhysicalObject/BP_M_PhysicObject.SM_PhysicObject` (`self.As BP Fridge`)) "None" (`/Game/Blueprint/PhysicalObject/BP_M_PhysicObject.SM_PhysicObject` (`self.As BP Fridge Door Top`)) "None"))

(fn `UserConstructionScript`)