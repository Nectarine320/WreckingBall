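; Physics prop that applies a data-asset preset, registers with the physics budget manager, and can start mounted on a destructible.
; When mounted, it stays non-simulated on the parent's side surface, chosen by a right-vector dot product.
; Hard hits, parent destruction, nearby same-side impacts or random damage shakes detach it with an outward impulse.
; Impact damage is disallowed while it is held or during a timed post-detach grace period.
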(event `self.ReceiveBeginPlay`
  ;[0 0.4851 1 0.5] Begin Play
  (`self.ApplyPhysicsPreset`)
  (`self.InitializeAttachedBehavior`)
  (`KismetSystemLibrary.DelayUntilNextTick`)
  (`self.RegisterToPhysicsBudget`))

(event `self.SM_PhysicObject.OnComponentHit`
  (params (HitComponent :type "PrimitiveComponent Object Reference") (OtherActor :type "Actor Object Reference") (OtherComp :type "PrimitiveComponent Object Reference") (NormalImpulse :type "Vector Structure") (Hit :type "HitResult Structure (by ref)"))
  ;[1 0 0.06535 0.5] Hit event
  (`self.HandleAttachedHit` OtherComp NormalImpulse))

(event `self.ReceiveEndPlay`
  (params (EndPlayReason :type "EEndPlayReason Enum" :default "Destroyed"))
  ;[0 0.153 1 0.5] Prop – désinscription du budget physique
  (`self.UnregisterFromPhysicsBudget`))

(event `self.OnParentDamaged`
  (params (Parent :type "Actor Object Reference") (ImpactLocation :type "Vector Structure") (ImpactNormal :type "Vector Structure") (Damage :type "Float (single-precision)"))
  ; Input on Binding
  (`self.HandleParentDamaged` (make `/Game/Blueprint/Impact/STR_ImpactData` ImpactLocation ImpactNormal (0.0 0.0 0.0) null) Damage))

(event `self.OnParentDestroyed`
  (params (Parent :type "Actor Object Reference"))
  ; Input on Binding
  (`self.DetachFromDestructible`))

(fn `ApplyPhysicsPreset`
  (`/Engine/EditorBlueprintResources/StandardMacros.IsValid` (`self.PhysicsPreset`)
    (:`Is Valid`
      (`PrimitiveComponent.SetMassOverrideInKg` (`self.SM_PhysicObject`) "None" (`/Game/Blueprint/Ball/Data/PDA_PhysicsProfile.MassKg` (`self.PhysicsPreset`)) true)
      (`PrimitiveComponent.SetLinearDamping` (`self.SM_PhysicObject`) (`/Game/Blueprint/Ball/Data/PDA_PhysicsProfile.LinearDamping` (`self.PhysicsPreset`)))
      (`PrimitiveComponent.SetAngularDamping` (`self.SM_PhysicObject`) (`/Game/Blueprint/Ball/Data/PDA_PhysicsProfile.AngularDamping` (`self.PhysicsPreset`)))
      (`PrimitiveComponent.SetPhysicsMaxAngularVelocityInDegrees` (`self.SM_PhysicObject`) (`/Game/Blueprint/Ball/Data/PDA_PhysicsProfile.MaxAngularVelocity` (`self.PhysicsPreset`)) false "None")
      (`/Engine/EditorBlueprintResources/StandardMacros.IsValid` (`/Game/Blueprint/Ball/Data/PDA_PhysicsProfile.PhysicalMaterial` (`self.PhysicsPreset`))
        (:`Is Valid`
          (`PrimitiveComponent.SetPhysMaterialOverride` (`self.SM_PhysicObject`) (`/Game/Blueprint/Ball/Data/PDA_PhysicsProfile.PhysicalMaterial` (`self.PhysicsPreset`))))))))

(fn `AssignHolder`
  (params (NewHolder :type "Actor Object Reference"))
  (set `self.CurrentHolder` NewHolder))

(fn `CanDealImpactDamage`
  (returns (CanDamage :type Boolean))
  (`/Engine/EditorBlueprintResources/StandardMacros.IsValid` (`self.CurrentHolder`)
    (:`Is Valid`
      (return false))
    (:`Is Not Valid`
      (return (not (`self.DetachGraceActive`))))))

(fn `DetachFromDestructible`
  (`/Engine/EditorBlueprintResources/StandardMacros.IsValid` (`self.AttachedParent`)
    (:`Is Valid`
      (`self.K2_DetachFromActor` "KeepWorld" "KeepWorld" "KeepWorld")
      (`PrimitiveComponent.SetSimulatePhysics` (`self.SM_PhysicObject`) true)
      (bind _profile (`self.GetPhysicsProfile`))
      (`PrimitiveComponent.AddImpulse` (`self.SM_PhysicObject`) (* (* (`self.GetActorRightVector` (`self.AttachedParent`)) (`self.GetAttachedSideSign`)) (`/Game/Blueprint/Ball/Data/PDA_PhysicsProfile.DetachImpulse` _profile)) "None" true)
      (set `self.AttachedParent` null)
      (bind _profile_2 (`self.GetPhysicsProfile`))
      (if (> (`/Game/Blueprint/Ball/Data/PDA_PhysicsProfile.DetachGraceSeconds` _profile_2) 0.0)
        (set `self.DetachGraceActive` true)
        (`KismetSystemLibrary.K2_SetTimer` self "EndDetachGrace" (`/Game/Blueprint/Ball/Data/PDA_PhysicsProfile.DetachGraceSeconds` _profile_2))))))

(fn `EndDetachGrace`
  (set `self.DetachGraceActive` false))

(fn `GetAttachedSideSign`
  (returns (SideSign :type "Float (double-precision)"))
  (return (`KismetMathLibrary.SignOfFloat` (`KismetMathLibrary.Dot_VectorVector` (- (`self.K2_GetActorLocation`) (`self.K2_GetActorLocation` (`self.AttachedParent`))) (`self.GetActorRightVector` (`self.AttachedParent`))))))

(fn `GetPhysicsProfile`
  (returns (Profile :type "/Game/Blueprint/Ball/Data/PDA_PhysicsProfile Object Reference"))
  (`/Engine/EditorBlueprintResources/StandardMacros.IsValid` (`self.PhysicsPreset`)
    (:`Is Valid`
      (return (`self.PhysicsPreset`)))
    (:`Is Not Valid`
      (return "/Game/Blueprint/Impact/Data/DA_Physics_Object_Default.DA_Physics_Object_Default"))))

(fn `HandleAttachedHit`
  (params (OtherComp :type "PrimitiveComponent Object Reference") (NormalImpulse :type "Vector Structure"))
  (`/Engine/EditorBlueprintResources/StandardMacros.IsValid` (`self.AttachedParent`)
    (:`Is Valid`
      (bind _returnvalue (`PrimitiveComponent.GetPhysicsLinearVelocity` OtherComp "None"))
      (bind _profile (`self.GetPhysicsProfile`))
      (if (>= (`KismetMathLibrary.FMax` (`KismetMathLibrary.VSize` _returnvalue) (`KismetMathLibrary.SafeDivide` (`KismetMathLibrary.VSize` (`local.NormalImpulse`)) (`PrimitiveComponent.GetMass` (`local.OtherComp`)))) (`/Game/Blueprint/Ball/Data/PDA_PhysicsProfile.DetachImpactSpeed` _profile))
        (`self.DetachFromDestructible`)))))

(fn `HandleParentDamaged`
  (params (ImpactData :type "/Game/Blueprint/Impact/STR_ImpactData Structure") (Damage :type "Float (double-precision)"))
  (`/Engine/EditorBlueprintResources/StandardMacros.IsValid` (`self.AttachedParent`)
    (:`Is Valid`
      (bind _destructible (`/Game/Blueprint/Impact/Destructible/BP_Destructible_Base.IsSideDestructible` (`self.AttachedParent`) (`self.GetAttachedSideSign`)))
      (if _destructible
        (bind _profile (`self.GetPhysicsProfile`))
        (if (or (<= (`/Game/Blueprint/Impact/Destructible/BP_Destructible_Base.CurrentHealth` (`self.AttachedParent`)) 0.0) (and (`self.IsImpactOnAttachedSide` (`local.ImpactData`)) (<= (`KismetMathLibrary.Vector_Distance` (`.Location_2_D59D6FBE46C7A7483A69D18B3893A402` (break `/Game/Blueprint/Impact/STR_ImpactData` (`local.ImpactData`))) (`self.K2_GetActorLocation`)) (`/Game/Blueprint/Ball/Data/PDA_PhysicsProfile.DetachRadius` _profile))))
          (`self.DetachFromDestructible`)
          (else
            (bind _shoulddetach (`self.RollShakeDetach` (`local.Damage`)))
            (if _shoulddetach
              (`self.DetachFromDestructible`))))))))

(fn `InitializeAttachedBehavior`
  (if (`self.UseAttachedBehavior`)
    (bind _asbp_destructible_base (cast `/Game/Blueprint/Impact/Destructible/BP_Destructible_Base` (`self.GetAttachParentActor`))
      (:`then`
        (set `self.AttachedParent` _asbp_destructible_base)
        (`PrimitiveComponent.SetSimulatePhysics` (`self.SM_PhysicObject`) false)
        (`PrimitiveComponent.SetNotifyRigidBodyCollision` (`self.SM_PhysicObject`) true)
        (bind _surface (`/Game/Blueprint/Impact/Destructible/BP_Destructible_Base.GetAttachSurfaceForSide` (`self.AttachedParent`) (`self.GetAttachedSideSign`)))
        (`self.K2_AttachToComponent` _surface "None" "KeepWorld" "KeepWorld" "KeepWorld" false))
      (:`CastFailed`
        (`PrimitiveComponent.SetSimulatePhysics` (`self.SM_PhysicObject`) true)))))

(fn `IsImpactOnAttachedSide`
  (params (ImpactData :type "/Game/Blueprint/Impact/STR_ImpactData Structure"))
  (returns (OnAttachedSide :type Boolean))
  (return (> (* (`KismetMathLibrary.Dot_VectorVector` (`.Normal_5_12160DF741D20ABA0B31FFB05AB1541D` (break `/Game/Blueprint/Impact/STR_ImpactData` ImpactData)) (`self.GetActorRightVector` (`self.AttachedParent`))) (`self.GetAttachedSideSign`)) 0.0)))

(fn `RegisterToPhysicsBudget`
  (bind _returnvalue (`GameplayStatics.GetActorOfClass` "/Script/WreckingBall.WB_PhysicsBudgetManager_Base"))
  (`/Engine/EditorBlueprintResources/StandardMacros.IsValid` _returnvalue
    (:`Is Valid`
      (`WB_PhysicsBudgetManager_Base.RegisterPhysicsProp` _returnvalue (`self.SM_PhysicObject`)))))

(fn `RollShakeDetach`
  (params (Damage :type "Float (double-precision)"))
  (returns (ShouldDetach :type Boolean))
  (bind _profile (`self.GetPhysicsProfile`))
  (if (and (> (`/Game/Blueprint/Ball/Data/PDA_PhysicsProfile.ShakeDetachMinDamage` _profile) 0.0) (>= (`local.Damage`) (`/Game/Blueprint/Ball/Data/PDA_PhysicsProfile.ShakeDetachMinDamage` _profile)))
    (return (`KismetMathLibrary.RandomBoolWithWeight` (`/Game/Blueprint/Ball/Data/PDA_PhysicsProfile.ShakeDetachChance` _profile)))
    (else
      (return false))))

(fn `UnregisterFromPhysicsBudget`
  (bind _returnvalue (`GameplayStatics.GetActorOfClass` "/Script/WreckingBall.WB_PhysicsBudgetManager_Base"))
  (`/Engine/EditorBlueprintResources/StandardMacros.IsValid` _returnvalue
    (:`Is Valid`
      (`WB_PhysicsBudgetManager_Base.UnregisterPhysicsProp` _returnvalue (`self.SM_PhysicObject`)))))

(fn `UserConstructionScript`
  (if (`self.UseAttachedBehavior`)
    (`PrimitiveComponent.SetSimulatePhysics` (`self.SM_PhysicObject`) false)))