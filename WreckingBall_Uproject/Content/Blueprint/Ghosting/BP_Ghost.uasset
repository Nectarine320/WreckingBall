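; BP_Ghost is a short-lived ghost actor that displays a skinned mesh in a ghost material.
; On BeginPlay its PoseableMesh takes the skinned asset from SkinAsset, reinitializing the pose, and gets MI_Ghost on every material slot.
; The actor then waits for LifeDuration and destroys itself, with no pose copy or fade logic in this Blueprint.
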(event `self.ReceiveBeginPlay`
  (`SkinnedMeshComponent.SetSkinnedAssetAndUpdate` (`self.PoseableMesh`) (`SkinnedMeshComponent.GetSkinnedAsset` (`self.Skin Asset`)) true)
  (for (_ _array_index) (`MeshComponent.GetMaterials` (`self.PoseableMesh`))
    (`PrimitiveComponent.SetMaterial` (`self.PoseableMesh`) _array_index "/Game/Art/Material/Master_Materials/MI_Ghost.MI_Ghost"))
  (`KismetSystemLibrary.Delay` (`self.LifeDuration`))
  (`self.K2_DestroyActor`))

(fn `UserConstructionScript`)